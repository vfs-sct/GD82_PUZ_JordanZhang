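; Actor component that lets its owner, character or physics object, pass through linked portals.
; On BeginPlay it builds a hidden mesh clone, shown in portal range and mirrored at the exit each tick while material clip planes slice both meshes.
; Overlap queries at the mirrored position push pawns and physics bodies beyond the exit.
; Teleporting remaps transform and clamped velocity, boosting pitched exits and using LaunchCharacter for tilted characters to avoid clipping.
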(event Custom|Update%20Character%20Velocity
  (params (New%20Velocity :type Vector) (Character :type Character%20Object%20Reference))
  (bind _returnvalue (Pawn|GetMovementComponent Character))
  ;[0 0 0] Update character velocity. If the character is tilted, use the launch character function that will apply the velocity one frame after and set the movement mode to falling, this is to avoid clipping issues.
  (if (== (Math|Float|SnapToGrid(Float) (.Pitch (Math|Rotator|BreakRotator (Transformation|GetActorRotation Character))) 1.0) 0.0)
    (Variables|/Script/Engine.MovementComponent|SetVelocity _returnvalue New%20Velocity)
    (else
      (Components|Movement|StopMovementImmediately _returnvalue)
      (Character|LaunchCharacter Character New%20Velocity true true))))

(event EventTick
  (params (DeltaSeconds :type Float%20%28single-precision%29))
  ;[0 0 0] Update mesh clone position and collisions.
  (if (Math|Boolean|ANDBoolean (Utilities|IsValid (Variables|Default|GetClone%20Root)) (Utilities|IsValid (Variables|Runtime|GetIn%20Portal)) (Utilities|IsValid (Variables|Runtime|GetOut%20Portal)) (Variables|Runtime|GetIs%20In%20Portal%20Range?))
    (Portals|UpdateClonePositionThroughPortals)
    (Clone|ApplyCloneCollisionForces)))

(event EventBeginPlay
  ;[0 0 0] On Begin Play, create a clone for this actor
  (bind _returnvalue (Clone|CreateOwnerClone false))
  (Variables|Default|SetClone%20Root _returnvalue))

(fn IsAttachedtoCharacter?
  (bind _ascharacter (Utilities|Casting|CastToCharacter (Components|GetOwner))
    (:then
      (return true _ascharacter))
    (:CastFailed
      (return false 0))))

(fn CreateOwnerClone
  (params (Visibility :type Boolean))
  (Utilities|IsValid (Variables|Default|GetClone%20Root)
    (:Is%20Not%20Valid
      (bind _output_get (LocalVariables|SetLocalOwnerRoot (Variables|/Script/Engine.Actor|GetRootComponent (Components|GetOwner))))
      (bind _returnvalue (Game|AddComponentbyClass (Components|GetOwner) (Utilities|GetClass _output_get) false))
      (bind _output_get_2 (LocalVariables|SetLocalCloneRoot _returnvalue))
      (Transformation|SetMobility _output_get_2 "Movable")
      (Clone|CopyMeshfromComponenttoComponent (LocalVariables|GetLocalOwnerRoot) (LocalVariables|GetLocalCloneRoot))
      (bind _output_get_3 (LocalVariables|SetLocalTempComponent (Variables|/Script/Engine.Actor|GetRootComponent (Components|GetOwner))))
      (bind _output_get_4 (LocalVariables|SetLocalTempChildrenComponents (Components|GetChildrenComponents _output_get_3 false)))
      (for _array_element _output_get_4
        (if (!= (Utilities|GetClass _array_element) "/Game/Puzzle_Template/zIgnore/Assets/Lasers/PT_Laser_BP.PT_Laser_BP_C")
          (bind _returnvalue_2 (Game|AddComponentbyClass (Components|GetOwner) (Utilities|GetClass _array_element) false (Transformation|GetRelativeTransform _array_element)))
          (Transformation|SetMobility _returnvalue_2 "Movable")
          (Clone|CopyMeshfromComponenttoComponent _array_element _returnvalue_2)
          (Transformation|AttachComponentToComponent _returnvalue_2 (LocalVariables|GetLocalCloneRoot) "None" "KeepWorld" "KeepWorld" "KeepWorld" true)))
      (Rendering|SetVisibility (LocalVariables|GetLocalCloneRoot) Visibility true)
      (return (LocalVariables|GetLocalCloneRoot)))))

(fn DestroyClone
  (Utilities|IsValid (Variables|Default|GetClone%20Root)
    (:Is%20Valid
      (Transformation|DetachFromComponent (Variables|Default|GetClone%20Root) "KeepRelative" "KeepRelative" "KeepRelative" false)
      (Components|DestroyComponent (Variables|Default|GetClone%20Root))
      (Variables|Default|SetClone%20Root 0))))

(fn CopyMeshfromComponenttoComponent
  (params (A :type Scene%20Component%20Object%20Reference) (B :type Scene%20Component%20Object%20Reference))
  (bind _asprimitive_component (Utilities|Casting|CastToPrimitiveComponent B))
  (Collision|SetCollisionObjectType _asprimitive_component "ECC_GameTraceChannel4")
  (Collision|SetCollisionEnabled _asprimitive_component "QueryOnly")
  (Collision|SetCollisionResponsetoAllChannels _asprimitive_component "ECR_Ignore")
  (Collision|SetCollisionResponsetoChannel _asprimitive_component "ECC_GameTraceChannel3" "ECR_Block")
  (bind _asstatic_mesh_component (Utilities|Casting|CastToStaticMeshComponent A)
    (:then
      (bind _asstatic_mesh_component_2 (Utilities|Casting|CastToStaticMeshComponent B))
      (Components|StaticMesh|SetStaticMesh _asstatic_mesh_component_2 (Variables|/Script/Engine.StaticMeshComponent|GetStaticMesh _asstatic_mesh_component))
      (Rendering|SetRenderCustomDepth _asstatic_mesh_component_2 (Variables|/Script/Engine.PrimitiveComponent|GetbRenderCustomDepth _asstatic_mesh_component))
      (Rendering|SetCustomDepthStencilValue _asstatic_mesh_component_2 (Variables|/Script/Engine.PrimitiveComponent|GetCustomDepthStencilValue _asstatic_mesh_component))
      (bind _output_get (Variables|/Script/Engine.ActorComponent|SetComponentTags _asstatic_mesh_component_2 (Variables|/Script/Engine.ActorComponent|GetComponentTags _asstatic_mesh_component)))
      (for (_array_element _array_index) (Rendering|Material|GetMaterials _asstatic_mesh_component)
        (if (Utilities|Array|ContainsItem _output_get "Instance")
          (bind _returnvalue (Rendering|Material|GetBaseMaterial _array_element))
          (Rendering|Material|SetMaterial _asstatic_mesh_component_2 _array_index _returnvalue)
          (else
            (Rendering|Material|SetMaterial _asstatic_mesh_component_2 _array_index _array_element)))))
    (:CastFailed
      (bind _asskeletal_mesh_component (Utilities|Casting|CastToSkeletalMeshComponent A))
      (bind _asskeletal_mesh_component_2 (Utilities|Casting|CastToSkeletalMeshComponent B))
      (Components|SkinnedMesh|SetSkinnedAssetandUpdate _asskeletal_mesh_component_2 (Class|SkinnedMeshComponent|GetSkinnedAsset _asskeletal_mesh_component) true)
      (Rendering|SetRenderCustomDepth _asskeletal_mesh_component_2 (Variables|/Script/Engine.PrimitiveComponent|GetbRenderCustomDepth _asskeletal_mesh_component))
      (Rendering|SetCustomDepthStencilValue _asskeletal_mesh_component_2 (Variables|/Script/Engine.PrimitiveComponent|GetCustomDepthStencilValue _asskeletal_mesh_component))
      (bind _output_get_2 (Variables|/Script/Engine.ActorComponent|SetComponentTags _asskeletal_mesh_component_2 (Variables|/Script/Engine.ActorComponent|GetComponentTags _asskeletal_mesh_component)))
      (for (_array_element_2 _array_index_2) (Rendering|Material|GetMaterials _asskeletal_mesh_component)
        (if (Utilities|Array|ContainsItem _output_get_2 "Instance")
          (bind _returnvalue_2 (Rendering|Material|GetBaseMaterial _array_element_2))
          (Rendering|Material|SetMaterial _asskeletal_mesh_component_2 _array_index_2 _returnvalue_2)
          (else
            (Rendering|Material|SetMaterial _asskeletal_mesh_component_2 _array_index_2 _array_element_2)))))))

(fn SetIsinPortalRange
  (params (Portal :type BP%20Portal%20Object%20Reference))
  (Variables|Runtime|SetIn%20Portal Portal)
  (Variables|Runtime|SetOut%20Portal (Variables|/Game/Puzzle_Template/Portals/BP_Portal.BP_Portal_C|GetLinked%20Portal%20Ref Portal))
  (Variables|Runtime|SetIs%20In%20Portal%20Range? true)
  (Rendering|SetVisibility (Variables|Default|GetClone%20Root) true true)
  (ClipPlane|EnableMeshPortalClippingPlane (Variables|/Script/Engine.Actor|GetRootComponent (Components|GetOwner)) (Variables|Runtime|GetIn%20Portal))
  (ClipPlane|EnableMeshPortalClippingPlane (Variables|Default|GetClone%20Root) (Variables|Runtime|GetOut%20Portal))
  (Portals|UpdateClonePositionThroughPortals)
  (Default|CallInPortalRange))

(fn SetIsNotinPortalRange
  (Variables|Runtime|SetIs%20In%20Portal%20Range? false)
  (Variables|Runtime|SetIn%20Portal 0)
  (Variables|Runtime|SetOut%20Portal 0)
  (Rendering|SetVisibility (Variables|Default|GetClone%20Root) false true)
  (ClipPlane|DisableMeshPortalClippingPlane (Variables|/Script/Engine.Actor|GetRootComponent (Components|GetOwner)))
  (Default|CallNotinPortalRange))

(fn UpdateClonePositionThroughPortals
  (Transformation|SetWorldLocationAndRotation (Variables|Default|GetClone%20Root) (Math|Transform|TransformLocation (Transformation|GetActorTransform (Variables|Runtime|GetOut%20Portal)) (Math|Transform|InverseTransformLocation (Transformation|GetWorldTransform (Variables|/Game/Puzzle_Template/Portals/BP_Portal.BP_Portal_C|GetBack (Variables|Runtime|GetIn%20Portal))) (Transformation|GetActorLocation (Components|GetOwner)))) (Math|Transform|TransformRotation (Transformation|GetActorTransform (Variables|Runtime|GetOut%20Portal)) (Math|Transform|InverseTransformRotation (Transformation|GetWorldTransform (Variables|/Game/Puzzle_Template/Portals/BP_Portal.BP_Portal_C|GetBack (Variables|Runtime|GetIn%20Portal))) (Transformation|GetActorRotation (Components|GetOwner)))) false false))

(fn TeleportActor
  (if (not (Variables|Runtime|GetIgnore%20Portals?))
    (if (and (Utilities|IsValid (Variables|Runtime|GetIn%20Portal)) (Utilities|IsValid (Variables|Runtime|GetOut%20Portal)))
      (bind (_returnvalue _character) (Utilities|IsAttachedtoCharacter?))
      (if _returnvalue
        (LocalVariables|SetLocal%20Character _character)
        (bind (_valid_ _new_location _new_rotation _new_control_rotation _new_velocity) (Utilities|CalculateTeleportCharacterEndTransform&Velocity (Variables|Runtime|GetIn%20Portal) (Variables|Runtime|GetOut%20Portal) (LocalVariables|GetLocal%20Character) (Variables|Settings|GetMin%20Character%20Velocity) (Variables|Settings|GetMax%20Character%20Velocity)))
        (if _valid_
          (Transformation|SetActorLocationAndRotation (LocalVariables|GetLocal%20Character) _new_location _new_rotation false true)
          (Pawn|SetControlRotation (Pawn|GetController (LocalVariables|GetLocal%20Character)) _new_control_rotation)
          (CallFunction|UpdateCharacterVelocity _new_velocity (LocalVariables|GetLocal%20Character))
          (Default|CallTeleported (Components|GetOwner) :!label _label)
          (return true))
        (else
          (LocalVariables|SetLocal%20Actor (Components|GetOwner))
          (bind (_valid__2 _new_location_2 _new_rotation_2 _new_velocity_2 _new_angular_velocity) (Utilities|CalculateTeleportActorEndTransform&Velocity (Variables|Runtime|GetIn%20Portal) (Variables|Runtime|GetOut%20Portal) (LocalVariables|GetLocal%20Actor) (Variables|Settings|GetMin%20Actor%20Velocity) (Variables|Settings|GetMax%20Actor%20Velocity)))
          (if _valid__2
            (Transformation|SetActorLocationAndRotation (LocalVariables|GetLocal%20Actor) _new_location_2 _new_rotation_2 false true)
            (bind _asprimitive_component (Utilities|Casting|CastToPrimitiveComponent (Variables|/Script/Engine.Actor|GetRootComponent (LocalVariables|GetLocal%20Actor))))
            (Physics|SetPhysicsLinearVelocity _asprimitive_component _new_velocity_2 false "None")
            (Class|PrimitiveComponent|SetPhysicsAngularVelocityinDegrees _asprimitive_component _new_angular_velocity false "None")
            (goto _label)))))))

(fn CalculateTeleportCharacterEndTransform&Velocity
  (params (In%20Portal :type BP%20Portal%20Object%20Reference) (Out%20Portal :type BP%20Portal%20Object%20Reference) (Character :type Character%20Object%20Reference) (Min%20Velocity :type Float%20%28double-precision%29) (Max%20Velocity :type Float%20%28double-precision%29))
  (bind _returnvalue (Transformation|GetActorTransform In%20Portal))
  (bind _rotation (Math|Transform|BreakTransform _returnvalue))
  (bind _pitch (Math|Rotator|BreakRotator _rotation))
  (Utilities|IsValid In%20Portal
    (:Is%20Valid
      (if (Default|IsLinkedPortalActive? In%20Portal)
        (LocalVariables|SetLocalPortalATransform (Transformation|GetWorldTransform (Variables|/Game/Puzzle_Template/Portals/BP_Portal.BP_Portal_C|GetBack In%20Portal)))
        (LocalVariables|SetLocalPortalBTransform (Transformation|GetActorTransform Out%20Portal))
        (LocalVariables|SetLocalNewLocation (- (Math|Transform|TransformLocation (LocalVariables|GetLocalPortalBTransform) (Math|Transform|InverseTransformLocation (LocalVariables|GetLocalPortalATransform) (+ (Transformation|GetActorLocation Character) (* (Transformation|GetVelocity Character) (Utilities|Time|GetWorldDeltaSeconds))))) (Math|Vector|SelectVector (* (Math|Vector|GetUpVector (Math|Rotator|MakeRotator (Math|Float|SelectFloat (.Roll (Math|Rotator|BreakRotator (.Rotation (Math|Transform|BreakTransform (LocalVariables|GetLocalPortalBTransform))))) 0.0 (== (Math|Float|SnapToGrid(Float) (Math|Float|Absolute(Float) (+ _pitch (.Pitch (Math|Rotator|BreakRotator (.Rotation (Math|Transform|BreakTransform (LocalVariables|GetLocalPortalBTransform))))))) 1.0) 9e+01)) (Math|Float|SelectFloat 0.0 (+ _pitch (.Pitch (Math|Rotator|BreakRotator (.Rotation (Math|Transform|BreakTransform (LocalVariables|GetLocalPortalBTransform)))))) (== (Math|Float|SnapToGrid(Float) (+ _pitch (.Pitch (Math|Rotator|BreakRotator (.Rotation (Math|Transform|BreakTransform (LocalVariables|GetLocalPortalBTransform)))))) 1.0) 1.8e+02)) (.Yaw (Math|Rotator|BreakRotator (.Rotation (Math|Transform|BreakTransform (LocalVariables|GetLocalPortalBTransform))))))) (* (.Z (Math|Vector|BreakVector (Variables|/Script/Engine.SceneComponent|GetRelativeLocation (Actor|GetComponentbyClass Character "/Script/Engine.CameraComponent")))) 2.0)) "0, 0, 0" (== (Math|Float|SnapToGrid(Float) (+ _pitch (.Pitch (Math|Rotator|BreakRotator (.Rotation (Math|Transform|BreakTransform (LocalVariables|GetLocalPortalBTransform)))))) 1.0) 1.8e+02))))
        (LocalVariables|SetLocalNewRotation (Math|Rotator|MakeRotator (Math|Float|SelectFloat (.Roll (Math|Rotator|BreakRotator (.Rotation (Math|Transform|BreakTransform (LocalVariables|GetLocalPortalBTransform))))) 0.0 (== (Math|Float|SnapToGrid(Float) (Math|Float|Absolute(Float) (+ _pitch (.Pitch (Math|Rotator|BreakRotator (.Rotation (Math|Transform|BreakTransform (LocalVariables|GetLocalPortalBTransform))))))) 1.0) 9e+01)) (Math|Float|SelectFloat 0.0 (+ _pitch (.Pitch (Math|Rotator|BreakRotator (.Rotation (Math|Transform|BreakTransform (LocalVariables|GetLocalPortalBTransform)))))) (== (Math|Float|SnapToGrid(Float) (+ _pitch (.Pitch (Math|Rotator|BreakRotator (.Rotation (Math|Transform|BreakTransform (LocalVariables|GetLocalPortalBTransform)))))) 1.0) 1.8e+02)) (.Yaw (Math|Rotator|BreakRotator (.Rotation (Math|Transform|BreakTransform (LocalVariables|GetLocalPortalBTransform)))))))
        (LocalVariables|SetLocalNewControlRotation (Math|Transform|TransformRotation (LocalVariables|GetLocalPortalBTransform) (Math|Transform|InverseTransformRotation (LocalVariables|GetLocalPortalATransform) (Pawn|GetControlRotation (Pawn|GetController Character) :!class /Script/Engine.Controller))))
        (if (> (Math|Float|Truncate (Math|Float|Absolute(Float) (.Pitch (Math|Rotator|BreakRotator (.Rotation (Math|Transform|BreakTransform (LocalVariables|GetLocalPortalBTransform))))))) 0)
          (LocalVariables|SetLocalNewVelocity (Math|Vector|VectorClampSizeMax (+ (Math|Transform|TransformDirection (LocalVariables|GetLocalPortalBTransform) (Math|Transform|InverseTransformDirection (LocalVariables|GetLocalPortalATransform) (Transformation|GetVelocity Character))) (* (Math|Vector|GetForwardVector (.Rotation (Math|Transform|BreakTransform (LocalVariables|GetLocalPortalBTransform)))) (Math|Float|Max(Float) (- (* (Math|Float|MapRangeClamped (Math|Float|Absolute(Float) (.Pitch (Math|Rotator|BreakRotator (.Rotation (Math|Transform|BreakTransform (LocalVariables|GetLocalPortalBTransform)))))) 0.0 9e+01 0.25 1.0) Min%20Velocity) (Math|Vector|VectorLength (Math|Transform|TransformDirection (LocalVariables|GetLocalPortalBTransform) (Math|Transform|InverseTransformDirection (LocalVariables|GetLocalPortalATransform) (Transformation|GetVelocity Character))))) 0.0))) Max%20Velocity))
          (else
            (LocalVariables|SetLocalNewVelocity (Math|Vector|VectorClampSizeMax (Math|Transform|TransformDirection (LocalVariables|GetLocalPortalBTransform) (Math|Transform|InverseTransformDirection (LocalVariables|GetLocalPortalATransform) (Transformation|GetVelocity Character))) Max%20Velocity))))
        (return true (LocalVariables|GetLocalNewLocation) (LocalVariables|GetLocalNewRotation) (LocalVariables|GetLocalNewControlRotation) (LocalVariables|GetLocalNewVelocity))
        (else
          (return false (LocalVariables|GetLocalNewLocation) (LocalVariables|GetLocalNewRotation) (LocalVariables|GetLocalNewControlRotation) (LocalVariables|GetLocalNewVelocity)))))))

(fn CalculateTeleportActorEndTransform&Velocity
  (params (In%20Portal :type BP%20Portal%20Object%20Reference) (Out%20Portal :type BP%20Portal%20Object%20Reference) (Actor :type Actor%20Object%20Reference) (Min%20Velocity :type Float%20%28double-precision%29) (Max%20Velocity :type Float%20%28double-precision%29))
  (if (Default|IsLinkedPortalActive? In%20Portal)
    (LocalVariables|SetLocalPortalATransform (Transformation|GetWorldTransform (Variables|/Game/Puzzle_Template/Portals/BP_Portal.BP_Portal_C|GetBack In%20Portal)))
    (LocalVariables|SetLocalPortalBTransform (Transformation|GetActorTransform Out%20Portal))
    (LocalVariables|SetLocalNewLocation (Math|Transform|TransformLocation (LocalVariables|GetLocalPortalBTransform) (Math|Transform|InverseTransformLocation (LocalVariables|GetLocalPortalATransform) (Transformation|GetActorLocation Actor))))
    (LocalVariables|SetLocalNewRotation (Math|Transform|TransformRotation (LocalVariables|GetLocalPortalBTransform) (Math|Transform|InverseTransformRotation (LocalVariables|GetLocalPortalATransform) (Transformation|GetActorRotation Actor))))
    (bind _asprimitive_component (Utilities|Casting|CastToPrimitiveComponent (Variables|/Script/Engine.Actor|GetRootComponent Actor)))
    (bind _returnvalue (Physics|GetPhysicsLinearVelocity _asprimitive_component "None"))
    (LocalVariables|SetLocalNewLinearVelocity (Math|Vector|ClampVectorSize (Math|Transform|TransformDirection (LocalVariables|GetLocalPortalBTransform) (Math|Transform|InverseTransformDirection (LocalVariables|GetLocalPortalATransform) _returnvalue)) (* Min%20Velocity (Math|Float|MapRangeClamped (Math|Float|Absolute(Float) (.Pitch (Math|Rotator|BreakRotator (.Rotation (Math|Transform|BreakTransform (LocalVariables|GetLocalPortalBTransform)))))) 0.0 9e+01 0.25 1.0)) Max%20Velocity))
    (LocalVariables|SetLocalNewAngularVelocity (Math|Transform|TransformDirection (LocalVariables|GetLocalPortalBTransform) (Math|Transform|InverseTransformDirection (LocalVariables|GetLocalPortalATransform) (Physics|GetPhysicsAngularVelocityinDegrees _asprimitive_component "None"))))
    (return true (LocalVariables|GetLocalNewLocation) (LocalVariables|GetLocalNewRotation) (LocalVariables|GetLocalNewLinearVelocity) (LocalVariables|GetLocalNewAngularVelocity))
    (else
      (return false (LocalVariables|GetLocalNewLocation) (LocalVariables|GetLocalNewRotation) (LocalVariables|GetLocalNewLinearVelocity) (LocalVariables|GetLocalNewAngularVelocity)))))

(fn EnableMeshPortalClippingPlane
  (params (Root%20Component :type Scene%20Component%20Object%20Reference) (Portal :type BP%20Portal%20Object%20Reference))
  (bind _returnvalue (Transformation|GetActorForwardVector Portal))
  (LocalVariables|SetLocalComponents (Components|GetChildrenComponents Root%20Component true))
  (Utilities|Array|Add (LocalVariables|GetLocalComponents) Root%20Component)
  (for _array_element (LocalVariables|GetLocalComponents)
    (bind _asmesh_component (Utilities|Casting|CastToMeshComponent _array_element))
    (Rendering|Material|SetVectorParameterValueonMaterials _asmesh_component "Plane Position" (+ (Transformation|GetActorLocation Portal) (* _returnvalue -1.0)))
    (Rendering|Material|SetVectorParameterValueonMaterials _asmesh_component "Plane Normal" _returnvalue)
    (Rendering|Material|SetScalarParameterValueonMaterials _asmesh_component "Enable Clip Plane" 1.0)))

(fn DisableMeshPortalClippingPlane
  (params (Root%20Component :type Scene%20Component%20Object%20Reference))
  (LocalVariables|SetLocalComponents (Components|GetChildrenComponents Root%20Component true))
  (Utilities|Array|Add (LocalVariables|GetLocalComponents) Root%20Component)
  (for _array_element (LocalVariables|GetLocalComponents)
    (bind _asmesh_component (Utilities|Casting|CastToMeshComponent _array_element))
    (Rendering|Material|SetScalarParameterValueonMaterials _asmesh_component "Enable Clip Plane" 0.0)))

(fn RefreshPortalsCapture
  (Utilities|FlowControl|Sequence
    (:then_0
      (bind _out_portal (Variables|Runtime|GetOut%20Portal)
        (:then
          (if (not (Variables|/Game/Puzzle_Template/Portals/BP_Portal.BP_Portal_C|GetIs%20Disabled? _out_portal))
            (Default|UpdateCapture2DLocation&Rotation _out_portal false)
            (Rendering|SceneCapture|CaptureScene (Variables|/Game/Puzzle_Template/Portals/BP_Portal.BP_Portal_C|GetCapture%202D _out_portal) :!class /Script/Engine.SceneCaptureComponent2D)))
        (:else)))
    (:then_1
      (bind _in_portal (Variables|Runtime|GetIn%20Portal)
        (:then
          (if (not (Variables|/Game/Puzzle_Template/Portals/BP_Portal.BP_Portal_C|GetIs%20Disabled? _in_portal))
            (Default|UpdateCapture2DLocation&Rotation _in_portal false)
            (Rendering|SceneCapture|CaptureScene (Variables|/Game/Puzzle_Template/Portals/BP_Portal.BP_Portal_C|GetCapture%202D _in_portal) :!class /Script/Engine.SceneCaptureComponent2D)))
        (:else)))))

(fn GetIgnorePortals
  (return (Variables|Runtime|GetIgnore%20Portals?)))

(fn RefreshMeshPortalClippingPlane
  (ClipPlane|EnableMeshPortalClippingPlane (Variables|/Script/Engine.Actor|GetRootComponent (Components|GetOwner)) (Variables|Runtime|GetIn%20Portal))
  (ClipPlane|EnableMeshPortalClippingPlane (Variables|Default|GetClone%20Root) (Variables|Runtime|GetOut%20Portal)))

(fn ApplyCloneCollisionForces
  (LocalVariables|SetLocalPortalATransform (Transformation|GetWorldTransform (Variables|/Game/Puzzle_Template/Portals/BP_Portal.BP_Portal_C|GetBack (Variables|Runtime|GetIn%20Portal))))
  (LocalVariables|SetLocalPortalBTransform (Transformation|GetActorTransform (Variables|Runtime|GetOut%20Portal)))
  (bind (_returnvalue _character) (Utilities|IsAttachedtoCharacter?))
  (if _returnvalue
    (bind _output_get (LocalVariables|SetLocal%20Character _character))
    (bind (_outactors _returnvalue_2) (Collision|CapsuleOverlapActors (Math|Transform|TransformLocation (LocalVariables|GetLocalPortalBTransform) (Math|Transform|InverseTransformLocation (LocalVariables|GetLocalPortalATransform) (Transformation|GetActorLocation _output_get))) (+ (.OutRadius (Components|Capsule|GetScaledCapsuleSize (Variables|/Script/Engine.Character|GetCapsuleComponent _output_get))) 1.0) (.OutHalfHeight (Components|Capsule|GetScaledCapsuleSize (Variables|/Script/Engine.Character|GetCapsuleComponent _output_get))) (Utilities|Array|MakeArray "ObjectTypeQuery4" "ObjectTypeQuery3") "/Script/Engine.Actor" (Utilities|Array|MakeArray (LocalVariables|GetLocal%20Character))))
    (if _returnvalue_2
      (for _array_element _outactors
        (if (>= (Math|Vector|DotProduct (Math|Vector|Normalize (- (Transformation|GetActorLocation _array_element) (Transformation|GetActorLocation (Variables|Runtime|GetOut%20Portal)))) (Transformation|GetActorForwardVector (Variables|Runtime|GetOut%20Portal))) 0.0)
          (Transformation|AddActorWorldOffset _array_element (* (Math|Transform|TransformDirection (LocalVariables|GetLocalPortalBTransform) (Math|Transform|InverseTransformDirection (LocalVariables|GetLocalPortalATransform) (Transformation|GetVelocity (LocalVariables|GetLocal%20Character)))) (Utilities|Time|GetWorldDeltaSeconds))))))
    (else
      (bind _output_get_2 (LocalVariables|SetLocal%20Actor (Components|GetOwner)))
      (bind _asprimitive_component (Utilities|Casting|CastToPrimitiveComponent (Variables|/Script/Engine.Actor|GetRootComponent _output_get_2)))
      (bind _outactors_2 (Collision|ComponentOverlapActors _asprimitive_component (Math|Transform|MakeTransform (Math|Transform|TransformLocation (LocalVariables|GetLocalPortalBTransform) (Math|Transform|InverseTransformLocation (LocalVariables|GetLocalPortalATransform) (Transformation|GetActorLocation _output_get_2))) (Transformation|GetWorldRotation (Variables|/Script/Engine.Actor|GetRootComponent _output_get_2)) (Transformation|GetWorldScale (Variables|/Script/Engine.Actor|GetRootComponent _output_get_2))) (Utilities|Array|MakeArray "ObjectTypeQuery4" "ObjectTypeQuery3") "/Script/Engine.Actor" (Utilities|Array|MakeArray (LocalVariables|GetLocal%20Actor))))
      (for _array_element_2 _outactors_2
        (if (>= (Math|Vector|DotProduct (Math|Vector|Normalize (- (Transformation|GetActorLocation _array_element_2) (Transformation|GetActorLocation (Variables|Runtime|GetOut%20Portal)))) (Transformation|GetActorForwardVector (Variables|Runtime|GetOut%20Portal))) 0.0)
          (Transformation|AddActorWorldOffset _array_element_2 (* (Math|Transform|TransformDirection (LocalVariables|GetLocalPortalBTransform) (Math|Transform|InverseTransformDirection (LocalVariables|GetLocalPortalATransform) (Transformation|GetVelocity (LocalVariables|GetLocal%20Actor)))) (Utilities|Time|GetWorldDeltaSeconds))))))))