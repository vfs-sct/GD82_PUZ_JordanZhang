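; Portal gun component that spawns two linked, initially disabled portals and an optional dynamic crosshair widget on begin play.
; TrySpawnPortal traces from the owner's camera for a portal-wall surface, then moves and enables the chosen portal with a camera shake.
; Placement uses multi-pass sphere traces to nudge the portal inside wall edges and away from obstacles or the other portal, then validates nine points.
; Helpers clear portals and fade the crosshair.
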(event Custom|Try%20Spawn%20Portal
  (params (Portal%20Index :type Integer))
  (bind _portal_1 (Variables|Runtime|GetPortal%201))
  (bind _portal_2 (Variables|Runtime|GetPortal%202))
  (bind _returnvalue (Utilities|Select :Index Portal%20Index :Option%200 _portal_1 :Option%201 _portal_2))
  ;[0 0 0] Check if we can place a teleport and adjust its position to fit it to the wall we are looking at.
  (bind (_valid_ _location _rotation) (CallFunction|FindValidPortalSpawnLocation Portal%20Index (Variables|Settings|GetPortals%20Size) (Variables|Settings|GetPortals%20Grid%20Snapping)))
  (if _valid_
    (Default|UpdatePortalLocation&Rotation _returnvalue _location _rotation)
    (Default|Disable/EnablePortal _returnvalue true)
    (Game|Feedback|ClientStartCameraShake (Game|GetPlayerController 0) "/Game/Puzzle_Template/Portals/Portal_Gun/PT_Portal_Gun_Fire_CS.PT_Portal_Gun_Fire_CS_C" 1.0 "CameraLocal" "0, 0, 0")))

(event EventBeginPlay
  ;[0 0 0] On Begin Play, Initialize Portals
  (CallFunction|InitializePortals))

(fn InitializePortals
  (bind _returnvalue (Game|SpawnActorfromClass "/Game/Puzzle_Template/Portals/BP_Portal.BP_Portal_C" (Math|Transform|MakeTransform "0, 0, 0" "0, 0, 0" "1.000000,1.000000,1.000000") "AlwaysSpawn" "OverrideRootScale" (Components|GetOwner) 0 (Variables|Settings|GetPortals%20Quality) (Variables|Settings|GetPortals%20Size) (Variables|Settings|GetEnable%20Portal%20Funnel?) 0))
  (bind _output_get (Variables|Runtime|SetPortal%201 _returnvalue))
  (Default|Disable/EnablePortal _output_get false)
  (bind _returnvalue_2 (Game|SpawnActorfromClass "/Game/Puzzle_Template/Portals/BP_Portal.BP_Portal_C" (Math|Transform|MakeTransform "0, 0, 0" "0, 0, 0" "1.000000,1.000000,1.000000") "AlwaysSpawn" "OverrideRootScale" (Components|GetOwner) 1 (Variables|Settings|GetPortals%20Quality) (Variables|Settings|GetPortals%20Size) (Variables|Settings|GetEnable%20Portal%20Funnel?) 0))
  (bind _output_get_2 (Variables|Runtime|SetPortal%202 _returnvalue_2))
  (Default|Disable/EnablePortal _output_get_2 false)
  (Default|UpdateLinkedPortalReference (Variables|Runtime|GetPortal%201) (Variables|Runtime|GetPortal%202))
  (Default|UpdateLinkedPortalReference (Variables|Runtime|GetPortal%202) (Variables|Runtime|GetPortal%201))
  (if (Variables|Settings|GetEnable%20Portal%20Gun%20Dynamic%20Crosshair?)
    (bind _returnvalue_3 (UserInterface|CreateWidget "/Game/Puzzle_Template/Portals/Portal_Gun/Widgets/PT_Portal_Gun_Crosshair_W.PT_Portal_Gun_Crosshair_W_C" 0 self))
    (bind _output_get_3 (Variables|Runtime|SetPortal%20Gun%20Crosshair%20Ref _returnvalue_3))
    (UserInterface|Viewport|AddtoViewport _output_get_3 0)))

(fn ClearPortals
  (bind _portal_gun_crosshair_ref (Variables|Runtime|GetPortal%20Gun%20Crosshair%20Ref))
  (Default|DeactivateAnim (Variables|Runtime|GetPortal%201) true)
  (UserInterface|Animation|PlayAnimation _portal_gun_crosshair_ref (Variables|/Game/Puzzle_Template/Portals/Portal_Gun/Widgets/PT_Portal_Gun_Crosshair_W.PT_Portal_Gun_Crosshair_W_C|GetPortal_Crosshair_Clear _portal_gun_crosshair_ref) 0.0 1 "Forward" 1.0 false))

(fn FindValidPortalSpawnLocation
  (params (Portal%20Index :type Integer) (Portal%20Size :type Vector%202D%20Structure :default "(X=50.000000,Y=100.000000)") (Grid%20Snap :type Float%20%28double-precision%29))
  (bind _array (Utilities|Array|MakeArray "(X=0.000000,Y=1.000000)" "(X=0.000000,Y=-1.000000)"))
  (bind _array_2 (Utilities|Array|MakeArray "(X=1.000000,Y=0.000000)" "(X=-1.000000,Y=0.000000)"))
  (bind _camera (Utilities|GetCameraReference)
    (:%20%20
      (bind (_outhit _returnvalue) (Collision|LineTraceForObjects (Transformation|GetWorldLocation _camera) (+ (Transformation|GetWorldLocation _camera) (* (Math|Vector|GetForwardVector _camera) 1e+04)) (Utilities|Array|MakeArray "ObjectTypeQuery9" "ObjectTypeQuery7" "ObjectTypeQuery1" "ObjectTypeQuery2") true (Utilities|Array|MakeArray (Utilities|Select :Index Portal%20Index :Option%200 (Variables|Runtime|GetPortal%201) :Option%201 (Variables|Runtime|GetPortal%202))) "None"))
      (bind _output_get (LocalVariables|SetLocalHit _outhit))
      (if _returnvalue
        (if (and (== (.PhysMat (Collision|BreakHitResult _output_get)) "/Game/Puzzle_Template/zIgnore/Materials/Physical_Materials/PT_Portal_Wall_PM.PT_Portal_Wall_PM") (or (Utilities|Enum|Equal(Enum) (Collision|GetCollisionObjectType (.HitComponent (Collision|BreakHitResult _output_get))) "ECC_GameTraceChannel6") (Utilities|Enum|Equal(Enum) (Collision|GetCollisionObjectType (.HitComponent (Collision|BreakHitResult _output_get))) "ECC_GameTraceChannel1")))
          (LocalVariables|SetLocalFinalLocation (.Location (|ResolveDesiredPortalLoc&Rot (LocalVariables|GetLocalHit))))
          (LocalVariables|SetLocalFinalRotation (.Rotation (|ResolveDesiredPortalLoc&Rot (LocalVariables|GetLocalHit))))
          (Utilities|FlowControl|Sequence
            (:then_0
              ;[0 0 0] Try to snap the portal to stay within the wall bounds (Up / Down - Right / Left)
              (for _array_element (Utilities|Array|MakeArray "(X=0.000000,Y=1.000000)" "(X=0.000000,Y=-1.000000)" "(X=1.000000,Y=0.000000)" "(X=-1.000000,Y=0.000000)")
                (bind (_outhit_2 _returnvalue_2) (Collision|SphereTraceForObjects (+ (+ (Math|Vector|RotateVector (Math|Vector|MakeVector 0.0 (.X (Math|Vector2D|BreakVector2D (* _array_element Portal%20Size))) (.Y (Math|Vector2D|BreakVector2D (* _array_element Portal%20Size)))) (LocalVariables|GetLocalFinalRotation)) (LocalVariables|GetLocalFinalLocation)) (* (Math|Vector|GetForwardVector (Math|Conversions|RotationFromXVector (.Normal (Collision|BreakHitResult (LocalVariables|GetLocalHit))))) 2.0)) (+ (+ (Math|Vector|RotateVector (Math|Vector|MakeVector 0.0 (.X (Math|Vector2D|BreakVector2D (* _array_element Portal%20Size))) (.Y (Math|Vector2D|BreakVector2D (* _array_element Portal%20Size)))) (LocalVariables|GetLocalFinalRotation)) (LocalVariables|GetLocalFinalLocation)) (* (Math|Vector|GetForwardVector (Math|Conversions|RotationFromXVector (.Normal (Collision|BreakHitResult (LocalVariables|GetLocalHit))))) -2.0)) 0.01 (Utilities|Array|MakeArray "ObjectTypeQuery9" "ObjectTypeQuery7") true 0 "None"))
                (if (not _returnvalue_2)
                  (bind (_outhit_3 _returnvalue_3) (Collision|SphereTraceForObjects (.TraceEnd (Collision|BreakHitResult _outhit_2)) (+ (.TraceEnd (Collision|BreakHitResult _outhit_2)) (Math|Vector|RotateVector (Math|Vector|MakeVector 0.0 (.X (Math|Vector2D|BreakVector2D (* (* _array_element -1.0) (+ Portal%20Size 2.0)))) (.Y (Math|Vector2D|BreakVector2D (* (* _array_element -1.0) (+ Portal%20Size 2.0))))) (LocalVariables|GetLocalFinalRotation))) 0.01 (Utilities|Array|MakeArray "ObjectTypeQuery9" "ObjectTypeQuery7") true 0 "None" :!label _label))
                  (if _returnvalue_3
                    (LocalVariables|SetLocalFinalLocation (+ (LocalVariables|GetLocalFinalLocation) (* (Math|Vector|GetUnitDirection(Vector) (.TraceStart (Collision|BreakHitResult _outhit_3)) (.TraceEnd (Collision|BreakHitResult _outhit_3))) (.Distance (Collision|BreakHitResult _outhit_3))))))
                  (elif (Math|Vector|NotEqual(Vector) (.Normal (Collision|BreakHitResult _outhit_2)) (.Normal (Collision|BreakHitResult (LocalVariables|GetLocalHit))) 0.1)
                    (goto _label))))
              ;[0 0 0] Try to snap the portal to stay within the wall bounds (Top Left / Top Right - Bottom Left / Bottom Right)
              (for (_array_element_2 _array_index) (Utilities|Array|MakeArray "(X=-1.000000,Y=1.000000)" "(X=1.000000,Y=1.000000)" "(X=-1.000000,Y=-1.000000)" "(X=1.000000,Y=-1.000000)")
                (bind (_outhit_4 _returnvalue_4) (Collision|SphereTraceForObjects (+ (+ (Math|Vector|RotateVector (Math|Vector|MakeVector 0.0 (.X (Math|Vector2D|BreakVector2D (* _array_element_2 Portal%20Size))) (.Y (Math|Vector2D|BreakVector2D (* _array_element_2 Portal%20Size)))) (LocalVariables|GetLocalFinalRotation)) (LocalVariables|GetLocalFinalLocation)) (* (Math|Vector|GetForwardVector (Math|Conversions|RotationFromXVector (.Normal (Collision|BreakHitResult (LocalVariables|GetLocalHit))))) 2.0)) (+ (+ (Math|Vector|RotateVector (Math|Vector|MakeVector 0.0 (.X (Math|Vector2D|BreakVector2D (* _array_element_2 Portal%20Size))) (.Y (Math|Vector2D|BreakVector2D (* _array_element_2 Portal%20Size)))) (LocalVariables|GetLocalFinalRotation)) (LocalVariables|GetLocalFinalLocation)) (* (Math|Vector|GetForwardVector (Math|Conversions|RotationFromXVector (.Normal (Collision|BreakHitResult (LocalVariables|GetLocalHit))))) -2.0)) 0.01 (Utilities|Array|MakeArray "ObjectTypeQuery9" "ObjectTypeQuery7") true 0 "None"))
                (if (not _returnvalue_4)
                  (LocalVariables|SetLocalCornersTempOffset "0, 0, 0")
                  (for _array_element_3 (Utilities|Select :Index _array_index :Option%200 (Utilities|Array|MakeArray "(X=1.000000,Y=0.000000)" "(X=0.000000,Y=-1.000000)") :Option%201 (Utilities|Array|MakeArray "(X=-1.000000,Y=0.000000)" "(X=0.000000,Y=-1.000000)") :Option%202 (Utilities|Array|MakeArray "(X=1.000000,Y=0.000000)" "(X=0.000000,Y=1.000000)") :Option%203 (Utilities|Array|MakeArray "(X=-1.000000,Y=0.000000)" "(X=0.000000,Y=1.000000)"))
                    (bind (_outhit_5 _returnvalue_5) (Collision|SphereTraceForObjects (.TraceEnd (Collision|BreakHitResult _outhit_4)) (+ (.TraceEnd (Collision|BreakHitResult _outhit_4)) (Math|Vector|RotateVector (Math|Vector|MakeVector 0.0 (.x (* _array_element_3 (+ Portal%20Size 2.0))) (.y (* _array_element_3 (+ Portal%20Size 2.0)))) (LocalVariables|GetLocalFinalRotation))) 0.01 (Utilities|Array|MakeArray "ObjectTypeQuery9" "ObjectTypeQuery7") true 0 "None"))
                    (if _returnvalue_5
                      (if (Class|KismetMathLibrary|EqualExactlyVectorVector (LocalVariables|GetLocalCornersTempOffset) "0, 0, 0")
                        (LocalVariables|SetLocalCornersTempOffset (* (Math|Vector|GetUnitDirection(Vector) (.TraceStart (Collision|BreakHitResult _outhit_5)) (.TraceEnd (Collision|BreakHitResult _outhit_5))) (.Distance (Collision|BreakHitResult _outhit_5))))
                        (elif (< (Math|Vector|VectorLength (* (Math|Vector|GetUnitDirection(Vector) (.TraceStart (Collision|BreakHitResult _outhit_5)) (.TraceEnd (Collision|BreakHitResult _outhit_5))) (.Distance (Collision|BreakHitResult _outhit_5)))) (Math|Vector|VectorLength (LocalVariables|GetLocalCornersTempOffset)))
                          (LocalVariables|SetLocalCornersTempOffset (* (Math|Vector|GetUnitDirection(Vector) (.TraceStart (Collision|BreakHitResult _outhit_5)) (.TraceEnd (Collision|BreakHitResult _outhit_5))) (.Distance (Collision|BreakHitResult _outhit_5))))))))
                  (LocalVariables|SetLocalFinalLocation (+ (LocalVariables|GetLocalFinalLocation) (LocalVariables|GetLocalCornersTempOffset)))))
              ;[0 0 0] Try to adjust the portal location if we hit another portal / an obstacle (Up / Down - Right / Left)
              (for _array_element_4 (Utilities|Array|MakeArray "(X=1.000000,Y=0.000000)" "(X=-1.000000,Y=0.000000)" "(X=0.000000,Y=1.000000)" "(X=0.000000,Y=-1.000000)")
                (bind (_outhit_6 _returnvalue_6) (Collision|SphereTraceForObjects (+ (+ (Math|Vector|RotateVector (Math|Vector|MakeVector 0.0 (.X (Math|Vector2D|BreakVector2D _array_element_4)) (.Y (Math|Vector2D|BreakVector2D _array_element_4))) (LocalVariables|GetLocalFinalRotation)) (LocalVariables|GetLocalFinalLocation)) (* (Math|Vector|GetForwardVector (Math|Conversions|RotationFromXVector (.Normal (Collision|BreakHitResult (LocalVariables|GetLocalHit))))) -2.0)) (+ (+ (Math|Vector|RotateVector (Math|Vector|MakeVector 0.0 (.X (Math|Vector2D|BreakVector2D _array_element_4)) (.Y (Math|Vector2D|BreakVector2D _array_element_4))) (LocalVariables|GetLocalFinalRotation)) (LocalVariables|GetLocalFinalLocation)) (* (Math|Vector|GetForwardVector (Math|Conversions|RotationFromXVector (.Normal (Collision|BreakHitResult (LocalVariables|GetLocalHit))))) 2.0)) 0.01 (Utilities|Array|MakeArray "ObjectTypeQuery1" "ObjectTypeQuery2") true (Utilities|Array|MakeArray (Utilities|Select :Index Portal%20Index :Option%200 (Variables|Runtime|GetPortal%201) :Option%201 (Variables|Runtime|GetPortal%202))) "None"))
                (if (not _returnvalue_6)
                  (bind (_outhit_7 _returnvalue_7) (Collision|SphereTraceForObjects (.TraceEnd (Collision|BreakHitResult _outhit_6)) (+ (.TraceEnd (Collision|BreakHitResult _outhit_6)) (Math|Vector|RotateVector (Math|Vector|MakeVector 0.0 (.x (* (+ Portal%20Size 1.0) (* _array_element_4 -1.0))) (.y (* (+ Portal%20Size 1.0) (* _array_element_4 -1.0)))) (LocalVariables|GetLocalFinalRotation))) 0.01 (Utilities|Array|MakeArray "ObjectTypeQuery1" "ObjectTypeQuery2") true (Utilities|Array|MakeArray (Utilities|Select :Index Portal%20Index :Option%200 (Variables|Runtime|GetPortal%201) :Option%201 (Variables|Runtime|GetPortal%202))) "None"))
                  (if _returnvalue_7
                    (LocalVariables|SetLocalFinalLocation (+ (* (Math|Vector|GetUnitDirection(Vector) (.TraceStart (Collision|BreakHitResult _outhit_7)) (.TraceEnd (Collision|BreakHitResult _outhit_7))) (- (.Distance (Collision|BreakHitResult _outhit_7)) (Math|Vector|Distance(Vector) (.TraceStart (Collision|BreakHitResult _outhit_7)) (.TraceEnd (Collision|BreakHitResult _outhit_7))))) (LocalVariables|GetLocalFinalLocation))))))
              ;[0 0 0] Try to adjust the portal location if we hit another portal / an obstacle (Top Left / Top Right - Bottom Left / Bottom Right)
              (for (_array_element_5 _array_index_2) (Utilities|Array|MakeArray "(X=0.000000,Y=1.000000)" "(X=0.000000,Y=-1.000000)" "(X=1.000000,Y=0.000000)" "(X=-1.000000,Y=0.000000)")
                (for _array_element_6 (Utilities|Select :Index _array_index_2 :Option%200 _array_2 :Option%201 _array_2 :Option%202 _array :Option%203 _array)
                  (bind (_outhit_8 _returnvalue_8) (Collision|SphereTraceForObjects (+ (+ (Math|Vector|RotateVector (Math|Vector|MakeVector 0.0 (.X (Math|Vector2D|BreakVector2D _array_element_6)) (.Y (Math|Vector2D|BreakVector2D _array_element_6))) (LocalVariables|GetLocalFinalRotation)) (Math|Vector|RotateVector (Math|Vector|MakeVector 0.0 (.X (Math|Vector2D|BreakVector2D (* _array_element_5 (- Portal%20Size (Math|Float|Max(Float) Grid%20Snap 5.0))))) (.Y (Math|Vector2D|BreakVector2D (* _array_element_5 (- Portal%20Size (Math|Float|Max(Float) Grid%20Snap 5.0)))))) (LocalVariables|GetLocalFinalRotation)) (LocalVariables|GetLocalFinalLocation)) (* (Math|Vector|GetForwardVector (Math|Conversions|RotationFromXVector (.Normal (Collision|BreakHitResult (LocalVariables|GetLocalHit))))) -2.0)) (+ (+ (Math|Vector|RotateVector (Math|Vector|MakeVector 0.0 (.X (Math|Vector2D|BreakVector2D _array_element_6)) (.Y (Math|Vector2D|BreakVector2D _array_element_6))) (LocalVariables|GetLocalFinalRotation)) (Math|Vector|RotateVector (Math|Vector|MakeVector 0.0 (.X (Math|Vector2D|BreakVector2D (* _array_element_5 (- Portal%20Size (Math|Float|Max(Float) Grid%20Snap 5.0))))) (.Y (Math|Vector2D|BreakVector2D (* _array_element_5 (- Portal%20Size (Math|Float|Max(Float) Grid%20Snap 5.0)))))) (LocalVariables|GetLocalFinalRotation)) (LocalVariables|GetLocalFinalLocation)) (* (Math|Vector|GetForwardVector (Math|Conversions|RotationFromXVector (.Normal (Collision|BreakHitResult (LocalVariables|GetLocalHit))))) 2.0)) 0.01 (Utilities|Array|MakeArray "ObjectTypeQuery1" "ObjectTypeQuery2") true (Utilities|Array|MakeArray (Utilities|Select :Index Portal%20Index :Option%200 (Variables|Runtime|GetPortal%201) :Option%201 (Variables|Runtime|GetPortal%202))) "None"))
                  (if (not _returnvalue_8)
                    (bind (_outhit_9 _returnvalue_9) (Collision|SphereTraceForObjects (.TraceEnd (Collision|BreakHitResult _outhit_8)) (+ (.TraceEnd (Collision|BreakHitResult _outhit_8)) (Math|Vector|RotateVector (Math|Vector|MakeVector 0.0 (.x (* Portal%20Size (* _array_element_6 -1.0))) (.y (* Portal%20Size (* _array_element_6 -1.0)))) (LocalVariables|GetLocalFinalRotation))) 0.01 (Utilities|Array|MakeArray "ObjectTypeQuery1" "ObjectTypeQuery2") true (Utilities|Array|MakeArray (Utilities|Select :Index Portal%20Index :Option%200 (Variables|Runtime|GetPortal%201) :Option%201 (Variables|Runtime|GetPortal%202))) "None"))
                    (if _returnvalue_9
                      (LocalVariables|SetLocalFinalLocation (+ (* (Math|Vector|GetUnitDirection(Vector) (.TraceStart (Collision|BreakHitResult _outhit_9)) (.TraceEnd (Collision|BreakHitResult _outhit_9))) (- (- (.Distance (Collision|BreakHitResult _outhit_9)) 1.0) (Math|Vector|Distance(Vector) (.TraceStart (Collision|BreakHitResult _outhit_9)) (.TraceEnd (Collision|BreakHitResult _outhit_9))))) (LocalVariables|GetLocalFinalLocation)))))))
              ;[0 0 0] Final check to confirm that we are not overlapping any portal / obstacle and we are fully on a portal wall.
              (bind _array_element_7 (Utilities|Array|ForEachLoopwithBreak (Utilities|Array|MakeArray "(X=0.000000,Y=0.000000)" "(X=0.000000,Y=1.000000)" "(X=0.000000,Y=-1.000000)" "(X=1.000000,Y=0.000000)" "(X=-1.000000,Y=0.000000)" "(X=-1.000000,Y=1.000000)" "(X=1.000000,Y=1.000000)" "(X=-1.000000,Y=-1.000000)" "(X=1.000000,Y=-1.000000)") :!label _label_2)
                (:LoopBody
                  (bind (_outhit_10 _returnvalue_10) (Collision|SphereTraceForObjects (+ (+ (Math|Vector|RotateVector (Math|Vector|MakeVector 0.0 (.X (Math|Vector2D|BreakVector2D (* _array_element_7 (- Portal%20Size 1.0)))) (.Y (Math|Vector2D|BreakVector2D (* _array_element_7 (- Portal%20Size 1.0))))) (LocalVariables|GetLocalFinalRotation)) (LocalVariables|GetLocalFinalLocation)) (* (Math|Vector|GetForwardVector (Math|Conversions|RotationFromXVector (.Normal (Collision|BreakHitResult (LocalVariables|GetLocalHit))))) 1e+01)) (+ (+ (Math|Vector|RotateVector (Math|Vector|MakeVector 0.0 (.X (Math|Vector2D|BreakVector2D (* _array_element_7 (- Portal%20Size 1.0)))) (.Y (Math|Vector2D|BreakVector2D (* _array_element_7 (- Portal%20Size 1.0))))) (LocalVariables|GetLocalFinalRotation)) (LocalVariables|GetLocalFinalLocation)) (* (Math|Vector|GetForwardVector (Math|Conversions|RotationFromXVector (.Normal (Collision|BreakHitResult (LocalVariables|GetLocalHit))))) -1e+01)) 0.01 (Utilities|Array|MakeArray "ObjectTypeQuery9" "ObjectTypeQuery7" "ObjectTypeQuery1" "ObjectTypeQuery2") true (Utilities|Array|MakeArray (Utilities|Select :Index Portal%20Index :Option%200 (Variables|Runtime|GetPortal%201) :Option%201 (Variables|Runtime|GetPortal%202))) "None"))
                  (if _returnvalue_10
                    (if (not (or (Utilities|Enum|Equal(Enum) (Collision|GetCollisionObjectType (.HitComponent (Collision|BreakHitResult _outhit_10))) "ECC_GameTraceChannel6") (Utilities|Enum|Equal(Enum) (Collision|GetCollisionObjectType (.HitComponent (Collision|BreakHitResult _outhit_10))) "ECC_GameTraceChannel1")))
                      (LocalVariables|SetLocalValid false)
                      (goto _label_2 Break))
                    (else
                      (LocalVariables|SetLocalValid false)
                      (goto _label_2 Break))))))
            (:then_1
              (return (LocalVariables|GetLocalValid) (LocalVariables|GetLocalFinalLocation) (LocalVariables|GetLocalFinalRotation))))
          (else
            (LocalVariables|SetLocalFinalLocation (.Location (Collision|BreakHitResult _output_get)) :!label _label_3)
            (LocalVariables|SetLocalFinalRotation (Math|Conversions|RotationFromXVector (.Normal (Collision|BreakHitResult _output_get))))
            (LocalVariables|SetLocalValid false)
            (return (LocalVariables|GetLocalValid) (LocalVariables|GetLocalFinalLocation) (LocalVariables|GetLocalFinalRotation))))
        (else
          (goto _label_3))))))

(fn IsPointOverlappingPortal
  (params (Point :type Vector) (Portal :type BP%20Portal%20Object%20Reference) (Portal%20Size :type Vector%202D%20Structure))
  (bind _returnvalue (- Portal%20Size 1.0))
  (bind (_x _y) (Math|Vector2D|BreakVector2D _returnvalue))
  (if (Variables|/Game/Puzzle_Template/Portals/BP_Portal.BP_Portal_C|GetIs%20Disabled? Portal)
    (return false)
    (else
      (return (Class|KismetMathLibrary|IsPointinBoxwithTransform Point (Transformation|GetActorTransform Portal) (Math|Vector|MakeVector 1.0 _x _y))))))

(fn ToggleCrosshairVisibility
  (params (Visible? :type Boolean))
  (bind _portal_gun_crosshair_ref (Variables|Runtime|GetPortal%20Gun%20Crosshair%20Ref))
  (bind _portal_gun_crosshair_ref_2 (Variables|Runtime|GetPortal%20Gun%20Crosshair%20Ref))
  (bind _portal_crosshair_fade_out (Variables|/Game/Puzzle_Template/Portals/Portal_Gun/Widgets/PT_Portal_Gun_Crosshair_W.PT_Portal_Gun_Crosshair_W_C|GetPortal_Crosshair_Fade_Out _portal_gun_crosshair_ref_2))
  (if Visible?
    (Class|UserWidget|PlayAnimationReverse _portal_gun_crosshair_ref _portal_crosshair_fade_out 1.0 false)
    (else
      (Class|UserWidget|PlayAnimationForward _portal_gun_crosshair_ref _portal_crosshair_fade_out 1.0 false))))

(fn IsNormalStraight?
  (params (Normal :type Vector))
  (bind _returnvalue (Math|Vector|VectorGetAbs Normal))
  (bind (_x _y _z) (Math|Vector|BreakVector _returnvalue))
  (return (Math|Boolean|ORBoolean (== _x 1.0) (== _y 1.0) (== _z 1.0))))

(fn VectorSnappedtoGrid(WithNormal)
  (params (Vector :type Vector) (Normal :type Vector) (Grid%20Size :type Float%20%28double-precision%29))
  (bind (_x _y _z) (Math|Vector|BreakVector Vector))
  (bind _returnvalue (Class|KismetMathLibrary|VectorSnappedtoGrid Vector Grid%20Size))
  (bind _returnvalue_2 (Math|Vector|VectorGetAbs Normal))
  (bind (_x_2 _y_2 _z_2) (Math|Vector|BreakVector _returnvalue_2))
  (bind (_x_3 _y_3 _z_3) (Math|Vector|BreakVector _returnvalue))
  (return (Math|Vector|MakeVector (Math|Float|SelectFloat _x_3 _x (Math|Float|NearlyEqual(Float) _x_2 0.0 0.01)) (Math|Float|SelectFloat _y_3 _y (Math|Float|NearlyEqual(Float) _y_2 0.0 0.01)) (Math|Float|SelectFloat _z_3 _z (Math|Float|NearlyEqual(Float) _z_2 0.0 0.01)))))