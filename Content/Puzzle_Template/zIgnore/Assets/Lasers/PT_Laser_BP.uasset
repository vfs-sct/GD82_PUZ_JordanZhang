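; Laser beam component for puzzles that powers laser receivers and hurts the player.
; While enabled, it multi-line-traces forward each tick, scaling itself and its sound attenuation to the beam length and placing impact sparks and audio at the hit.
; Receivers, filtered by interface and physical material, get connect, update and disconnect messages as tracked hits change.
; Blocking hits on actors with player health start a looping timer that applies damage and horizontal knockback.
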(event Custom|Enable%20Laser
  ;[0 0 0] Enable laser
  (Variables|Runtime|SetIs%20Enabled? true)
  (CallFunction|InitiateSoundComponents)
  (Components|Tick|SetComponentTickEnabled true)
  (Rendering|SetVisibility true true)
  (Utilities|ToggleSound (Variables|Components|GetLaser%20Sound%20Component) true))

(event Custom|Disable%20Laser
  (bind _laser_impact_niagara_system (Variables|Runtime|GetLaser%20Impact%20Niagara%20System))
  ;[0 0 0] Disable laser
  (Variables|Runtime|SetIs%20Enabled? false)
  (Components|Tick|SetComponentTickEnabled false)
  (Rendering|SetVisibility false false)
  (Utilities|ToggleSound (Variables|Components|GetLaser%20Sound%20Component) false)
  (Utilities|ToggleSound (Variables|Components|GetLaser%20Hit%20Sound%20Component) false)
  (Utilities|Time|ClearandInvalidateTimerbyHandle (Variables|Runtime|GetDamage%20Timer))
  (Utilities|IsValid _laser_impact_niagara_system
    (:Is%20Valid
      (Rendering|SetVisibility _laser_impact_niagara_system false false))
    (:Is%20Not%20Valid
      _))
  (for _array_element (Variables|Runtime|GetCurrent%20Detected%20Components)
    (Class|PTLaserReceiverBPI|OnLaserDisconnected(Message) (Components|GetOwner _array_element) (Components|GetOwner)))
  (Utilities|Array|Clear (Variables|Runtime|GetCurrent%20Detected%20Components)))

(event Custom|Start%20Damaging%20Actor
  (params (Health%20System :type BPC%20Player%20Health%20Object%20Reference))
  ;[0 0 0] Damage Timer
  (bind _returnvalue (Utilities|Time|SetTimerbyEvent (delegate Custom|Damage%20Actor) 0.03 true))
  (Variables|Runtime|SetDamage%20Timer _returnvalue))

(event Custom|Damage%20Actor
  ;[0 0 0] Damage Timer
  (if (Variables|Runtime|GetIs%20Enabled?)
    (CallFunction|ApplyDamagetoHitActor (Variables|Runtime|GetTemp%20Damage%20Hit%20Result) (stale Custom|Start%20Damaging%20Actor Health%20System))))

(event EventEndPlay
  (params (EndPlayReason :type EEndPlayReason%20Enum :default "Destroyed"))
  ;[0 0 0] On end play, disconnect any detected laser receiver
  (CallFunction|DisableLaser))

(event EventTick
  (params (DeltaSeconds :type Float%20%28single-precision%29))
  ;[0 0 0] On tick, update the end location of the laser and activate any laser receivers
  (CallFunction|UpdateLaserLocation&PowerReceivers))

(fn UpdateLaserLocation&PowerReceivers
  (bind _self self)
  (bind _laser_size (Variables|Settings|GetLaser%20Size))
  (bind _laser_size_2 (Variables|Settings|GetLaser%20Size))
  (bind _laser_max_distance (Variables|Settings|GetLaser%20Max%20Distance))
  (bind _damage_timer (Variables|Runtime|GetDamage%20Timer))
  (bind _returnvalue (Utilities|Time|IsValidTimerHandle _damage_timer))
  (bind _returnvalue_2 (Transformation|GetWorldLocation _self))
  (bind _returnvalue_3 (Math|Vector|MakeVector _laser_max_distance _laser_size _laser_size))
  (bind (_outhits _returnvalue_4) (Collision|MultiLineTraceByChannel _returnvalue_2 (+ _returnvalue_2 (* (Math|Vector|GetForwardVector _self) (Variables|Settings|GetLaser%20Max%20Distance))) "TraceTypeQuery3" true (Variables|Runtime|GetActors%20to%20Ignore) "None"))
  (if (!= (Utilities|Array|LastIndex _outhits) -1)
    (Transformation|SetWorldScale3D self (Math|Vector|MakeVector (+ (Math|Vector|Distance(Vector) (.TraceStart (Collision|BreakHitResult (Utilities|Array|Get(acopy) _outhits (Utilities|Array|LastIndex _outhits)))) (Math|Vector|SelectVector (.Location (Collision|BreakHitResult (Utilities|Array|Get(acopy) _outhits (Utilities|Array|LastIndex _outhits)))) (.TraceEnd (Collision|BreakHitResult (Utilities|Array|Get(acopy) _outhits (Utilities|Array|LastIndex _outhits)))) (.bBlockingHit (Collision|BreakHitResult (Utilities|Array|Get(acopy) _outhits (Utilities|Array|LastIndex _outhits)))))) 1.0) _laser_size_2 _laser_size_2))
    (Utilities|UpdateLaserSoundAttenuation (Math|Vector|MakeVector (+ (Math|Vector|Distance(Vector) (.TraceStart (Collision|BreakHitResult (Utilities|Array|Get(acopy) _outhits (Utilities|Array|LastIndex _outhits)))) (Math|Vector|SelectVector (.Location (Collision|BreakHitResult (Utilities|Array|Get(acopy) _outhits (Utilities|Array|LastIndex _outhits)))) (.TraceEnd (Collision|BreakHitResult (Utilities|Array|Get(acopy) _outhits (Utilities|Array|LastIndex _outhits)))) (.bBlockingHit (Collision|BreakHitResult (Utilities|Array|Get(acopy) _outhits (Utilities|Array|LastIndex _outhits)))))) 1.0) _laser_size_2 _laser_size_2))
    (if _returnvalue_4
      (bind _laser_impact_niagara_system (Utilities|GetorCreateLaserImpactParticles)
        (:%20%20
          (Transformation|SetWorldLocationAndRotation _laser_impact_niagara_system (Math|Vector|SelectVector (.Location (Collision|BreakHitResult (Utilities|Array|Get(acopy) _outhits (Utilities|Array|LastIndex _outhits)))) (.TraceEnd (Collision|BreakHitResult (Utilities|Array|Get(acopy) _outhits (Utilities|Array|LastIndex _outhits)))) (.bBlockingHit (Collision|BreakHitResult (Utilities|Array|Get(acopy) _outhits (Utilities|Array|LastIndex _outhits))))) (Math|Conversions|RotationFromXVector (.Normal (Collision|BreakHitResult (Utilities|Array|Get(acopy) _outhits (Utilities|Array|LastIndex _outhits))))) false false)
          (Transformation|SetWorldLocation (Variables|Components|GetLaser%20Hit%20Sound%20Component) (Math|Vector|SelectVector (.Location (Collision|BreakHitResult (Utilities|Array|Get(acopy) _outhits (Utilities|Array|LastIndex _outhits)))) (.TraceEnd (Collision|BreakHitResult (Utilities|Array|Get(acopy) _outhits (Utilities|Array|LastIndex _outhits)))) (.bBlockingHit (Collision|BreakHitResult (Utilities|Array|Get(acopy) _outhits (Utilities|Array|LastIndex _outhits))))) false false)
          (for _array_element _outhits
            (bind _output_get (LocalVariables|SetLocal%20Current%20Hit _array_element))
            (bind _output_get_2 (LocalVariables|SetLocal%20Hit%20Component (.HitComponent (Collision|BreakHitResult _output_get))))
            (Utilities|Array|AddUnique (LocalVariables|GetLocal%20Hit%20Components) _output_get_2)
            (if (not (Utilities|Array|ContainsItem (Variables|Runtime|GetCurrent%20Detected%20Components) (LocalVariables|GetLocal%20Hit%20Component)))
              (bind _returnvalue_5 (Utilities|CanHitComponentReceiveLaser? (LocalVariables|GetLocal%20Current%20Hit)))
              (if _returnvalue_5
                (bind _returnvalue_6 (Class|PTLaserReceiverBPI|IsReceivingLaser?(Message) (Components|GetOwner (LocalVariables|GetLocal%20Hit%20Component))))
                (if (not _returnvalue_6)
                  (Utilities|Array|AddUnique (Variables|Runtime|GetCurrent%20Detected%20Components) (LocalVariables|GetLocal%20Hit%20Component))
                  (Class|PTLaserReceiverBPI|OnLaserConnected(Message) (Components|GetOwner (LocalVariables|GetLocal%20Hit%20Component)) (Components|GetOwner) (LocalVariables|GetLocal%20Current%20Hit))
                  (if (.bBlockingHit (Collision|BreakHitResult (LocalVariables|GetLocal%20Current%20Hit)))
                    (bind _laser_impact_niagara_system_2 (Utilities|GetorCreateLaserImpactParticles)
                      (:%20%20
                        (Rendering|SetVisibility _laser_impact_niagara_system_2 false false)
                        (Utilities|ToggleSound (Variables|Components|GetLaser%20Hit%20Sound%20Component) false)
                        (if _returnvalue :!label _label
                          (Utilities|Time|ClearandInvalidateTimerbyHandle (Variables|Runtime|GetDamage%20Timer))))))
                  (else
                    (if (.bBlockingHit (Collision|BreakHitResult (LocalVariables|GetLocal%20Current%20Hit))) :!label _label_2
                      (bind _laser_impact_niagara_system_3 (Utilities|GetorCreateLaserImpactParticles)
                        (:%20%20
                          (Rendering|SetVisibility _laser_impact_niagara_system_3 true false)
                          (Utilities|ToggleSound (Variables|Components|GetLaser%20Hit%20Sound%20Component) true)
                          (bind (_valid_ _health_system) (Utilities|CanActorbeDamaged? (.HitActor (Collision|BreakHitResult (LocalVariables|GetLocal%20Current%20Hit)))))
                          (if _valid_
                            (Variables|Runtime|SetTemp%20Damage%20Hit%20Result (LocalVariables|GetLocal%20Current%20Hit))
                            (if (not _returnvalue)
                              (CallFunction|StartDamagingActor _health_system))
                            (else
                              (goto _label))))))))
                (else
                  (goto _label_2)))
              (else
                (bind _returnvalue_7 (Utilities|CanHitComponentReceiveLaser? (LocalVariables|GetLocal%20Current%20Hit)))
                (if _returnvalue_7
                  (Class|PTLaserReceiverBPI|OnLaserUpdateHitResult(Message) (Components|GetOwner (LocalVariables|GetLocal%20Hit%20Component)) (Components|GetOwner) (LocalVariables|GetLocal%20Current%20Hit))
                  (else
                    (Utilities|Array|RemoveItem (LocalVariables|GetLocal%20Hit%20Components) (LocalVariables|GetLocal%20Hit%20Component)))))))))
      (else
        (bind _laser_impact_niagara_system_4 (Utilities|GetorCreateLaserImpactParticles :!label _label_3)
          (:%20%20
            (Rendering|SetVisibility _laser_impact_niagara_system_4 false false)
            (if (Utilities|Time|IsValidTimerHandle (Variables|Runtime|GetDamage%20Timer))
              (Utilities|Time|ClearandInvalidateTimerbyHandle (Variables|Runtime|GetDamage%20Timer)))))))
    (else
      (Transformation|SetWorldScale3D self _returnvalue_3)
      (Utilities|UpdateLaserSoundAttenuation _returnvalue_3)
      (Utilities|ToggleSound (Variables|Components|GetLaser%20Hit%20Sound%20Component) false)
      (goto _label_3)))
  (bind _output_get_3 (LocalVariables|SetLocal%20Detected%20Components%20Copy (Variables|Runtime|GetCurrent%20Detected%20Components)))
  (for _array_element_2 _output_get_3
    (if (not (Utilities|Array|ContainsItem (LocalVariables|GetLocal%20Hit%20Components) _array_element_2))
      (Utilities|Array|RemoveItem (Variables|Runtime|GetCurrent%20Detected%20Components) _array_element_2)
      (Class|PTLaserReceiverBPI|OnLaserDisconnected(Message) (Components|GetOwner _array_element_2) (Components|GetOwner)))))

(fn ApplyDamagetoHitActor
  (params (Hit :type Hit%20Result%20Structure) (Health%20System :type BPC%20Player%20Health%20Object%20Reference))
  (LocalVariables|SetLocalHitActor (.HitActor (Collision|BreakHitResult Hit)))
  (Default|DealDamage Health%20System (Variables|Settings|GetDamage%20Amount) (Components|GetOwner) true)
  (Audio|Components|Audio|Play (Variables|Components|GetLaser%20Player%20Hit%20Sound%20Component) 0.0)
  (bind _ascharacter (Utilities|Casting|CastToCharacter (LocalVariables|GetLocalHitActor)))
  (Character|LaunchCharacter _ascharacter (Math|Vector|MakeVector (.X (Math|Vector|BreakVector (* (+ (* (Math|Vector|Normalize (- (Transformation|GetActorLocation (LocalVariables|GetLocalHitActor)) (.Location (Collision|BreakHitResult Hit)))) 2.0) (* (Math|Vector|GetForwardVector) 1.0)) (Variables|Settings|GetDamage%20Knockback%20Multiplier)))) (.Y (Math|Vector|BreakVector (* (+ (* (Math|Vector|Normalize (- (Transformation|GetActorLocation (LocalVariables|GetLocalHitActor)) (.Location (Collision|BreakHitResult Hit)))) 2.0) (* (Math|Vector|GetForwardVector) 1.0)) (Variables|Settings|GetDamage%20Knockback%20Multiplier)))) 0.0) false false))

(fn CanActorbeDamaged?
  (params (Actor :type Actor%20Object%20Reference))
  (bind _output_get (LocalVariables|SetLocalPlayerHealthComponent (Actor|GetComponentbyClass Actor "/Game/Puzzle_Template/Player/BPC_Player_Health.BPC_Player_Health_C")))
  (Utilities|IsValid _output_get
    (:Is%20Valid
      (return true _output_get))
    (:Is%20Not%20Valid
      (return false 0))))

(fn ToggleSound
  (params (Audio%20Component :type Audio%20Component%20Object%20Reference) (Activate? :type Boolean))
  (bind _returnvalue (Audio|Components|Audio|IsPlaying Audio%20Component))
  (Utilities|IsValid Audio%20Component
    (:Is%20Valid
      (if Activate?
        (if (not _returnvalue)
          (Audio|Components|Audio|Play Audio%20Component 0.0))
        (elif _returnvalue
          (Audio|Components|Audio|Stop Audio%20Component))))))

(fn InitiateSoundComponents
  (Utilities|FlowControl|Sequence
    (:then_0
      (Utilities|IsValid (Variables|Components|GetLaser%20Sound%20Component)
        (:Is%20Not%20Valid
          (bind _returnvalue (Audio|SpawnSoundAttached (Variables|Sounds|GetLaser%20Sound) self "None" "0, 0, 0" "0, 0, 0" "SnapToTarget" true 1.0 1.0 0.0 "/Game/Puzzle_Template/zIgnore/Assets/Lasers/Sounds/PT_Laser_Att.PT_Laser_Att" 0 false))
          (bind _output_get (Variables|Components|SetLaser%20Sound%20Component _returnvalue))
          (Audio|Components|Audio|Stop _output_get))))
    (:then_1
      (Utilities|IsValid (Variables|Components|GetLaser%20Hit%20Sound%20Component)
        (:Is%20Not%20Valid
          (bind _returnvalue_2 (Audio|SpawnSoundAttached (Variables|Sounds|GetLaser%20Hit%20Sound) self "None" "0, 0, 0" "0, 0, 0" "SnapToTarget" true 1.0 1.0 0.0 "/Game/Puzzle_Template/zIgnore/Assets/Lasers/Sounds/PT_Laser_Hit_Att.PT_Laser_Hit_Att" 0 false))
          (bind _output_get_2 (Variables|Components|SetLaser%20Hit%20Sound%20Component _returnvalue_2))
          (Audio|Components|Audio|Stop _output_get_2))))
    (:then_2
      (Utilities|IsValid (Variables|Components|GetLaser%20Player%20Hit%20Sound%20Component)
        (:Is%20Not%20Valid
          (bind _returnvalue_3 (Audio|SpawnSound2D (Variables|Sounds|GetLaser%20Hit%20Player%20Sound) 1.0 1.0 0.0 0 false false))
          (bind _output_get_3 (Variables|Components|SetLaser%20Player%20Hit%20Sound%20Component _returnvalue_3))
          (Audio|Components|Audio|Stop _output_get_3))))))

(fn UpdateLaserSoundAttenuation
  (params (Extent :type Vector))
  (bind _laser_sound_component (Variables|Components|GetLaser%20Sound%20Component)
    (:then
      (bind _output_get (LocalVariables|SetLocalAtt (Variables|/Script/Engine.SoundAttenuation|GetAttenuation (Variables|/Script/Engine.AudioComponent|GetAttenuationSettings _laser_sound_component))))
      (Utilities|Struct|SetmembersinSoundAttenuationSettings _output_get Extent)
      (Audio|Components|Audio|AdjustAttenuation (Variables|Components|GetLaser%20Sound%20Component) (LocalVariables|GetLocalAtt)))
    (:else)))

(fn CanHitComponentReceiveLaser?
  (params (Hit :type Hit%20Result%20Structure%20%28by%20ref%29))
  (bind _physmat (Collision|BreakHitResult Hit))
  (if (Utilities|DoesObjectImplementInterface (.HitActor (Collision|BreakHitResult Hit)) "/Game/Puzzle_Template/Prefabs/Blueprints/Interfaces/PT_Laser_Receiver_BPI.PT_Laser_Receiver_BPI_C")
    (Utilities|IsValid _physmat
      (:Is%20Valid
        (if (Utilities|Array|ContainsItem (Variables|Settings|GetLaser%20Check%20Physical%20Materials) _physmat)
          (return true)
          (else
            _)))
      (:Is%20Not%20Valid
        _))
    (return false)
    (else
      (return false))))