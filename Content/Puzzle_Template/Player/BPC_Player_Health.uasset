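; Player health component for the puzzle template's player character that handles damage, timed regeneration and death.
; DealDamage lowers clamped health, then optionally starts regeneration and camera shake, and drives a damage overlay widget with the health percentage.
; Regeneration runs on a delayed looping timer that clears itself at max health.
; At zero health, a DoOnce-guarded handler calls OnDeath, fades out and restarts the level at the current checkpoint.
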(event Custom|Init%20Health%20Regen
  ;[0 0 0] Health Regeneration
  (bind _returnvalue (Utilities|Time|SetTimerbyEvent (delegate Custom|Regen%20Health) (Variables|Settings|HealthRegen|GetHealth%20Regen%20Interval) true false (Variables|Settings|HealthRegen|GetHealth%20Regen%20Initial%20Delay))))

(event Custom|Regen%20Health
  ;[0 0 0] Health Regeneration
  (bind _output_get (Variables|Settings|SetCurrent%20Health (Math|Integer|Clamp(Integer) (+ (Variables|Settings|GetCurrent%20Health) (Variables|Settings|HealthRegen|GetHealth%20Regen%20Amount)) 0 (Variables|Settings|GetMax%20Health))))
  (if (>= _output_get (Variables|Settings|GetMax%20Health))
    (Utilities|Time|ClearandInvalidateTimerbyHandle (stale Custom|Init%20Health%20Regen _returnvalue))))

(event Custom|On%20Health%20Reached%200
  ;[0 0 0] The on death event gets called when "Current Health" equals to 0, here we fade out and restart the current level
  (Utilities|FlowControl|DoOnce false
    (:Completed
      (Default|CallOnDeath)
      (CallFunction|StartFadeTransition 0.15 0.0 true false)
      (Utilities|FlowControl|Delay 0.15)
      (CallFunction|RestartPTLevelatCurrentCheckpoint))))

(event EventBeginPlay
  ;[0 0 0] Initialize by binding the Any Damage event to a function within this component, then create the damage overlay widget.
  (Utilities|Casting|CastToCharacter (Components|GetOwner)
    (:then
      (bind _returnvalue (UserInterface|CreateWidget "/Game/Puzzle_Template/Player/Widgets/PT_Player_Damage_Overlay_W.PT_Player_Damage_Overlay_W_C" 0 "(R=1.000000,G=0.000000,B=0.000000,A=1.000000)" 5.0))
      (bind _output_get (Variables|Runtime|SetDamage%20Overlay _returnvalue))
      (UserInterface|Viewport|AddtoViewport _output_get 1))
    (:CastFailed
      (Development|PrintString "The \"PT_Player_Health_System_AC\" should be only attached to the player character." true true "(R=1.000000,G=0.000000,B=0.020756,A=1.000000)"))))

(fn DealDamage
  (params (Damage :type Integer) (Damage%20Causer :type Actor%20Object%20Reference) (Play%20Camera%20Shake? :type Boolean))
  (bind _damage_overlay (Variables|Runtime|GetDamage%20Overlay))
  (bind _output_get (Variables|Settings|SetCurrent%20Health (Math|Integer|Clamp(Integer) (- (Variables|Settings|GetCurrent%20Health) Damage) 0 (Variables|Settings|GetMax%20Health))))
  (if (== _output_get 0)
    (CallFunction|OnHealthReached0)
    (else
      (Utilities|FlowControl|Sequence
        (:then_0
          (if (Variables|Settings|HealthRegen|GetEnable%20Health%20Regen)
            (CallFunction|InitHealthRegen)))
        (:then_1
          (if Play%20Camera%20Shake?
            (Game|Feedback|ClientStartCameraShake (Game|GetPlayerController 0) (Variables|Settings|Effects|GetDamage%20Taken%20Camera%20Shake) (Variables|Settings|Effects|GetDamage%20Taken%20Camera%20Shake%20Intensity) "CameraLocal" "0, 0, 0")))
        (:then_2
          (Utilities|IsValid _damage_overlay
            (:Is%20Valid
              (Default|PlayDamageAnim _damage_overlay (/ (Math|Conversions|ToFloat(Integer) (Variables|Settings|GetCurrent%20Health)) (Math|Conversions|ToFloat(Integer) (Variables|Settings|GetMax%20Health))) 3.0))))))))