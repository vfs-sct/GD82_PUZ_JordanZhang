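; Character component that lets the player interact with and physics-grab actors, including through linked portals.
; Each tick a camera trace, continued through active portals, finds interface-implementing targets and toggles outlines and crosshair.
; The owner triggers interaction or grabbing, with a runtime Physics Handle following the trace and releasing beyond a maximum distance.
; Held objects teleport when the view or character crosses portals, and a box trace reduces Chaos jitter against walls.
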(event Custom|Start%20Interaction
  ;[0 0 0] Start and End interaction, this should be called from your character
  (Utilities|IsValid (Variables|Runtime|Actors|GetInteraction%20Actor)
    (:Is%20Valid
      (switch Utilities|FlowControl|Switch|SwitchonPT_Interaction_Type_Enum (Variables|Runtime|GetInteract%20Type)
        (:NewEnumerator0
          (Class|PTInteractableBPI|OnBeginInteract(Message) (Variables|Runtime|Actors|GetInteraction%20Actor)))
        (:NewEnumerator1
          (CallFunction|StartGrab (Variables|Runtime|Actors|GetInteraction%20Actor)))))))

(event Custom|End%20Interaction
  ;[0 0 0] Start and End interaction, this should be called from your character
  (Utilities|IsValid (Variables|Runtime|Actors|GetInteraction%20Actor)
    (:Is%20Valid
      (switch Utilities|FlowControl|Switch|SwitchonPT_Interaction_Type_Enum (Variables|Runtime|GetInteract%20Type)
        (:NewEnumerator0
          (Class|PTInteractableBPI|OnEndInteract(Message) (Variables|Runtime|Actors|GetInteraction%20Actor)))
        (:NewEnumerator1
          (CallFunction|EndGrab))))))

(event EventBeginPlay
  ;[0 0 0] On Begin Play, Initiate the grabbing system and add the interaction widget to the viewport
  (CallFunction|InitGrabSystem)
  (if (Variables|Interaction|GetCreate%20Interaction%20Crosshair?)
    (bind _returnvalue (UserInterface|CreateWidget "/Game/Puzzle_Template/Player/Widgets/PT_Interaction_Crosshair_W.PT_Interaction_Crosshair_W_C" (Game|GetPlayerController 0) self))
    (bind _output_get (Variables|Runtime|SetInteraction%20Crosshair%20Widget _returnvalue))
    (UserInterface|Viewport|AddtoPlayerScreen _output_get)))

(event EventTick
  (params (DeltaSeconds :type Float%20%28single-precision%29))
  ;[0 0 0] Tick, check for interactables and update the grabbed component location and rotation if we are grabbing something.
  (CallFunction|CheckInteractables&Grabbables)
  (if (Grab|GetIsGrabbing)
    (Grab|UpdateGrabLocation&Rotation true)))

(event Custom|Start%20Grab
  (params (Actor :type Actor%20Object%20Reference))
  ;[0 0 0] Start Grabbing
  (bind _output_get (Variables|Runtime|Actors|SetGrabbed%20Actor Actor))
  (Utilities|IsValid _output_get
    (:Is%20Valid
      (bind _asmesh_component (Utilities|Casting|CastToMeshComponent (Variables|/Script/Engine.Actor|GetRootComponent _output_get)))
      (Class|PTGrabbaleBPI|OnBeginGrab(Message) (Variables|Runtime|Actors|GetGrabbed%20Actor) self)
      (Variables|Runtime|Components|SetGrabbed%20Mesh _asmesh_component)
      (Physics|Components|PhysicsHandle|GrabComponentatLocationwithRotation (Variables|Runtime|Components|GetPhysics%20Handle) (Variables|Runtime|Components|GetGrabbed%20Mesh) "None" (Transformation|GetWorldLocation (Variables|Runtime|Components|GetGrabbed%20Mesh)) (Transformation|GetWorldRotation _asmesh_component))
      (Variables|Runtime|SetIs%20Grabbing true)
      (bind _returnvalue (Utilities|GetCharacterReference))
      (Collision|IgnoreActorwhenMoving (Variables|/Script/Engine.Character|GetCapsuleComponent _returnvalue) (Variables|Runtime|Actors|GetGrabbed%20Actor) true)
      (bind (_valid_ _returnvalue_2) (Utilities|GetPortableComponentfromActor (Variables|Runtime|Actors|GetGrabbed%20Actor)))
      (if _valid_
        (Variables|/Game/Puzzle_Template/Portals/BPC_Portable.BPC_Portable_C|SetIgnore%20Portals? _returnvalue_2 true)
        (Audio|PlaySound2D (Variables|Grab|GetStart%20Grab%20Sound) 0.8 (Math|Random|RandomFloatinRange 0.9 1.1) 0.0 0 0)))))

(event Custom|End%20Grab
  ;[0 0 0] End Grab
  (Utilities|IsValid (Variables|Runtime|Components|GetGrabbed%20Mesh)
    (:Is%20Valid
      (bind _returnvalue (Physics|GetPhysicsLinearVelocity (Variables|Runtime|Components|GetGrabbed%20Mesh) "None"))
      (Physics|SetPhysicsLinearVelocity (Variables|Runtime|Components|GetGrabbed%20Mesh) (Math|Vector|VectorClampSizeMax _returnvalue (Variables|Grab|GetGrab%20Max%20Velocity%20On%20End%20Grab)) false "None")
      (Class|PrimitiveComponent|SetPhysicsAngularVelocityinDegrees (Variables|Runtime|Components|GetGrabbed%20Mesh) (Math|Vector|VectorClampSizeMax (Physics|GetPhysicsAngularVelocityinDegrees (Variables|Runtime|Components|GetGrabbed%20Mesh) "None") (Variables|Grab|GetGrab%20Max%20Velocity%20On%20End%20Grab)) false "None")
      (Class|PTGrabbaleBPI|OnEndGrab(Message) (Variables|Runtime|Actors|GetGrabbed%20Actor))
      (Physics|Components|PhysicsHandle|ReleaseComponent (Variables|Runtime|Components|GetPhysics%20Handle))
      (bind _returnvalue_2 (Utilities|GetCharacterReference))
      (Collision|IgnoreActorwhenMoving (Variables|/Script/Engine.Character|GetCapsuleComponent _returnvalue_2) (Variables|Runtime|Actors|GetGrabbed%20Actor) false)
      (bind (_valid_ _returnvalue_3) (Utilities|GetPortableComponentfromActor (Variables|Runtime|Actors|GetGrabbed%20Actor)))
      (if _valid_
        (Variables|/Game/Puzzle_Template/Portals/BPC_Portable.BPC_Portable_C|SetIgnore%20Portals? _returnvalue_3 false))
      (Variables|Runtime|Components|SetGrabbed%20Mesh 0)
      (Variables|Runtime|Actors|SetGrabbed%20Actor 0)
      (Variables|Runtime|SetIs%20Grabbing false)
      (Audio|PlaySound2D (Variables|Grab|GetEnd%20Grab%20Sound) 0.8 (Math|Random|RandomFloatinRange 0.9 1.1) 0.0 0 0))))

(event Custom|Try%20Bind%20Owner%20Character%20Teleported
  ;[0 0 0] Try bind on character teleported, if we are grabbing, this will call the teleloper grab to target location function, we need the character teleported variable in order to have a smooth grabbable transition.
  (bind _returnvalue (Utilities|GetCharacterReference))
  (Utilities|IsValid (Actor|GetComponentbyClass _returnvalue "/Game/Puzzle_Template/Portals/BPC_Portable.BPC_Portable_C")
    (:Is%20Valid
      (EventDispatchers|AssignTeleported (Actor|GetComponentbyClass _returnvalue "/Game/Puzzle_Template/Portals/BPC_Portable.BPC_Portable_C") (delegate Custom|On_Character_Teleported)))))

(event Custom|On_Character_Teleported
  (params (Actor :type Actor%20Object%20Reference))
  ;[0 0 0] Try bind on character teleported, if we are grabbing, this will call the teleloper grab to target location function, we need the character teleported variable in order to have a smooth grabbable transition.
  (if (Grab|GetIsGrabbing)
    (Variables|Runtime|SetCharacter%20Teleported%20While%20Grab? true)
    (Grab|TeleportGrabtoTargetLocation false)
    (Utilities|FlowControl|Delay 0.0)
    (Variables|Runtime|SetCharacter%20Teleported%20While%20Grab? false)))

(event Custom|Init%20Grab%20System
  ;[0 0 0] Create the Physics Handle component and update the variables
  (|CreatePhysicsHandle
    (:%20
      (CallFunction|TryBindOwnerCharacterTeleported))))

(fn CheckInteractables&Grabbables
  (bind _camera (Utilities|GetCameraReference)
    (:%20%20
      (bind (_camera_hit _portal_hit _blocking_hit_ _looking_out_of_portal_ _portal) (CallFunction|CustomLineTracebyChannel (Transformation|GetWorldLocation _camera) (+ (Transformation|GetWorldLocation _camera) (* (Math|Vector|GetForwardVector _camera) (Math|Float|SelectFloat (Variables|Grab|GetGrab%20Distance%20From%20Camera) (Variables|Interaction|GetInteraction%20Range) (Grab|GetIsGrabbing)))) "TraceTypeQuery4" true (select (Grab|GetIsGrabbing) (Utilities|Array|MakeArray (Variables|Runtime|Actors|GetGrabbed%20Actor)) (Utilities|Array|MakeArray)) "None" true "PORTAL"))
      (Variables|Runtime|SetCamera%20Hit _camera_hit)
      (Variables|Runtime|SetPortal%20Hit _portal_hit)
      (if (Math|Boolean|NotEqual(Boolean) _looking_out_of_portal_ (Variables|Runtime|GetInteracting%20Through%20Portal?))
        (bind _output_get (Variables|Runtime|SetInteracting%20Through%20Portal? _looking_out_of_portal_))
        (if _output_get
          (Variables|Runtime|Actors|SetInteraction%20Portal%20Ref _portal)
          (Grab|TeleportGrabtoTargetLocation true)
          (else
            (Grab|TeleportGrabtoTargetLocation true)
            (Variables|Runtime|Actors|SetInteraction%20Portal%20Ref 0))))
      (if (not (Grab|GetIsGrabbing))
        (LocalVariables|SetLocal%20Hovered%20Actor (.HitActor (Collision|BreakHitResult (select (Variables|Runtime|GetInteracting%20Through%20Portal?) (Variables|Runtime|GetPortal%20Hit) (Variables|Runtime|GetCamera%20Hit)))))
        (if (.bBlockingHit (Collision|BreakHitResult (select (Variables|Runtime|GetInteracting%20Through%20Portal?) (Variables|Runtime|GetPortal%20Hit) (Variables|Runtime|GetCamera%20Hit))))
          (if (Utilities|DoesObjectImplementInterface (LocalVariables|GetLocal%20Hovered%20Actor) "/Game/Puzzle_Template/Prefabs/Blueprints/Interfaces/PT_Interactable_BPI.PT_Interactable_BPI_C")
            (Variables|Runtime|SetInteract%20Type "NewEnumerator0")
            (bind _can_interact_ (Class|PTInteractableBPI|CanInteract?(Message) (LocalVariables|GetLocal%20Hovered%20Actor)))
            (if _can_interact_
              (if (!= (Variables|Runtime|Actors|GetInteraction%20Actor) (LocalVariables|GetLocal%20Hovered%20Actor)) :!label _label
                (Utilities|IsValid (Variables|Runtime|Actors|GetInteraction%20Actor)
                  (:Is%20Valid
                    (Utilities|ToggleOutlines (Variables|Runtime|Actors|GetInteraction%20Actor) false))
                  (:Is%20Not%20Valid
                    _))
                (bind _output_get_2 (Variables|Runtime|Actors|SetInteraction%20Actor (LocalVariables|GetLocal%20Hovered%20Actor)))
                (Utilities|ToggleOutlines _output_get_2 true)
                (Utilities|TogglePortalGunCrosshairifAvailable false)
                (bind _interaction_crosshair_widget (Variables|Runtime|GetInteraction%20Crosshair%20Widget)
                  (:then
                    (Default|ToggleInteract _interaction_crosshair_widget true))
                  (:else)))
              (else
                (Utilities|IsValid (Variables|Runtime|Actors|GetInteraction%20Actor) :!label _label_2
                  (:Is%20Valid
                    (Utilities|ToggleOutlines (Variables|Runtime|Actors|GetInteraction%20Actor) false)
                    (Variables|Runtime|Actors|SetInteraction%20Actor 0)
                    (Utilities|TogglePortalGunCrosshairifAvailable true)
                    (bind _interaction_crosshair_widget_2 (Variables|Runtime|GetInteraction%20Crosshair%20Widget)
                      (:then
                        (Default|ToggleInteract _interaction_crosshair_widget_2 false))
                      (:else))))))
            (elif (Utilities|DoesObjectImplementInterface (LocalVariables|GetLocal%20Hovered%20Actor) "/Game/Puzzle_Template/Prefabs/Blueprints/Interfaces/PT_Grabbale_BPI.PT_Grabbale_BPI_C")
              (Variables|Runtime|SetInteract%20Type "NewEnumerator1")
              (goto _label)
              (else
                (goto _label_2))))
          (else
            (goto _label_2)))))))

(fn GetIsGrabbing
  (return (Variables|Runtime|GetIs%20Grabbing)))

(fn GetIsInteractingThroughPortal
  (return (Variables|Runtime|GetInteracting%20Through%20Portal?)))

(fn ToggleOutlines
  (params (Actor :type Actor%20Object%20Reference) (Enabled? :type Boolean) (__WorldContext :type Object%20Object%20Reference))
  (bind _output_get (LocalVariables|SetLocalChildren (Actor|GetComponentsByClass Actor "/Script/Engine.MeshComponent")))
  (for _array_element _output_get
    (if (not (Components|ComponentHasTag _array_element "NO_OUTLINE"))
      (Rendering|SetRenderCustomDepth _array_element Enabled?)
      (Rendering|SetCustomDepthStencilValue _array_element 5))))

(fn CustomLineTracebyChannel
  (params (Start :type Vector) (End :type Vector) (TraceChannel :type ETraceTypeQuery%20Enum :default "TraceTypeQuery1") (bTraceComplex :type Boolean) (ActorsToIgnore :type Array%20of%20Actor%20Object%20References) (DrawDebugType :type EDrawDebugTrace%20Enum :default "None") (bIgnoreSelf :type Boolean) (Portal%20Tag :type Name :default "PORTAL"))
  (bind _outhit (Collision|LineTraceByChannel Start End TraceChannel bTraceComplex ActorsToIgnore DrawDebugType bIgnoreSelf))
  (bind _output_get (LocalVariables|SetLocalHit _outhit))
  (if (.bBlockingHit (Collision|BreakHitResult _output_get))
    (if (Components|ComponentHasTag (.HitComponent (Collision|BreakHitResult _output_get)) Portal%20Tag)
      (bind _asbp_portal (Utilities|Casting|CastToBP_Portal (.HitActor (Collision|BreakHitResult _output_get)))
        (:then
          (bind _output_get_2 (LocalVariables|SetLocalHitPortal _asbp_portal))
          (if (Default|IsLinkedPortalActive? _output_get_2)
            (bind (_outhit_2 _returnvalue) (Collision|LineTraceByChannel (Math|Transform|TransformLocation (Transformation|GetActorTransform (Variables|/Game/Puzzle_Template/Portals/BP_Portal.BP_Portal_C|GetLinked%20Portal%20Ref _output_get_2)) (Math|Transform|InverseTransformLocation (Transformation|GetWorldTransform (Variables|/Game/Puzzle_Template/Portals/BP_Portal.BP_Portal_C|GetBack _output_get_2)) (.Location (Collision|BreakHitResult (LocalVariables|GetLocalHit))))) (+ (Math|Transform|TransformLocation (Transformation|GetActorTransform (Variables|/Game/Puzzle_Template/Portals/BP_Portal.BP_Portal_C|GetLinked%20Portal%20Ref _output_get_2)) (Math|Transform|InverseTransformLocation (Transformation|GetWorldTransform (Variables|/Game/Puzzle_Template/Portals/BP_Portal.BP_Portal_C|GetBack _output_get_2)) (.Location (Collision|BreakHitResult (LocalVariables|GetLocalHit))))) (* (Math|Transform|TransformDirection (Transformation|GetActorTransform (Variables|/Game/Puzzle_Template/Portals/BP_Portal.BP_Portal_C|GetLinked%20Portal%20Ref _output_get_2)) (Math|Transform|InverseTransformDirection (Transformation|GetWorldTransform (Variables|/Game/Puzzle_Template/Portals/BP_Portal.BP_Portal_C|GetBack _output_get_2)) (Math|Vector|GetUnitDirection(Vector) (.TraceStart (Collision|BreakHitResult (LocalVariables|GetLocalHit))) (.TraceEnd (Collision|BreakHitResult (LocalVariables|GetLocalHit)))))) (- (Math|Vector|Distance(Vector) Start End) (.Distance (Collision|BreakHitResult (LocalVariables|GetLocalHit)))))) TraceChannel bTraceComplex ActorsToIgnore DrawDebugType bIgnoreSelf))
            (return (LocalVariables|GetLocalHit) _outhit_2 _returnvalue true (LocalVariables|GetLocalHitPortal))
            (else
              (return (LocalVariables|GetLocalHit) (LocalVariables|GetLocalHit) true false 0))))
        (:CastFailed
          _)))
    (return (LocalVariables|GetLocalHit) (LocalVariables|GetLocalHit) true false 0)
    (else
      (return (LocalVariables|GetLocalHit) (LocalVariables|GetLocalHit) false false 0))))

(fn UpdateGrabLocation&Rotation
  (params (Check%20Distance? :type Boolean))
  (bind _interacting_through_portal_ (Variables|Runtime|GetInteracting%20Through%20Portal?))
  (bind _portal_hit (Variables|Runtime|GetPortal%20Hit))
  (bind _camera_hit (Variables|Runtime|GetCamera%20Hit))
  (bind _returnvalue (select _interacting_through_portal_ _portal_hit _camera_hit))
  (bind (_bblockinghit _binitialoverlap _time _distance _location _impactpoint _normal _impactnormal _physmat _hitactor _hitcomponent _hitbonename _bonename _hititem _elementindex _faceindex _tracestart _traceend) (Collision|BreakHitResult _returnvalue))
  (bind _returnvalue_2 (Math|Vector|GetUnitDirection(Vector) _tracestart _traceend))
  (bind _returnvalue_3 (Math|Conversions|RotationFromXVector _returnvalue_2))
  (bind (_roll _pitch _yaw) (Math|Rotator|BreakRotator _returnvalue_3))
  (Utilities|IsValid (Variables|Runtime|Actors|GetGrabbed%20Actor)
    (:Is%20Valid
      (LocalVariables|SetLocalEndLocation (Math|Vector|SelectVector _location _traceend _bblockinghit))
      (LocalVariables|SetLocalEndRotation (Math|Rotator|MakeRotator _roll 0.0 _yaw))
      (if (Variables|Runtime|GetSkip%20Chaos%20Physics%20Fix?)
        _
        (else
          (|TryFixJitteryChaosPhysics)))
      (Class|PhysicsHandleComponent|SetTargetLocationandRotation (Variables|Runtime|Components|GetPhysics%20Handle) (LocalVariables|GetLocalEndLocation) (LocalVariables|GetLocalEndRotation))
      (if Check%20Distance?
        (Utilities|CheckDistanceGrabtoObject)))
    (:Is%20Not%20Valid
      (Variables|Runtime|Components|SetGrabbed%20Mesh 0)
      (Variables|Runtime|Actors|SetGrabbed%20Actor 0)
      (Physics|Components|PhysicsHandle|ReleaseComponent (Variables|Runtime|Components|GetPhysics%20Handle))
      (Variables|Runtime|SetIs%20Grabbing false)
      (bind _interaction_crosshair_widget (Variables|Runtime|GetInteraction%20Crosshair%20Widget)
        (:then
          (Default|ToggleInteract _interaction_crosshair_widget false))
        (:else)))))

(fn GetPortableComponentfromActor
  (params (Actor :type Actor%20Object%20Reference))
  (bind _returnvalue (Actor|GetComponentbyClass Actor "/Game/Puzzle_Template/Portals/BPC_Portable.BPC_Portable_C"))
  (Utilities|IsValid _returnvalue
    (:Is%20Valid
      (return true _returnvalue))
    (:Is%20Not%20Valid
      (return false 0))))

(fn TeleportGrabtoTargetLocation
  (params (Check%20Portals%20Distance? :type Boolean))
  (bind _grabbed_mesh (Variables|Runtime|Components|GetGrabbed%20Mesh))
  ;[0 0 0] Intantly teleports the grabbed actor to the target location, this happens when we start looking through a teleport
  (if (not (Variables|Runtime|GetCharacter%20Teleported%20While%20Grab?))
    (if (Grab|GetIsGrabbing)
      (Variables|Runtime|SetSkip%20Chaos%20Physics%20Fix? true)
      (|CalculateEndLocationOffset
        (:%20%20
          (Grab|UpdateGrabLocation&Rotation false)
          (Physics|Components|PhysicsHandle|ReleaseComponent (Variables|Runtime|Components|GetPhysics%20Handle))
          (|CalculateEndLocation&Rotation
            (:%20%20
              (bind (_valid_ _returnvalue) (Utilities|GetPortableComponentfromActor (Variables|Runtime|Actors|GetGrabbed%20Actor)))
              (if _valid_
                (Utilities|IsValid (Variables|/Game/Puzzle_Template/Portals/BPC_Portable.BPC_Portable_C|GetIn%20Portal _returnvalue)
                  (:Is%20Valid
                    (bind _output_get (LocalVariables|SetLocalInPortal (Variables|/Game/Puzzle_Template/Portals/BPC_Portable.BPC_Portable_C|GetIn%20Portal _returnvalue)))
                    (Default|OnActorExitPortal _output_get (Variables|Runtime|Actors|GetGrabbed%20Actor))
                    (Default|OnActorEnterPortal (Variables|/Game/Puzzle_Template/Portals/BP_Portal.BP_Portal_C|GetLinked%20Portal%20Ref _output_get) (Variables|Runtime|Actors|GetGrabbed%20Actor) false))
                  (:Is%20Not%20Valid
                    _)))
              (Transformation|SetWorldLocationAndRotation (Variables|Runtime|Components|GetGrabbed%20Mesh) (LocalVariables|GetLocalEndLocation) (LocalVariables|GetLocalEndRotation) false true)
              (Physics|Components|PhysicsHandle|GrabComponentatLocationwithRotation (Variables|Runtime|Components|GetPhysics%20Handle) _grabbed_mesh "None" (Transformation|GetWorldLocation _grabbed_mesh) (Transformation|GetWorldRotation _grabbed_mesh))
              (Variables|Runtime|SetSkip%20Chaos%20Physics%20Fix? false))))))))

(fn TogglePortalGunCrosshairifAvailable
  (params (Visible? :type Boolean))
  (bind _returnvalue (Components|GetOwner))
  (bind _returnvalue_2 (Actor|GetComponentbyClass _returnvalue "/Game/Puzzle_Template/Portals/Portal_Gun/BPC_Portals_Gun.BPC_Portals_Gun_C"))
  (Utilities|IsValid _returnvalue_2
    (:Is%20Valid
      (Default|ToggleCrosshairVisibility _returnvalue_2 Visible?))))