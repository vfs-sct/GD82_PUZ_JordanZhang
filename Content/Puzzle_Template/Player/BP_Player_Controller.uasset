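; Player controller for the puzzle template that adds the input mapping context and keeps the player upright after portal travel.
; Each tick it interpolates any control rotation roll back toward zero.
; ResetPawnRotation, typically called by the character after a portal, uses a duration-scaled timeline to lerp a tilted pawn upright toward the control yaw.
; Controller yaw is suspended during the lerp and restored when it finishes.
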(event Custom|Reset%20Pawn%20Rotation
  (params (Duration :type Float%20%28double-precision%29))
  (bind _returnvalue (Pawn|GetControlledPawn))
  (bind _returnvalue_2 (Pawn|GetControlledPawn))
  ;[0 0 0] Reset controlled pawn rotation smoothly, this is usually called from the "PT_Player_Character" blueprint after going through a portal.
  (bind _output_get (Variables|Runtime|SetTemp%20Controlled%20Pawn%20Rotation (Transformation|GetActorRotation (Pawn|GetControlledPawn))))
  (if (or (not (Math|Float|NearlyEqual(Float) (.Roll (Math|Rotator|BreakRotator _output_get)) 0.0 1.0)) (not (Math|Float|NearlyEqual(Float) (.Pitch (Math|Rotator|BreakRotator _output_get)) 0.0 1.0)))
    (Variables|/Script/Engine.Pawn|SetbUseControllerRotationYaw _returnvalue_2 false)
    (Components|Timeline|SetPlayRate (Variables|Default|GetReset_Pawn_Rotation_TL) (/ 1.0 Duration))
    (bind _alpha (Timeline|Reset_Pawn_Rotation_TL PlayFromStart)
      (:Update
        (Transformation|SetActorRotation _returnvalue (Math|Rotator|Lerp(Rotator) (Variables|Runtime|GetTemp%20Controlled%20Pawn%20Rotation) (Math|Rotator|MakeRotator 0.0 0.0 (.Yaw (Math|Rotator|BreakRotator (Pawn|GetControlRotation :!class /Script/Engine.Controller)))) _alpha true) true))
      (:Finished
        (Variables|/Script/Engine.Pawn|SetbUseControllerRotationYaw _returnvalue true)))
    (else
      (Variables|/Script/Engine.Pawn|SetbUseControllerRotationYaw _returnvalue_2 true))))

(event EventTick
  (params (DeltaSeconds :type Float%20%28single-precision%29))
  ;[0 0 0] Keep the control rotation valid by setting the roll value to 0.
  (CallFunction|KeepValidControlRotation))

(event EventBeginPlay
  ;[0 0 0] Update input mapping context
  (Input|AddMappingContext (PlayerController|LocalPlayerSubsystems|GetEnhancedInputLocalPlayerSubsystem) "/Game/Puzzle_Template/Inputs/PT_Input_Mappings_IM.PT_Input_Mappings_IM" 0 "(bIgnoreAllPressedKeysUntilRelease=True,bForceImmediately=False,bNotifyUserSettings=False)"))

(fn ConstructionScript)

(fn KeepValidControlRotation
  (bind _returnvalue (Pawn|GetControlRotation :!class /Script/Engine.Controller))
  (bind (_roll _pitch _yaw) (Math|Rotator|BreakRotator _returnvalue))
  (if (not (Math|Float|NearlyEqual(Float) (Math|Float|Absolute(Float) (.Roll (Math|Rotator|BreakRotator (Pawn|GetControlRotation :!class /Script/Engine.Controller)))) 0.0 0.0001))
    (Pawn|SetControlRotation (Math|Interpolation|RInterpTo _returnvalue (Math|Rotator|MakeRotator 0.0 _pitch _yaw) (Utilities|Time|GetWorldDeltaSeconds) 5.0))))