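; Procedural stair prefab for puzzle level geometry, built in the construction script from a configurable step count.
; GenerateStair adds one static mesh component per step, each shifted a fixed amount along negative Y and up Z to form a 45-degree flight.
; It then stretches SmoothCollisionPivot along Y in proportion to the step count, so the smooth collision grows with the stair.
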(fn ConstructionScript
  (CallFunction|GenerateStair))

(fn GenerateStair
  (for _index (range 1 (Variables|Settings|GetSteps%20Amount))
    (bind _output_get (LocalVariables|SetLocal%20Next%20Step%20Location (+ (LocalVariables|GetLocal%20Next%20Step%20Location) "0,-50.000000,50.000000")))
    (AddComponent|AddStaticMeshComponent false (Math|Transform|MakeTransform _output_get "0, 0, 0" "1.000000,1.000000,1.000000")))
  (Transformation|SetRelativeScale3D (Variables|Default|GetSmooth%20Collision%20Pivot) (Math|Vector|MakeVector 1.0 (+ 0.35 (/ (* (Variables|Settings|GetSteps%20Amount) 35.369999) 1e+02)) 1.0)))