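; Base power source Blueprint for the puzzle template that switches power on or off for a given list of actors.
; TogglePowerToActors stores the power state, then sends received or stopped messages through the PT_Power_Receiver_BPI interface.
; Actors lacking that interface trigger a printed error.
; An audio component, with attenuation set at construction, optionally plays a separate sound for starting and stopping power.
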(fn ConstructionScript
  (|CallParentFunction)
  (Variables|/Script/Engine.AudioComponent|SetAttenuationSettings (Variables|Default|GetPower%20Audio) (Variables|Sounds|GetSounds%20Attenuation)))

(fn TogglePowertoActors
  (params (Give%20Power? :type Boolean) (Actors :type Array%20of%20Actor%20Object%20References))
  (Variables|Runtime|SetIs%20Giving%20Power? Give%20Power?)
  (Utilities|PlayPowerSounds)
  (for _array_element Actors
    (if (Utilities|DoesObjectImplementInterface _array_element "/Game/Puzzle_Template/Prefabs/Blueprints/Interfaces/PT_Power_Receiver_BPI.PT_Power_Receiver_BPI_C")
      (if Give%20Power?
        (Class|PTPowerReceiverBPI|OnPowerReceived(Message) _array_element)
        (else
          (Class|PTPowerReceiverBPI|OnPowerStop(Message) _array_element)))
      (else
        (Development|PrintText (Utilities|Text|FormatText "ERROR: Unable to send power to {Actor}, this actor doesn't implement the \"Power_Receiver_Interface\"." _array_element) true true "(R=1.000000,G=0.000000,B=0.007234,A=1.000000)" 5.0)))))

(fn PlayPowerSounds
  (if (Variables|Runtime|GetIs%20Giving%20Power?)
    (if (Variables|Sounds|GetPlay%20Giving%20Power%20Sound?)
      (Audio|Components|Audio|SetSound (Variables|Default|GetPower%20Audio) (Variables|Sounds|GetGiving%20Power%20Sound))
      (Audio|Components|Audio|Play (Variables|Default|GetPower%20Audio) 0.0))
    (elif (Variables|Sounds|GetPlay%20Stopped%20Giving%20Power%20Sound?)
      (Audio|Components|Audio|SetSound (Variables|Default|GetPower%20Audio) (Variables|Sounds|GetStopped%20Giving%20Power%20Sound))
      (Audio|Components|Audio|Play (Variables|Default|GetPower%20Audio) 0.0))))