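; Base puzzle actor for objects that receive power from one or more power sources.
; A counter tracks active sources, firing ReceivingPower when it rises to one and StoppedReceivingPower when it returns to zero, both empty hooks for child Blueprints.
; Each transition can play its own sound on a shared, attenuated audio component.
; The CallOnPowerReceived and CallOnPowerStopped notifications run only when the matching sound is enabled.
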(event Custom|Stopped%20Receiving%20Power
  ;[0 0 0] These 2 events should be used when creating a child actor from this actor.
)

(event Custom|Receiving%20Power
  ;[0 0 0] These 2 events should be used when creating a child actor from this actor.
)

(event EventOnPowerReceived
  (bind _powered___unpowered_audio (Variables|Default|GetPowered%20/%20Unpowered%20Audio))
  ;[0 0 0] Manage multiple power sources
  (bind _result (Math|Integer|IncrementInt (Variables|Runtime|GetCurrent%20Power%20Sources%20Amount))
    (:%20%20
      (if (== _result 1)
        (CallFunction|ReceivingPower)
        (if (Variables|Sounds|GetPlay%20Powered%20Sound?)
          (Audio|Components|Audio|SetSound _powered___unpowered_audio (Variables|Sounds|GetPowered%20Sound))
          (Audio|Components|Audio|Play _powered___unpowered_audio 0.0)
          (Default|CallOnPowerReceived))))))

(event EventOnPowerStop
  (bind _powered___unpowered_audio (Variables|Default|GetPowered%20/%20Unpowered%20Audio))
  ;[0 0 0] Manage multiple power sources
  (bind _result (Math|Integer|DecrementInt (Variables|Runtime|GetCurrent%20Power%20Sources%20Amount))
    (:%20%20
      (if (== _result 0)
        (CallFunction|StoppedReceivingPower)
        (if (Variables|Sounds|GetPlay%20Unpowered%20Sound?)
          (Audio|Components|Audio|SetSound _powered___unpowered_audio (Variables|Sounds|GetUnpowered%20Sound))
          (Audio|Components|Audio|Play _powered___unpowered_audio 0.0)
          (Default|CallOnPowerStopped))))))

(fn ConstructionScript
  (Variables|/Script/Engine.AudioComponent|SetAttenuationSettings (Variables|Default|GetPowered%20/%20Unpowered%20Audio) (Variables|Sounds|GetSounds%20Attenuation)))