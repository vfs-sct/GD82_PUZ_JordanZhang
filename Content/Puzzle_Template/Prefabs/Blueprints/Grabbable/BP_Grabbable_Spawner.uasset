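; Grabbable spawner for puzzles that spawns an actor of a configurable class at its spawn point when it receives power.
; Spawns are tracked in an array, and exceeding the optional cap animates away and removes the oldest.
; A blocked or failed spawn sets an error material state and plays an error sound.
; A timeline drives the mesh's material state, reversing when power stops.
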(event Custom|Play%20Mesh%20Materials%20Animation
  ;[0 0 0] Animate the state of the materials included in the mesh
  (bind _alpha (Timeline|Animate_Mesh_Materials Play)
    (:Update
      (Rendering|Material|SetScalarParameterValueonMaterials (Variables|Default|GetMesh) "State" _alpha))))

(event Custom|Reverse%20Mesh%20Materials%20Animation
  ;[0 0 0] Animate the state of the materials included in the mesh
  (bind _alpha (Timeline|Animate_Mesh_Materials Reverse)
    (:Update
      (Rendering|Material|SetScalarParameterValueonMaterials (Variables|Default|GetMesh) "State" _alpha))))

(event EventReceivingPower
  (bind _spawn_point (Variables|Default|GetSpawn%20Point))
  (bind _spawned_grabbables (Variables|Settings|GetSpawned%20Grabbables))
  (bind _spawn_audio (Variables|Default|GetSpawn%20Audio))
  (bind _spawn_audio_2 (Variables|Default|GetSpawn%20Audio))
  (bind _output (Utilities|Array|Get(acopy) _spawned_grabbables))
  ;[0 0 0] Receiving Power
  (bind _returnvalue (Game|SpawnActorfromClass (Variables|Settings|GetGrabbable%20To%20Spawn) (Math|Transform|MakeTransform (Transformation|GetWorldLocation _spawn_point) (Math|Conversions|RotationFromXVector (Math|Vector|GetRightVector _spawn_point)) (Variables|Settings|GetGrabbable%20Scale)) "DontSpawnIfColliding" "SelectDefaultAtRuntime" 0 true 0))
  (Utilities|IsValid _returnvalue
    (:Is%20Valid
      (Utilities|Array|Add (Variables|Settings|GetSpawned%20Grabbables) _returnvalue)
      (Rendering|Material|SetScalarParameterValueonMaterials (Variables|Default|GetMesh) "Error_State" 0.0)
      (CallFunction|PlayMeshMaterialsAnimation)
      (Audio|Components|Audio|SetSound _spawn_audio_2 (Variables|Sounds|GetSpawn%20Sound))
      (Audio|Components|Audio|Play _spawn_audio_2 0.0)
      (if (> (Variables|Settings|GetMax%20Spawned%20Grabbables) 0)
        (if (< (Variables|Settings|GetMax%20Spawned%20Grabbables) (Utilities|Array|Length (Variables|Settings|GetSpawned%20Grabbables)))
          (Utilities|IsValid _output
            (:Is%20Valid
              (Default|AnimateDestroy _output)
              (Utilities|Array|RemoveIndex (Variables|Settings|GetSpawned%20Grabbables)))))))
    (:Is%20Not%20Valid
      (Rendering|Material|SetScalarParameterValueonMaterials (Variables|Default|GetMesh) "Error_State" 1.0)
      (CallFunction|PlayMeshMaterialsAnimation)
      (Audio|Components|Audio|SetSound _spawn_audio (Variables|Sounds|GetSpawn%20Error%20Sound))
      (Audio|Components|Audio|Play _spawn_audio 0.0))))

(event EventStoppedReceivingPower
  ;[0 0 0] Stopped Receiving Power
  (CallFunction|ReverseMeshMaterialsAnimation))

(fn ConstructionScript
  (|CallParentFunction)
  (Variables|/Script/Engine.AudioComponent|SetAttenuationSettings (Variables|Default|GetSpawn%20Audio) (Variables|Default|GetSounds%20Attenuation)))