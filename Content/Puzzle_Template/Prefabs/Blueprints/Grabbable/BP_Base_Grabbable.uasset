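; Base Blueprint for grabbable puzzle objects, providing scale-in and scale-out animations and physical impact sounds.
; On BeginPlay it applies the configured sound and attenuation, then optionally grows from near zero to its initial scale via a timeline.
; AnimateDestroy shrinks the actor with a second timeline before destroying it.
; Mesh hits above a speed threshold play the impact sound, throttled by a DoOnce with a short random delay.
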(event OnComponentHit(Mesh)
  (params (HitComponent :type Primitive%20Component%20Object%20Reference) (OtherActor :type Actor%20Object%20Reference) (OtherComp :type Primitive%20Component%20Object%20Reference) (NormalImpulse :type Vector :default "0, 0, 0") (Hit :type Hit%20Result%20Structure%20%28by%20ref%29))
  ;[0 0 0] Play sounds when the grabbable hits something
  (if (Variables|Sounds|GetPlay%20Impact%20Sounds?)
    (if (> (Math|Float|Absolute(Float) (Math|Vector|VectorLength (Transformation|GetComponentVelocity HitComponent))) 125.0)
      (Utilities|FlowControl|DoOnce false :!label _label
        (:Completed
          (Audio|Components|Audio|Play (Variables|Default|GetImpact%20Sounds%20Audio) 0.0)
          (Utilities|FlowControl|Delay (Math|Random|RandomFloatinRange 0.1 0.2))
          (goto _label Reset))))))

(event Custom|Animate%20Destroy
  ;[0 0 0] Destroy Animation
  (Variables|Runtime|SetInitial%20Scale (Transformation|GetActorScale3D))
  (bind _alpha (Timeline|Destroy_Anim_TL PlayFromStart)
    (:Update
      (Transformation|SetActorScale3D (Math|Vector|Lerp(Vector) "0, 0, 0" (Variables|Runtime|GetInitial%20Scale) _alpha)))
    (:Finished
      (Actor|DestroyActor))))

(event EventBeginPlay
  ;[0 0 0] Spawn Animation
  (CallFunction|UpdateSounds)
  (Variables|Runtime|SetInitial%20Scale (Transformation|GetActorScale3D))
  (if (Variables|Settings|GetPlay%20Spawn%20Animation)
    (bind _alpha (Timeline|Spawn_Anim_TL Play)
      (:Update
        (Transformation|SetActorScale3D (Math|Vector|Lerp(Vector) "0.010000,0.010000,0.010000" (Variables|Runtime|GetInitial%20Scale) _alpha))))))

(fn ConstructionScript)

(fn UpdateSounds
  (Audio|Components|Audio|SetSound (Variables|Default|GetImpact%20Sounds%20Audio) (Variables|Sounds|GetImpact%20Sound))
  (Variables|/Script/Engine.AudioComponent|SetAttenuationSettings (Variables|Default|GetImpact%20Sounds%20Audio) (Variables|Sounds|GetImpact%20Attenuation)))