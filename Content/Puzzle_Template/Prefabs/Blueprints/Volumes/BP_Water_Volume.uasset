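; Water volume prefab that makes physics objects float and instantly kills the player on contact via BPC_Player_Health.
; The construction script sizes the box by Depth and offsets it downward.
; Begin play or overlap starts a looping timer that pushes up simulating components whose center of mass is below the Water component and damps their spin.
; The timer clears itself once nothing overlaps the volume.
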(event OnComponentBeginOverlap(Volume)
  (params (OverlappedComponent :type Primitive%20Component%20Object%20Reference) (OtherActor :type Actor%20Object%20Reference) (OtherComp :type Primitive%20Component%20Object%20Reference) (OtherBodyIndex :type Integer) (bFromSweep :type Boolean) (SweepResult :type Hit%20Result%20Structure%20%28by%20ref%29))
  (bind _returnvalue (Actor|GetComponentbyClass OtherActor "/Game/Puzzle_Template/Player/BPC_Player_Health.BPC_Player_Health_C"))
  ;[0 0 0] On Begin Overlap, start pushing overlapping components up.
  (bind _returnvalue_2 (Utilities|Time|SetTimerbyEvent (delegate Custom|Add%20Force%20To%20Overlapping%20Components) 0.01 true))
  (Variables|Runtime|SetTimer%20Handle _returnvalue_2)
  (CallFunction|AddForcetoOverlappingComponents)
  (if (== OtherActor (Game|GetPlayerCharacter 0))
    (Utilities|IsValid _returnvalue
      (:Is%20Valid
        (Default|DealDamage _returnvalue 9999999 self false)))))

(event Custom|Add%20Force%20To%20Overlapping%20Components
  (bind _volume (Variables|Default|GetVolume))
  (bind _outoverlappingcomponents (Class|PrimitiveComponent|GetOverlappingComponents _volume))
  ;[0 0 0] On Begin Overlap, start pushing overlapping components up.
  (if (> (Utilities|Array|Length _outoverlappingcomponents) 0)
    (CallFunction|AddForceUptoComponents _outoverlappingcomponents)
    (else
      (Utilities|Time|ClearandInvalidateTimerbyHandle (Variables|Runtime|GetTimer%20Handle)))))

(event EventBeginPlay
  ;[0 0 0] On begin play, check whether or not we are overlapping any component, and start the time if we are.
  (if (> (Utilities|Array|Length (Class|PrimitiveComponent|GetOverlappingComponents (Variables|Default|GetVolume))) 0)
    ;[0 0 0] On Begin Overlap, start pushing overlapping components up.
    (bind _returnvalue (Utilities|Time|SetTimerbyEvent (delegate Custom|Add%20Force%20To%20Overlapping%20Components) 0.01 true))
    (Variables|Runtime|SetTimer%20Handle _returnvalue)
    (CallFunction|AddForcetoOverlappingComponents)
    (if (== (stale OnComponentBeginOverlap(Volume) OtherActor) (Game|GetPlayerCharacter 0))
      (Utilities|IsValid (Actor|GetComponentbyClass (stale OnComponentBeginOverlap(Volume) OtherActor) "/Game/Puzzle_Template/Player/BPC_Player_Health.BPC_Player_Health_C")
        (:Is%20Valid
          (Default|DealDamage (Actor|GetComponentbyClass (stale OnComponentBeginOverlap(Volume) OtherActor) "/Game/Puzzle_Template/Player/BPC_Player_Health.BPC_Player_Health_C") 9999999 self false))))))

(fn ConstructionScript
  (Components|Box|SetBoxExtent (Variables|Default|GetVolume) (Math|Vector|MakeVector 5e+01 5e+01 (Variables|Default|GetDepth)) true)
  (Transformation|SetRelativeLocation (Variables|Default|GetVolume) (Math|Vector|MakeVector 0.0 0.0 (* (Variables|Default|GetDepth) -1.0)) false false))

(fn AddForceUptoComponents
  (params (Components :type Array%20of%20Primitive%20Component%20Object%20References))
  (for _array_element Components
    (if (Physics|IsSimulatingPhysics _array_element "None")
      (if (< (.Z (Math|Vector|BreakVector (Physics|GetCenterOfMass _array_element "None"))) (.Z (Math|Vector|BreakVector (Transformation|GetWorldLocation (Variables|Default|GetWater)))))
        (Physics|AddForce _array_element (Math|Vector|MakeVector 0.0 0.0 (/ (Variables|Default|GetForce%20Multiplier) (Utilities|Time|GetWorldDeltaSeconds))) "None" true)
        (Class|PrimitiveComponent|SetAllPhysicsAngularVelocityinDegrees _array_element (/ (Physics|GetPhysicsAngularVelocityinDegrees _array_element "None") 1.01) false)))))