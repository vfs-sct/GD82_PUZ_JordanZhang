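; BP_Blocking_Volume is a puzzle template volume that selectively blocks the player, physics objects, lasers or everything, according to its Type.
; UpdateType picks the mesh material from a Materials map keyed by Type, with a default fallback.
; Construction updates only the material for editor preview.
; BeginPlay also sets collision, ignoring all channels and then blocking Pawn, PhysicsBody, GameTraceChannel2 (lasers) or all channels.
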(event EventBeginPlay
  (CallFunction|UpdateType false))

(fn ConstructionScript
  (CallFunction|UpdateType true))

(fn UpdateType
  (params (Only%20Update%20Material? :type Boolean))
  (bind _type (Variables|Settings|GetType))
  (bind _materials (Variables|Settings|GetMaterials))
  (bind (_value _returnvalue) (Utilities|Map|Find _materials _type))
  (if _returnvalue
    (Rendering|Material|SetMaterial (Variables|Default|GetMesh) 0 _value)
    (else
      (Rendering|Material|SetMaterial (Variables|Default|GetMesh) 0 "/Game/Puzzle_Template/zIgnore/Assets/Blocking_Volumes/PT_Blocking_Volume_M.PT_Blocking_Volume_M")))
  (if (not Only%20Update%20Material?)
    (Collision|SetCollisionResponsetoAllChannels (Variables|Default|GetMesh) "ECR_Ignore")
    (switch Utilities|FlowControl|Switch|SwitchonPT_Blocking_Volume_Type_Enum (Variables|Settings|GetType)
      (:NewEnumerator0
        (Collision|SetCollisionResponsetoChannel (Variables|Default|GetMesh) "ECC_Pawn" "ECR_Block"))
      (:NewEnumerator1
        (Collision|SetCollisionResponsetoChannel (Variables|Default|GetMesh) "ECC_PhysicsBody" "ECR_Block"))
      (:NewEnumerator2
        (Collision|SetCollisionResponsetoChannel (Variables|Default|GetMesh) "ECC_GameTraceChannel2" "ECR_Block"))
      (:NewEnumerator3
        (Collision|SetCollisionResponsetoAllChannels (Variables|Default|GetMesh) "ECR_Block")))))