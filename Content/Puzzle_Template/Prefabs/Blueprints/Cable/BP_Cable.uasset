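; BP_Cable is a spline-based cable prop for puzzles that animates when it receives or stops receiving power.
; Construction makes spline points linear, then places a stretched, rotated mesh between each pair, plus joint meshes at interior points and optionally at either end.
; Segments share one dynamic material instance.
; The power events play or reverse a timeline that drives that material's State parameter.
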(event EventReceivingPower
  ;[0 0 0] Animate the cable when it receives power or stops receiving power.
  (bind _alpha (Timeline|Cables_Power_Anim Play)
    (:Update
      (Rendering|Material|SetScalarParameterValue (Variables|Runtime|GetCable%20Material%20Instance) "State" _alpha :!class /Script/Engine.MaterialInstanceDynamic))))

(event EventStoppedReceivingPower
  ;[0 0 0] Animate the cable when it receives power or stops receiving power.
  (bind _alpha (Timeline|Cables_Power_Anim Reverse)
    (:Update
      (Rendering|Material|SetScalarParameterValue (Variables|Runtime|GetCable%20Material%20Instance) "State" _alpha :!class /Script/Engine.MaterialInstanceDynamic))))

(fn ConstructionScript
  (CallFunction|UpdateCable))

(fn UpdateCable
  (bind _cable_scale (Variables|Settings|GetCable%20Scale))
  (bind _returnvalue (Rendering|Material|CreateDynamicMaterialInstance "/Game/Puzzle_Template/zIgnore/Materials/PT_Power_MI.PT_Power_MI" "None" "None" :!class /Script/Engine.KismetMaterialLibrary))
  (Variables|Runtime|SetCable%20Material%20Instance _returnvalue)
  (for _index (range 0 (- (Spline|GetNumberOfSplinePoints (Variables|Default|GetCable%20Spline)) 1))
    (LocalVariables|SetLocal%20Index _index)
    (Spline|SetSplinePointType (Variables|Default|GetCable%20Spline) (LocalVariables|GetLocal%20Index) "Linear" true)
    (if (!= (LocalVariables|GetLocal%20Index) (- (Spline|GetNumberOfSplinePoints (Variables|Default|GetCable%20Spline)) 1))
      (bind _returnvalue_2 (AddComponent|AddStaticMeshComponent false (Math|Transform|MakeTransform (/ (+ (Spline|GetLocationatSplinePoint (Variables|Default|GetCable%20Spline) (LocalVariables|GetLocal%20Index) "Local") (Math|Vector|SelectVector (Spline|GetLocationatSplinePoint (Variables|Default|GetCable%20Spline) (+ (LocalVariables|GetLocal%20Index) 1) "Local") "0, 0, 0" (!= (LocalVariables|GetLocal%20Index) (- (Spline|GetNumberOfSplinePoints (Variables|Default|GetCable%20Spline)) 1)))) 2.0) (Math|Rotator|FindLookatRotation (Spline|GetLocationatSplinePoint (Variables|Default|GetCable%20Spline) (LocalVariables|GetLocal%20Index) "Local") (Math|Vector|SelectVector (Spline|GetLocationatSplinePoint (Variables|Default|GetCable%20Spline) (+ (LocalVariables|GetLocal%20Index) 1) "Local") "0, 0, 0" (!= (LocalVariables|GetLocal%20Index) (- (Spline|GetNumberOfSplinePoints (Variables|Default|GetCable%20Spline)) 1)))) (Math|Vector|MakeVector (* (Math|Vector|Distance(Vector) (Spline|GetLocationatSplinePoint (Variables|Default|GetCable%20Spline) (LocalVariables|GetLocal%20Index) "Local") (Math|Vector|SelectVector (Spline|GetLocationatSplinePoint (Variables|Default|GetCable%20Spline) (+ (LocalVariables|GetLocal%20Index) 1) "Local") "0, 0, 0" (!= (LocalVariables|GetLocal%20Index) (- (Spline|GetNumberOfSplinePoints (Variables|Default|GetCable%20Spline)) 1)))) 0.2) _cable_scale _cable_scale))))
      (Rendering|Material|SetMaterial _returnvalue_2 0 (Variables|Runtime|GetCable%20Material%20Instance))
      (if (== (LocalVariables|GetLocal%20Index) 0)
        (if (Variables|Settings|GetShow%20End%20Joint?)
          (AddComponent|AddStaticMeshComponent false (Math|Transform|MakeTransform (Spline|GetLocationatSplinePoint (Variables|Default|GetCable%20Spline) (LocalVariables|GetLocal%20Index) "Local") "0, 0, 0" (Math|Conversions|ToVector(Float) (Variables|Settings|GetCable%20Scale))) :!label _label))
        (else
          (goto _label)))
      (elif (Variables|Settings|GetShow%20Start%20Joint?)
        (goto _label)))))