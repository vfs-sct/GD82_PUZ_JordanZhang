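; Puzzle template checkpoint that activates once when the player overlaps it, recording its ID as the game mode's current checkpoint.
; Activation also optionally shows a popup, powers down listed actors through the power receiver interface, fires a checkpoint-activated call and can clear portal-gun portals.
; The construction script previews the spawn point with a capsule at an offset, optionally ground-snapped by a downward trace, and labels the checkpoint with its ID.
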(event Collision|EventActorBeginOverlap
  (params (OtherActor :type Actor%20Object%20Reference))
  (bind _returnvalue (Game|GetPlayerCharacter 0))
  (bind _returnvalue_2 (Actor|GetComponentbyClass _returnvalue "/Game/Puzzle_Template/Portals/Portal_Gun/BPC_Portals_Gun.BPC_Portals_Gun_C"))
  ;[0 0 0] On Begin Overlap, when the player overlaps this checkpoint, activate it and unpower all the actors to unpower.
  (if (== OtherActor (Game|GetPlayerCharacter 0))
    (if (not (Variables|Runtime|GetIs%20Activated?))
      (Variables|Runtime|SetIs%20Activated? true)
      (Utilities|UpdateGamemodeIndex)
      (Utilities|ShowCheckpointPopupText)
      (Utilities|UnpowerActors)
      (Default|CallCheckpointActivated)
      (if (Variables|Settings|GetClear%20Portals?)
        (Utilities|IsValid _returnvalue_2
          (:Is%20Valid
            (Default|ClearPortals _returnvalue_2)))))))

(fn ConstructionScript
  (bind _capsule (Variables|Default|GetCapsule))
  (bind _returnvalue (Utilities|GetPlayerSpawnLocation 8e+01 2e+01))
  (Transformation|SetWorldLocation _capsule _returnvalue false false)
  (Transformation|SetRelativeRotation _capsule (Math|Rotator|MakeRotator 0.0 0.0 (Variables|PlayerSettings|GetPlayer%20Spawn%20Yaw%20Offset)) false false)
  (Rendering|Components|TextRender|SetText (Variables|Default|GetTextRenderer) (Utilities|Text|ToText(String) (Utilities|String|Append "Checkpoint ID: " (Utilities|String|ToString(Integer) (Variables|Settings|GetCheckpoint%20ID))))))

(fn GetPlayerSpawnLocation
  (params (Capsule%20Half%20Height :type Float%20%28double-precision%29) (Capsule%20Radius :type Float%20%28double-precision%29))
  (bind _returnvalue (Transformation|GetActorLocation))
  (bind _player_spawn_offset (Variables|PlayerSettings|GetPlayer%20Spawn%20Offset))
  (bind _returnvalue_2 (+ _player_spawn_offset _returnvalue))
  (if (Variables|PlayerSettings|GetSnap%20Player%20To%20Ground?)
    (bind _outhit (Collision|LineTraceByChannel _returnvalue_2 (+ _returnvalue_2 (* (Math|Vector|VectorUp) -1e+04)) "TraceTypeQuery1" true 0 "None"))
    (return (+ (Math|Vector|SelectVector (.Location (Collision|BreakHitResult _outhit)) (.TraceEnd (Collision|BreakHitResult _outhit)) (.bBlockingHit (Collision|BreakHitResult _outhit))) (Math|Vector|MakeVector 0.0 0.0 Capsule%20Half%20Height)))
    (else
      (return (+ (Variables|PlayerSettings|GetPlayer%20Spawn%20Offset) (Transformation|GetActorLocation))))))

(fn UpdateGamemodeIndex
  (bind _asgm_game_scene (Utilities|Casting|CastToGM_GameScene (Game|GetGameMode)))
  (Variables|/Game/Puzzle_Template/Gamemodes/GM_GameScene.GM_GameScene_C|SetCurrent%20Checkpoint%20ID _asgm_game_scene (Variables|Settings|GetCheckpoint%20ID)))

(fn UnpowerActors
  (for _array_element (Variables|Settings|GetActors%20To%20Unpower)
    (if (Utilities|DoesObjectImplementInterface _array_element "/Game/Puzzle_Template/Prefabs/Blueprints/Interfaces/PT_Power_Receiver_BPI.PT_Power_Receiver_BPI_C")
      (Class|PTPowerReceiverBPI|OnPowerStop(Message) _array_element))))

(fn ShowCheckpointPopupText
  ;[0 0 0] Show a checkpoint text popup if enabled
  (if (Variables|Settings|GetShow%20Popup%20Text%20On%20Activation?)
    (bind _returnvalue (UserInterface|CreateWidget "/Game/Puzzle_Template/Prefabs/Blueprints/Widgets/PT_Checkpoint_Text_Popup_WB.PT_Checkpoint_Text_Popup_WB_C" 0 (Variables|Settings|GetPopup%20Text)))
    (UserInterface|Viewport|AddtoViewport _returnvalue 0)))