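; BP_Pressure_Plate is a puzzle pressure plate that powers an array of linked actors while something overlaps its collision box.
; The first overlap turns power on and plays a timeline that lowers the button and drives the back panel material's State parameter.
; When the last overlap ends, it cuts power and reverses the timeline.
; Two cross-resetting DoOnce gates keep each transition from repeating with multiple overlaps.
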(event OnComponentBeginOverlap(CollisionBox)
  (params (OverlappedComponent :type Primitive%20Component%20Object%20Reference) (OtherActor :type Actor%20Object%20Reference) (OtherComp :type Primitive%20Component%20Object%20Reference) (OtherBodyIndex :type Integer) (bFromSweep :type Boolean) (SweepResult :type Hit%20Result%20Structure%20%28by%20ref%29))
  ;[0 0 0] On Begin Overlap with the collision box, give power to all actors in the array, then play an animation.
  (Utilities|FlowControl|Sequence
    (:then_0
      (Utilities|FlowControl|DoOnce false
        (:Completed
          (CallFunction|TogglePowertoActors true (Variables|Default|GetActors%20To%20Power))
          (bind _alpha (Timeline|Lower_Button Play)
            (:Update
              (Transformation|SetRelativeLocation (Variables|Components|GetButton) (Math|Vector|Lerp(Vector) "0.000000,0.000000,20.000000" "0.000000,0.000000,16.000000" _alpha) false false)
              (Rendering|Material|SetScalarParameterValueonMaterials (Variables|Components|GetBack%20Panel) "State" _alpha))))))
    (:then_1
      (Utilities|FlowControl|DoOnce false) ; enters at Reset
    )))

(event OnComponentEndOverlap(CollisionBox)
  (params (OverlappedComponent :type Primitive%20Component%20Object%20Reference) (OtherActor :type Actor%20Object%20Reference) (OtherComp :type Primitive%20Component%20Object%20Reference) (OtherBodyIndex :type Integer))
  ;[0 0 0] On Begin Overlap with the collision box, give power to all actors in the array, then play an animation.
  (if (== (Utilities|Array|Length (Class|PrimitiveComponent|GetOverlappingComponents (Variables|Components|GetCollision%20Box))) 0)
    (Utilities|FlowControl|Sequence
      (:then_0
        (Utilities|FlowControl|DoOnce false
          (:Completed
            (CallFunction|TogglePowertoActors false (Variables|Default|GetActors%20To%20Power))
            (bind _alpha (Timeline|Lower_Button Reverse)
              (:Update
                (Transformation|SetRelativeLocation (Variables|Components|GetButton) (Math|Vector|Lerp(Vector) "0.000000,0.000000,20.000000" "0.000000,0.000000,16.000000" _alpha) false false)
                (Rendering|Material|SetScalarParameterValueonMaterials (Variables|Components|GetBack%20Panel) "State" _alpha))))))
      (:then_1
        (Utilities|FlowControl|DoOnce false) ; enters at Reset
      ))))

(fn ConstructionScript
  (|CallParentFunction))