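; Battery socket for puzzles that powers its linked actors while a charged battery is inserted.
; An overlapping grabbable battery is released from the grab, has physics disabled and is eased into place in two moves.
; A charged battery starts draining, toggles power on and plays a timeline driving the mesh's "State" material parameter.
; Battery dispatchers for grabbed, died and destroyed cut power and reverse that animation.
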(event OnComponentBeginOverlap(BatteryDetectionBox)
  (params (OverlappedComponent :type Primitive%20Component%20Object%20Reference) (OtherActor :type Actor%20Object%20Reference) (OtherComp :type Primitive%20Component%20Object%20Reference) (OtherBodyIndex :type Integer) (bFromSweep :type Boolean) (SweepResult :type Hit%20Result%20Structure%20%28by%20ref%29))
  (bind _battery_location_2 (Variables|Default|GetBattery%20Location%202))
  (bind _battery_location_1 (Variables|Default|GetBattery%20Location%201))
  (bind _returnvalue (Transformation|GetWorldTransform _battery_location_1))
  (bind _returnvalue_2 (Transformation|GetWorldTransform _battery_location_2))
  (bind (_location _rotation) (Math|Transform|BreakTransform _returnvalue))
  (bind (_location_2 _rotation_2) (Math|Transform|BreakTransform _returnvalue_2))
  ;[0 0 0] If a battery is detected, move it to the correct location and start giving power to the actors to power.
  (Utilities|IsValid (Variables|Default|GetCurrent%20Battery)
    (:Is%20Not%20Valid
      (bind _asbp_battery_grabbable (Utilities|Casting|CastToBP_Battery_Grabbable OtherActor))
      (bind _output_get (Variables|Default|SetCurrent%20Battery _asbp_battery_grabbable))
      (bind _grab_component (Variables|/Game/Puzzle_Template/Prefabs/Blueprints/Battery/BP_Battery_Grabbable.BP_Battery_Grabbable_C|GetGrab%20Component _output_get)
        (:then
          (Default|EndGrab _grab_component)
          (Collision|SetActorEnableCollision (Variables|Default|GetCurrent%20Battery) false)
          (Physics|SetSimulatePhysics (Variables|/Game/Puzzle_Template/Prefabs/Blueprints/Grabbable/BP_Base_Grabbable.BP_Base_Grabbable_C|GetMesh _output_get) false)
          (Components|MoveComponentTo (Variables|/Game/Puzzle_Template/Prefabs/Blueprints/Grabbable/BP_Base_Grabbable.BP_Base_Grabbable_C|GetMesh _output_get) _location _rotation true true 0.4 true)
          (Utilities|FlowControl|Delay 0.1)
          (Components|MoveComponentTo (Variables|/Game/Puzzle_Template/Prefabs/Blueprints/Grabbable/BP_Base_Grabbable.BP_Base_Grabbable_C|GetMesh _output_get) _location_2 _rotation_2 false true 0.125 true)
          (Collision|SetActorEnableCollision (Variables|Default|GetCurrent%20Battery) true)
          (if (> (Variables|/Game/Puzzle_Template/Prefabs/Blueprints/Battery/BP_Battery_Grabbable.BP_Battery_Grabbable_C|GetCurrent%20Charge (Variables|Default|GetCurrent%20Battery)) 0.0)
            (Default|InitConsumeBattery (Variables|Default|GetCurrent%20Battery))
            (CallFunction|TogglePowertoActors true (Variables|Default|GetActors%20To%20Power))
            (CallFunction|PlayMeshMaterialsAnimation)
            (EventDispatchers|AssignOnGrabbed (Variables|Default|GetCurrent%20Battery) (EventDispatchers|CreateEvent :!event Custom|On%20Current%20Battery%20Grabbed))
            (EventDispatchers|AssignOnBatteryDied (Variables|Default|GetCurrent%20Battery) (EventDispatchers|CreateEvent :!event Custom|On%20Current%20Battery%20Died))
            (EventDispatchers|BindEventtoOnBatteryDestroyed (Variables|Default|GetCurrent%20Battery) (EventDispatchers|CreateEvent :!event Custom|On%20Battery%20Destroyed))
            (else
              (Audio|Components|Audio|SetSound (Variables|Default|GetPower%20Audio) (Variables|Default|GetGiving%20Power%20Sound))
              (Audio|Components|Audio|Play (Variables|Default|GetPower%20Audio) 0.0)
              (EventDispatchers|AssignOnGrabbed (Variables|Default|GetCurrent%20Battery) (EventDispatchers|CreateEvent :!event Custom|On%20Current%20Battery%20Grabbed)))))
        (:else
          (Variables|Default|SetCurrent%20Battery 0))))))

(event Custom|Play%20Mesh%20Materials%20Animation
  ;[0 0 0] Animate the state of the materials included in the mesh
  (bind _alpha (Timeline|Animate_Mesh_Materials Play)
    (:Update
      (Rendering|Material|SetScalarParameterValueonMaterials (Variables|Default|GetMesh) "State" _alpha))))

(event Custom|Reverse%20Mesh%20Materials%20Animation
  ;[0 0 0] Animate the state of the materials included in the mesh
  (bind _alpha (Timeline|Animate_Mesh_Materials Reverse)
    (:Update
      (Rendering|Material|SetScalarParameterValueonMaterials (Variables|Default|GetMesh) "State" _alpha))))

(event Custom|On%20Current%20Battery%20Grabbed
  ;[0 0 0] Instantly stops giving power if the connected battery gets grabbed.
  (Default|UnbindAllDispatchers (Variables|Default|GetCurrent%20Battery))
  (Physics|SetSimulatePhysics (Variables|/Game/Puzzle_Template/Prefabs/Blueprints/Grabbable/BP_Base_Grabbable.BP_Base_Grabbable_C|GetMesh (Variables|Default|GetCurrent%20Battery)) true)
  (Default|StopConsumeBattery (Variables|Default|GetCurrent%20Battery))
  (CallFunction|ReverseMeshMaterialsAnimation)
  (if (> (Variables|/Game/Puzzle_Template/Prefabs/Blueprints/Battery/BP_Battery_Grabbable.BP_Battery_Grabbable_C|GetCurrent%20Charge (Variables|Default|GetCurrent%20Battery)) 0.0)
    (CallFunction|TogglePowertoActors false (Variables|Default|GetActors%20To%20Power)))
  (Variables|Default|SetCurrent%20Battery 0))

(event Custom|On%20Current%20Battery%20Died
  ;[0 0 0] This event is called by the PT_Battery_BP when it runs out of charge, when this happen remove power from any connected actor.
  (EventDispatchers|UnbindEventfromOnBatteryDied (Variables|Default|GetCurrent%20Battery) (delegate Custom|On%20Current%20Battery%20Died))
  (CallFunction|TogglePowertoActors false (Variables|Default|GetActors%20To%20Power))
  (CallFunction|ReverseMeshMaterialsAnimation))

(event Custom|On%20Battery%20Destroyed
  ;[0 0 0] Instantly stops giving power if the connected battery gets destroyed.
  (Default|UnbindAllDispatchers (Variables|Default|GetCurrent%20Battery))
  (CallFunction|ReverseMeshMaterialsAnimation)
  (if (> (Variables|/Game/Puzzle_Template/Prefabs/Blueprints/Battery/BP_Battery_Grabbable.BP_Battery_Grabbable_C|GetCurrent%20Charge (Variables|Default|GetCurrent%20Battery)) 0.0)
    (CallFunction|TogglePowertoActors false (Variables|Default|GetActors%20To%20Power))))

(fn ConstructionScript
  (|CallParentFunction))