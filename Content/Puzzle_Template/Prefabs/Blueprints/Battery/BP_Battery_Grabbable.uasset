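; A grabbable puzzle battery that holds a charge, drains it over a set duration unless infinite, and shows it on its materials.
; A timeline, rate-scaled and resumed from the current charge, updates progress and connector material parameters, mirrored by component tag onto the portal clone meshes when in range.
; It stores its grab component for battery slots and notifies them through dispatchers when grabbed, depleted or destroyed.
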(event InPortalRange(PT_Portable_AC)
  ;[0 0 0] When we enter or leave a portal range, toggle the actor tick so that we can update the state of the clone mesh.
  (CallFunction|UpdateProgressMaterials))

(event Custom|Init%20Consume%20Battery
  ;[0 0 0] Timeline to slowly decrease the battery charge based on the duration
  (if (not (Variables|Settings|GetInfinite%20Charge?))
    (Components|Timeline|SetPlayRate (Variables|Default|GetConsume_Battery_TL) (/ 1.0 (Variables|Settings|GetCharge%20Duration)))
    (Components|Timeline|SetNewTime (Variables|Default|GetConsume_Battery_TL) (Math|Float|MapRangeClamped (Variables|Settings|GetCurrent%20Charge) 0.0 1.0 1.0 0.0))
    (bind _percent (Timeline|Consume_Battery_TL Play)
      (:Update
        (Variables|Settings|SetCurrent%20Charge _percent)
        (CallFunction|UpdateProgressMaterials))
      (:Finished
        (if (<= (Variables|Settings|GetCurrent%20Charge) 0.0)
          (Default|CallOnBatteryDied))))))

(event Custom|Stop%20Consume%20Battery
  ;[0 0 0] Timeline to slowly decrease the battery charge based on the duration
  (bind _percent (Timeline|Consume_Battery_TL Stop)
    (:Update
      (Variables|Settings|SetCurrent%20Charge _percent)
      (CallFunction|UpdateProgressMaterials))
    (:Finished
      (if (<= (Variables|Settings|GetCurrent%20Charge) 0.0)
        (Default|CallOnBatteryDied)))))

(event EventAnimateDestroy
  ;[0 0 0] If the battery gets destroyed, call the "On Battery Destroyed" dispatcher, this will notify battery slots in case this battery is connected.
  (|CallParentFunction)
  (Utilities|FlowControl|DoOnce false
    (:Completed
      (Default|CallOnBatteryDestroyed))))

(event EventDestroyed
  ;[0 0 0] If the battery gets destroyed, call the "On Battery Destroyed" dispatcher, this will notify battery slots in case this battery is connected.
  (Utilities|FlowControl|DoOnce false
    (:Completed
      (Default|CallOnBatteryDestroyed))))

(event EventOnBeginGrab
  (params (Grab%20Component :type BPC%20Interaction%20and%20Grab%20Object%20Reference))
  ;[0 0 0] Save a grab component variable, this will be used by "PT_Battery_Slots"
  (|CallParentFunction Grab%20Component)
  (Variables|Runtime|SetGrab%20Component Grab%20Component)
  (Default|CallOnGrabbed))

(event EventOnEndGrab
  ;[0 0 0] Save a grab component variable, this will be used by "PT_Battery_Slots"
  (|CallParentFunction)
  (Variables|Runtime|SetGrab%20Component 0))

(fn ConstructionScript
  (CallFunction|UpdateProgressMaterials))

(fn UpdateProgressMaterials
  (bind _pt_portable_ac (Variables|Default|GetPT_Portable_AC))
  (Utilities|FlowControl|Sequence
    (:then_0
      (Rendering|Material|SetScalarParameterValueonMaterials (Variables|Default|GetBattery_Progress) "Percent" (Variables|Settings|GetCurrent%20Charge))
      (Rendering|Material|SetScalarParameterValueonMaterials (Variables|Default|GetBattery_Progress) "State" 1.0)
      (Rendering|Material|SetScalarParameterValueonMaterials (Variables|Default|GetBattery_Connector) "State" (Math|Float|SelectFloat 0.0 1.0 (<= (Variables|Settings|GetCurrent%20Charge) 0.0))))
    (:then_1
      (if (Variables|/Game/Puzzle_Template/Portals/BPC_Portable.BPC_Portable_C|GetIs%20In%20Portal%20Range? _pt_portable_ac)
        (bind _output_get (LocalVariables|SetLocalCloneComponents (Components|GetChildrenComponents (Variables|/Game/Puzzle_Template/Portals/BPC_Portable.BPC_Portable_C|GetClone%20Root _pt_portable_ac) false)))
        (for _array_element _output_get
          (bind _asstatic_mesh_component (Utilities|Casting|CastToStaticMeshComponent _array_element))
          (switch name (Utilities|Array|Get(acopy) (Variables|/Script/Engine.ActorComponent|GetComponentTags _asstatic_mesh_component))
            (:Progress
              (Rendering|Material|SetScalarParameterValueonMaterials _asstatic_mesh_component "Percent" (Variables|Settings|GetCurrent%20Charge))
              (Rendering|Material|SetScalarParameterValueonMaterials _asstatic_mesh_component "State" 1.0))
            (:Input
              (Rendering|Material|SetScalarParameterValueonMaterials _asstatic_mesh_component "State" (Math|Float|SelectFloat 0.0 1.0 (<= (Variables|Settings|GetCurrent%20Charge) 0.0))))))))))

(fn UnbindAllDispatchers
  (EventDispatchers|UnbindallEventsfromOnGrabbed)
  (EventDispatchers|UnbindallEventsfromOnBatteryDied)
  (EventDispatchers|UnbindallEventsfromOnBatteryDestroyed))