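; Launchpad puzzle prefab that, while powered or always powered, launches overlapping characters and physics-simulating objects.
; LaunchActor takes velocity from the pad's up vector or predicts an arc to TargetLocation, with optional velocity overrides and spin for physics objects.
; Characters can lose move input until they hit something or teleport via BPC_Portable.
; Timelines animate material power and launch states; the construction script orients the direction arrow and sets initial power.
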(event Custom|Play%20Mesh%20Materials%20Animation
  ;[0 0 0] Animate the state of the materials included in the mesh
  (bind _alpha (Timeline|Animate_Mesh_Materials Play)
    (:Update
      (Rendering|Material|SetScalarParameterValueonMaterials (Variables|Default|GetMesh) "State" _alpha))))

(event Custom|Reverse%20Mesh%20Materials%20Animation
  ;[0 0 0] Animate the state of the materials included in the mesh
  (bind _alpha (Timeline|Animate_Mesh_Materials Reverse)
    (:Update
      (Rendering|Material|SetScalarParameterValueonMaterials (Variables|Default|GetMesh) "State" _alpha))))

(event Custom|Play%20Mesh%20Launch%20Materials%20Animation
  ;[0 0 0] Animate the launch state of the materials.
  (bind _alpha (Timeline|Launch_Animate_Mesh_Materials PlayFromStart)
    (:Update
      (Rendering|Material|SetScalarParameterValueonMaterials (Variables|Default|GetMesh) "Launch State" _alpha))))

(event Custom|Stop%20Mesh%20Launch%20Materials%20Animation
  ;[0 0 0] Animate the launch state of the materials.
  (bind _alpha (Timeline|Launch_Animate_Mesh_Materials Stop)
    (:Update
      (Rendering|Material|SetScalarParameterValueonMaterials (Variables|Default|GetMesh) "Launch State" _alpha))))

(event Collision|EventActorBeginOverlap
  (params (OtherActor :type Actor%20Object%20Reference))
  ;[0 0 0] Launch actors that start overlapping.
  (if (Variables|Runtime|GetActivated)
    (Utilities|LaunchActor OtherActor)))

(event EventReceivingPower
  (bind _launchpad_detection (Variables|Default|GetLaunchpad_Detection))
  ;[0 0 0] Receiving Power
  (if (not (Variables|Settings|GetAlways%20Powered?))
    (CallFunction|PlayMeshMaterialsAnimation)
    (Variables|Runtime|SetActivated true)
    (bind _outactors (Collision|ComponentOverlapActors _launchpad_detection (Transformation|GetWorldTransform _launchpad_detection) (Utilities|Array|MakeArray "ObjectTypeQuery3" "ObjectTypeQuery4") "/Script/Engine.Actor" (Utilities|Array|MakeArray self)))
    (for _array_element _outactors
      (Utilities|LaunchActor _array_element))))

(event EventStoppedReceivingPower
  ;[0 0 0] Stopped Receiving Power
  (if (not (Variables|Settings|GetAlways%20Powered?))
    (CallFunction|ReverseMeshMaterialsAnimation)
    (CallFunction|StopMeshLaunchMaterialsAnimation)
    (Variables|Runtime|SetActivated false)
    (Rendering|Material|SetScalarParameterValueonMaterials (Variables|Default|GetMesh) "Launch State" 0.0)))

(fn ConstructionScript
  (bind _mesh (Variables|Default|GetMesh))
  (bind _pt_launch_sound_cue (Variables|Default|GetPT_Launch_Sound_Cue))
  (bind _target_location (Variables|Settings|GetTarget%20Location))
  (bind (_x _y) (Math|Vector|BreakVector _target_location))
  (|CallParentFunction)
  (Rendering|Material|SetScalarParameterValueonMaterials _mesh "Direction Arrow Angle" (Class|KismetMathLibrary|ClampAxis (.Yaw (Math|Rotator|BreakRotator (Math|Rotator|Delta(Rotator) (Math|Conversions|RotationFromXVector (* (Transformation|GetActorRightVector) -1.0)) (Math|Conversions|RotationFromXVector (Math|Vector|GetUnitDirection(Vector) (Transformation|GetActorLocation) (+ (Variables|Settings|GetTarget%20Location) (Transformation|GetActorLocation)))))))))
  (Rendering|Material|SetScalarParameterValueonMaterials _mesh "Direction Arrow Opacity Multiplier" (Math|Conversions|ToFloat(Boolean) (and (or (!= _x 0.0) (!= _y 0.0)) (Utilities|Enum|NotEqual(Enum) (Variables|Settings|GetLaunch%20Type) "NewEnumerator0"))))
  (Audio|Components|Audio|SetSound _pt_launch_sound_cue (Variables|Sounds|GetLaunch%20Sound))
  (Variables|/Script/Engine.AudioComponent|SetAttenuationSettings _pt_launch_sound_cue (Variables|Default|GetSounds%20Attenuation))
  (if (Variables|Settings|GetAlways%20Powered?)
    (Variables|Runtime|SetActivated true)
    (Rendering|Material|SetScalarParameterValueonMaterials (Variables|Default|GetMesh) "State" 1.0)
    (else
      (Variables|Runtime|SetActivated false)
      (Rendering|Material|SetScalarParameterValueonMaterials (Variables|Default|GetMesh) "State" 0.0))))

(fn LaunchActor
  (params (Actor :type Actor%20Object%20Reference))
  (bind _ascharacter (Utilities|Casting|CastToCharacter Actor)
    (:then
      (bind _output_get (LocalVariables|SetLocalCharacter _ascharacter))
      (LocalVariables|SetLocalCharacterGravityZ (Components|Movement|GetGravityZ (Variables|/Script/Engine.Character|GetCharacterMovement _output_get)))
      (CallFunction|PlayMeshLaunchMaterialsAnimation)
      (if (Variables|Sounds|GetPlay%20Launch%20Sound?)
        (Audio|Components|Audio|Play (Variables|Default|GetPT_Launch_Sound_Cue) 0.0))
      (switch Utilities|FlowControl|Switch|SwitchonPT_Launchpad_Launch_Type_Enum (Variables|Settings|GetLaunch%20Type)
        (:NewEnumerator0
          (LocalVariables|SetLocalEndVelocity (* (Math|Vector|GetUpVector (Variables|Default|GetMesh)) (Variables|Settings|GetLaunch%20Force))))
        (:NewEnumerator1
          (bind _tossvelocity (Class|GameplayStatics|BlueprintSuggestProjectileVelocity (Transformation|GetActorLocation (LocalVariables|GetLocalCharacter)) (+ (Transformation|GetActorLocation) (Variables|Settings|GetTarget%20Location)) (Variables|Settings|GetLaunch%20Force) (LocalVariables|GetLocalCharacterGravityZ) "DoNotTrace" 0.0 false false false))
          (LocalVariables|SetLocalEndVelocity _tossvelocity))
        (:NewEnumerator2
          (bind _outlaunchvelocity (Game|SuggestProjectileVelocityCustomArc (Transformation|GetActorLocation (LocalVariables|GetLocalCharacter)) (+ (Transformation|GetActorLocation) (Variables|Settings|GetTarget%20Location)) (LocalVariables|GetLocalCharacterGravityZ) (Variables|Settings|GetCustom%20Arc)))
          (LocalVariables|SetLocalEndVelocity _outlaunchvelocity)))
      (Character|LaunchCharacter (LocalVariables|GetLocalCharacter) (LocalVariables|GetLocalEndVelocity) (Variables|Settings|GetOverride%20XY%20Velocity?) (Variables|Settings|GetOverride%20Z%20Velocity?))
      (if (and (Variables|Settings|Character|GetDisable%20Move%20Input?) (or (Variables|Settings|Character|GetReset%20Move%20Input%20On%20Collision?) (Variables|Settings|Character|GetReset%20Move%20Input%20On%20Teleported?)))
        (Utilities|IsValid (Pawn|GetController (LocalVariables|GetLocalCharacter))
          (:Is%20Valid
            (Input|SetIgnoreMoveInput (Pawn|GetController (LocalVariables|GetLocalCharacter)) true)
            (Utilities|FlowControl|Sequence
              (:then_0
                (if (Variables|Settings|Character|GetReset%20Move%20Input%20On%20Collision?)
                  (Collision|BindEventtoOnActorHit (LocalVariables|GetLocalCharacter) (EventDispatchers|CreateEvent :!event LaunchedCharacterHit))))
              (:then_1
                (if (Variables|Settings|Character|GetReset%20Move%20Input%20On%20Teleported?)
                  (Utilities|IsValid (Actor|GetComponentbyClass (LocalVariables|GetLocalCharacter) "/Game/Puzzle_Template/Portals/BPC_Portable.BPC_Portable_C")
                    (:Is%20Valid
                      (EventDispatchers|BindEventtoTeleported (Actor|GetComponentbyClass (LocalVariables|GetLocalCharacter) "/Game/Puzzle_Template/Portals/BPC_Portable.BPC_Portable_C") (EventDispatchers|CreateEvent :!event LaunchedCharacterTeleported)))))))))))
    (:CastFailed
      (bind _asprimitive_component (Utilities|Casting|CastToPrimitiveComponent (Variables|/Script/Engine.Actor|GetRootComponent Actor)))
      (bind _output_get_2 (LocalVariables|SetLocalMesh _asprimitive_component))
      (if (Physics|IsSimulatingPhysics _output_get_2 "None")
        (CallFunction|PlayMeshLaunchMaterialsAnimation)
        (if (Variables|Sounds|GetPlay%20Launch%20Sound?)
          (Audio|Components|Audio|Play (Variables|Default|GetPT_Launch_Sound_Cue) 0.0))
        (switch Utilities|FlowControl|Switch|SwitchonPT_Launchpad_Launch_Type_Enum (Variables|Settings|GetLaunch%20Type)
          (:NewEnumerator0
            (LocalVariables|SetLocalEndVelocity (* (Math|Vector|GetUpVector (Variables|Default|GetMesh)) (Variables|Settings|GetLaunch%20Force))))
          (:NewEnumerator1
            (bind _tossvelocity_2 (Class|GameplayStatics|BlueprintSuggestProjectileVelocity (Transformation|GetWorldLocation (LocalVariables|GetLocalMesh)) (+ (Transformation|GetActorLocation) (Variables|Settings|GetTarget%20Location)) (Variables|Settings|GetLaunch%20Force) -9.8e+02 "DoNotTrace" 0.0 false false false))
            (LocalVariables|SetLocalEndVelocity _tossvelocity_2))
          (:NewEnumerator2
            (bind _outlaunchvelocity_2 (Game|SuggestProjectileVelocityCustomArc (Transformation|GetWorldLocation (LocalVariables|GetLocalMesh)) (+ (Transformation|GetActorLocation) (Variables|Settings|GetTarget%20Location)) -9.8e+02 (Variables|Settings|GetCustom%20Arc)))
            (LocalVariables|SetLocalEndVelocity _outlaunchvelocity_2)))
        (bind _returnvalue (Physics|GetPhysicsLinearVelocity (LocalVariables|GetLocalMesh) "None"))
        (LocalVariables|SetLocalEndVelocity (Math|Vector|MakeVector (Math|Float|SelectFloat (.X (Math|Vector|BreakVector (LocalVariables|GetLocalEndVelocity))) (.x (+ _returnvalue (Math|Vector|MakeVector (.X (Math|Vector|BreakVector (LocalVariables|GetLocalEndVelocity))) (.Y (Math|Vector|BreakVector (LocalVariables|GetLocalEndVelocity))) (.Z (Math|Vector|BreakVector (LocalVariables|GetLocalEndVelocity)))))) (Variables|Settings|GetOverride%20XY%20Velocity?)) (Math|Float|SelectFloat (.Y (Math|Vector|BreakVector (LocalVariables|GetLocalEndVelocity))) (.y (+ _returnvalue (Math|Vector|MakeVector (.X (Math|Vector|BreakVector (LocalVariables|GetLocalEndVelocity))) (.Y (Math|Vector|BreakVector (LocalVariables|GetLocalEndVelocity))) (.Z (Math|Vector|BreakVector (LocalVariables|GetLocalEndVelocity)))))) (Variables|Settings|GetOverride%20XY%20Velocity?)) (Math|Float|SelectFloat (.Z (Math|Vector|BreakVector (LocalVariables|GetLocalEndVelocity))) (.z (+ _returnvalue (Math|Vector|MakeVector (.X (Math|Vector|BreakVector (LocalVariables|GetLocalEndVelocity))) (.Y (Math|Vector|BreakVector (LocalVariables|GetLocalEndVelocity))) (.Z (Math|Vector|BreakVector (LocalVariables|GetLocalEndVelocity)))))) (Variables|Settings|GetOverride%20Z%20Velocity?))))
        (Class|PrimitiveComponent|SetAllPhysicsLinearVelocity (LocalVariables|GetLocalMesh) (LocalVariables|GetLocalEndVelocity) false)
        (Utilities|FlowControl|Sequence
          (:then_0
            (if (Variables|Settings|Actors|GetOverride%20Angular%20Velocity?)
              (Class|PrimitiveComponent|SetAllPhysicsAngularVelocityinDegrees (LocalVariables|GetLocalMesh) (* (* (Math|Vector|GetRightVector (Math|Rotator|MakeRotfromX (LocalVariables|GetLocalEndVelocity))) (/ (Math|Vector|VectorLength (LocalVariables|GetLocalEndVelocity)) 8.0)) (Variables|Settings|Actors|GetAngular%20Velocity%20Multiplier)) false)))
          (:then_1
            (if (Variables|Settings|Actors|GetReset%20Actor%20Rotation?)
              (Transformation|SetWorldRotation (LocalVariables|GetLocalMesh) (Math|Rotator|MakeRotator 0.0 0.0 (.Yaw (Math|Rotator|BreakRotator (Math|Rotator|MakeRotfromX (LocalVariables|GetLocalEndVelocity))))) false false))))))))

(fn LaunchedCharacterHit
  (params (SelfActor :type Actor%20Object%20Reference) (OtherActor :type Actor%20Object%20Reference) (NormalImpulse :type Vector) (Hit :type Hit%20Result%20Structure%20%28by%20ref%29))
  (bind _ascharacter (Utilities|Casting|CastToCharacter SelfActor))
  (LocalVariables|SetLocalCharacter _ascharacter)
  (Input|ResetIgnoreMoveInput (Game|GetPlayerController 0))
  (CallFunction|UnbindAllCharacterEvents (LocalVariables|GetLocalCharacter))
  (return))

(fn LaunchedCharacterTeleported
  (params (Actor :type Actor%20Object%20Reference))
  (bind _ascharacter (Utilities|Casting|CastToCharacter Actor))
  (LocalVariables|SetLocalCharacter _ascharacter)
  (Input|ResetIgnoreMoveInput (Game|GetPlayerController 0))
  (CallFunction|UnbindAllCharacterEvents (LocalVariables|GetLocalCharacter))
  (return))

(fn UnbindAllCharacterEvents
  (params (Character :type Character%20Object%20Reference))
  (bind _returnvalue (Actor|GetComponentbyClass Character "/Game/Puzzle_Template/Portals/BPC_Portable.BPC_Portable_C"))
  (Collision|UnbindEventfromOnActorHit Character (EventDispatchers|CreateEvent self :!event LaunchedCharacterHit))
  (Utilities|IsValid _returnvalue
    (:Is%20Valid
      (EventDispatchers|UnbindEventfromTeleported _returnvalue (EventDispatchers|CreateEvent self :!event LaunchedCharacterTeleported)))))