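; Floor-mounted laser receiver for the puzzle template that powers linked actors while a laser is connected to it.
; Laser connect and disconnect events set the receiving flag and toggle power on ActorsToPower.
; The same events play or reverse a timeline that drives the mesh materials' State parameter, and a getter exposes the receiving state.
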(event Custom|Play%20Mesh%20Materials%20Animation
  ;[0 0 0] Animate the state of the materials included in the mesh
  (bind _alpha (Timeline|Animate_Mesh_Materials Play)
    (:Update
      (Rendering|Material|SetScalarParameterValueonMaterials (Variables|Default|GetMesh) "State" _alpha))))

(event Custom|Reverse%20Mesh%20Materials%20Animation
  ;[0 0 0] Animate the state of the materials included in the mesh
  (bind _alpha (Timeline|Animate_Mesh_Materials Reverse)
    (:Update
      (Rendering|Material|SetScalarParameterValueonMaterials (Variables|Default|GetMesh) "State" _alpha))))

(event EventOnLaserConnected
  (params (From%20Actor :type Actor%20Object%20Reference) (Hit%20Result :type Hit%20Result%20Structure))
  ;[0 0 0] On laser on
  (Variables|Runtime|SetIs%20Receiving%20Laser true)
  (CallFunction|PlayMeshMaterialsAnimation)
  (CallFunction|TogglePowertoActors true (Variables|Default|GetActors%20To%20Power)))

(event EventOnLaserDisconnected
  (params (From%20Actor :type Actor%20Object%20Reference))
  ;[0 0 0] On laser off
  (Variables|Runtime|SetIs%20Receiving%20Laser false)
  (CallFunction|ReverseMeshMaterialsAnimation)
  (CallFunction|TogglePowertoActors false (Variables|Default|GetActors%20To%20Power)))

(fn ConstructionScript
  (|CallParentFunction))

(fn IsReceivingLaser?
  (return (Variables|Runtime|GetIs%20Receiving%20Laser)))