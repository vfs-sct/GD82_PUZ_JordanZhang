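; BP_Laser_Box_Grabbable is a puzzle laser box that emits its own laser while it receives one.
; Laser connect and disconnect events toggle the PTLaser component and play or reverse a timeline driving the mesh materials' "State" parameter.
; Its portable component enables actor tick only within portal range, where Tick copies that material state to the clone mesh so both match.
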(event InPortalRange(PT_Portable_AC)
  ;[0 0 0] When we enter or leave a portal range, toggle the actor tick so that we can update the state of the clone mesh.
  (Actor|Tick|SetActorTickEnabled true))

(event NotinPortalRange(PT_Portable_AC)
  ;[0 0 0] When we enter or leave a portal range, toggle the actor tick so that we can update the state of the clone mesh.
  (Actor|Tick|SetActorTickEnabled false))

(event Custom|Play%20Mesh%20Materials%20Animation
  ;[0 0 0] Animate the state of the materials included in the mesh
  (bind _alpha (Timeline|Animate_Mesh_Materials Play)
    (:Update
      (Variables|Runtime|SetMesh%20State _alpha)
      (Rendering|Material|SetScalarParameterValueonMaterials (Variables|Character|GetMesh) "State" (Variables|Runtime|GetMesh%20State)))))

(event Custom|Reverse%20Mesh%20Materials%20Animation
  ;[0 0 0] Animate the state of the materials included in the mesh
  (bind _alpha (Timeline|Animate_Mesh_Materials Reverse)
    (:Update
      (Variables|Runtime|SetMesh%20State _alpha)
      (Rendering|Material|SetScalarParameterValueonMaterials (Variables|Character|GetMesh) "State" (Variables|Runtime|GetMesh%20State)))))

(event EventTick
  (params (DeltaSeconds :type Float%20%28single-precision%29))
  ;[0 0 0] The tick event only gets enabled when this actor is in range of a portal, we need this to update the state of our mesh to match the master state.
  (bind _asstatic_mesh_component (Utilities|Casting|CastToStaticMeshComponent (Variables|/Game/Puzzle_Template/Portals/BPC_Portable.BPC_Portable_C|GetClone%20Root (Variables|Default|GetPT_Portable_AC))))
  (Rendering|Material|SetScalarParameterValueonMaterials _asstatic_mesh_component "State" (Variables|Runtime|GetMesh%20State)))

(event EventOnLaserDisconnected
  (params (From%20Actor :type Actor%20Object%20Reference))
  ;[0 0 0] On laser off
  (Variables|Runtime|SetReceiving%20Laser? false)
  (Default|DisableLaser (Variables|Default|GetPT_Laser))
  (CallFunction|ReverseMeshMaterialsAnimation))

(event EventOnLaserConnected
  (params (From%20Actor :type Actor%20Object%20Reference) (Hit%20Result :type Hit%20Result%20Structure))
  ;[0 0 0] On laser on
  (Variables|Runtime|SetReceiving%20Laser? true)
  (Default|EnableLaser (Variables|Default|GetPT_Laser))
  (CallFunction|PlayMeshMaterialsAnimation))

(fn ConstructionScript)

(fn IsReceivingLaser?
  (return (Variables|Runtime|GetReceiving%20Laser?)))