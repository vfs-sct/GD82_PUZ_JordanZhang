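; BP_Laser_Receiver is a puzzle prefab that powers a list of linked actors while a laser is connected to it.
; Laser connect and disconnect events give or remove power through TogglePowerToActors on ActorsToPower.
; The same events play or reverse a timeline that drives the "State" scalar parameter on the receiver mesh's materials.
; IsReceivingLaser always returns false, and the construction script only calls its parent.
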(event EventOnLaserDisconnected
  (params (From%20Actor :type Actor%20Object%20Reference))
  ;[0 0 0] On laser off
  (CallFunction|TogglePowertoActors false (Variables|Default|GetActors%20To%20Power))
  ;[0 0 0] Animate the state of the materials included in the mesh
  (bind _alpha (Timeline|Animate_Mesh_Materials Reverse)
    (:Update
      (Rendering|Material|SetScalarParameterValueonMaterials (Variables|Default|GetLaser%20Receiver%20Mesh) "State" _alpha))))

(event EventOnLaserConnected
  (params (From%20Actor :type Actor%20Object%20Reference) (Hit%20Result :type Hit%20Result%20Structure))
  ;[0 0 0] On laser on
  (CallFunction|TogglePowertoActors true (Variables|Default|GetActors%20To%20Power))
  ;[0 0 0] Animate the state of the materials included in the mesh
  (bind _alpha (Timeline|Animate_Mesh_Materials Play)
    (:Update
      (Rendering|Material|SetScalarParameterValueonMaterials (Variables|Default|GetLaser%20Receiver%20Mesh) "State" _alpha))))

(fn ConstructionScript
  (|CallParentFunction))

(fn IsReceivingLaser?
  (return false))