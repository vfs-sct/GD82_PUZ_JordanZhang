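; Laser source puzzle prefab that emits a laser either permanently or only while receiving power.
; AlwaysPowered enables the PTLaser at BeginPlay and ignores power events; otherwise ReceivingPower and StoppedReceivingPower toggle the laser.
; A timeline plays or reverses alongside the laser, driving the "State" material parameter on the source mesh.
; The construction script presets that parameter from AlwaysPowered.
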(event Custom|Play%20Mesh%20Materials%20Animation
  ;[0 0 0] Animate mesh materials and laser distance multiplier
  (bind _alpha (Timeline|Animate_Mesh_Materials Play)
    (:Update
      (Rendering|Material|SetScalarParameterValueonMaterials (Variables|Default|GetLaser_Source_Mesh) "State" _alpha))))

(event Custom|Reverse%20Mesh%20Materials%20Animation
  ;[0 0 0] Animate mesh materials and laser distance multiplier
  (bind _alpha (Timeline|Animate_Mesh_Materials Reverse)
    (:Update
      (Rendering|Material|SetScalarParameterValueonMaterials (Variables|Default|GetLaser_Source_Mesh) "State" _alpha))))

(event EventBeginPlay
  (bind _pt_laser (Variables|Default|GetPT_Laser))
  ;[0 0 0] On begin play, check the "Always On?" variable and enable the laser if its set to TRUE.
  (if (Variables|Settings|GetAlways%20Powered?)
    (Default|EnableLaser _pt_laser)
    (CallFunction|PlayMeshMaterialsAnimation)
    (else
      (Default|DisableLaser _pt_laser)
      (CallFunction|ReverseMeshMaterialsAnimation))))

(event EventReceivingPower
  ;[0 0 0] Handle Power
  (if (not (Variables|Settings|GetAlways%20Powered?))
    (Default|EnableLaser (Variables|Default|GetPT_Laser))
    (CallFunction|PlayMeshMaterialsAnimation)))

(event EventStoppedReceivingPower
  ;[0 0 0] Handle Power
  (if (not (Variables|Settings|GetAlways%20Powered?))
    (Default|DisableLaser (Variables|Default|GetPT_Laser))
    (CallFunction|ReverseMeshMaterialsAnimation)))

(fn ConstructionScript
  (|CallParentFunction)
  (if (Variables|Settings|GetAlways%20Powered?)
    (Rendering|Material|SetScalarParameterValueonMaterials (Variables|Default|GetLaser_Source_Mesh) "State" 1.0)
    (else
      (Rendering|Material|SetScalarParameterValueonMaterials (Variables|Default|GetLaser_Source_Mesh) "State" 0.0))))