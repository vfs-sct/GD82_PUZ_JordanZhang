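; Puzzle laser mirror that reflects each incoming laser by spawning its own outgoing laser component at the hit point.
; A map keyed by source actor reuses one laser per source, aimed along the reflection of the trace direction about the hit normal.
; A timeline animates the mesh material State on connection and reverses when all lasers are off.
; The construction script picks the mirror mesh from MeshType.
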(event Custom|Play%20Mesh%20Materials%20Animation
  ;[0 0 0] Animate the state of the materials included in the mesh
  (bind _alpha (Timeline|Animate_Mesh_Material Play)
    (:Update
      (Rendering|Material|SetScalarParameterValueonMaterials (Variables|Default|GetLaser_Mirror) "State" _alpha))))

(event Custom|Reverse%20Mesh%20Materials%20Animation
  ;[0 0 0] Animate the state of the materials included in the mesh
  (bind _alpha (Timeline|Animate_Mesh_Material Reverse)
    (:Update
      (Rendering|Material|SetScalarParameterValueonMaterials (Variables|Default|GetLaser_Mirror) "State" _alpha))))

(event EventOnLaserUpdateHitResult
  (params (From%20Actor :type Actor%20Object%20Reference) (Hit%20Result :type Hit%20Result%20Structure))
  (bind (_new_location _new_rotation) (CallFunction|GetLaserLocation&RotationfromHitResult Hit%20Result))
  (bind _connected_lasers_map (Variables|Runtime|GetConnected%20Lasers%20Map))
  (bind (_value _returnvalue) (Utilities|Map|Find _connected_lasers_map From%20Actor))
  ;[0 0 0] On laser update
  (if _returnvalue
    (Transformation|SetWorldLocationAndRotation _value _new_location _new_rotation false false)))

(event EventOnLaserDisconnected
  (params (From%20Actor :type Actor%20Object%20Reference))
  (bind _connected_lasers_map (Variables|Runtime|GetConnected%20Lasers%20Map))
  (bind (_value _returnvalue) (Utilities|Map|Find _connected_lasers_map From%20Actor))
  ;[0 0 0] On laser off
  (if _returnvalue
    (Default|DisableLaser _value)
    (if (CallFunction|AreAllLasersOff?)
      (CallFunction|ReverseMeshMaterialsAnimation))))

(event EventOnLaserConnected
  (params (From%20Actor :type Actor%20Object%20Reference) (Hit%20Result :type Hit%20Result%20Structure))
  ;[0 0 0] On laser on
  (CallFunction|UpdateConnectedLasersMapandUpdateLaser From%20Actor Hit%20Result)
  (CallFunction|PlayMeshMaterialsAnimation))

(fn ConstructionScript
  (CallFunction|UpdateMesh))

(fn UpdateMesh
  (Components|StaticMesh|SetStaticMesh (Variables|Default|GetLaser_Mirror) (Utilities|Select :Index (Variables|Settings|GetMesh%20Type) :NewEnumerator0 "/Game/Puzzle_Template/zIgnore/Assets/Lasers/Laser_Mirror/PT_Laser_Mirror_2x4_SM.PT_Laser_Mirror_2x4_SM" :NewEnumerator1 "/Game/Puzzle_Template/zIgnore/Assets/Lasers/Laser_Mirror/PT_Laser_Mirror_2x4_45_Degrees_SM.PT_Laser_Mirror_2x4_45_Degrees_SM" :NewEnumerator3 "/Game/Puzzle_Template/zIgnore/Assets/Lasers/Laser_Mirror/PT_Laser_Mirror_2x2_SM.PT_Laser_Mirror_2x2_SM" :NewEnumerator2 "/Game/Puzzle_Template/zIgnore/Assets/Lasers/Laser_Mirror/PT_Laser_Mirror_2x2_45_Degrees_SM.PT_Laser_Mirror_2x2_45_Degrees_SM")))

(fn UpdateConnectedLasersMapandUpdateLaser
  (params (Actor :type Actor%20Object%20Reference) (Hit%20Result :type Hit%20Result%20Structure))
  (bind _connected_lasers_map (Variables|Runtime|GetConnected%20Lasers%20Map))
  (bind (_value _returnvalue) (Utilities|Map|Find _connected_lasers_map Actor))
  (bind (_new_location _new_rotation) (CallFunction|GetLaserLocation&RotationfromHitResult Hit%20Result))
  (bind (_new_location_2 _new_rotation_2) (CallFunction|GetLaserLocation&RotationfromHitResult Hit%20Result))
  (if _returnvalue
    (Transformation|SetWorldLocationAndRotation _value _new_location_2 _new_rotation_2 false false)
    (Default|EnableLaser _value)
    (return)
    (else
      (bind _returnvalue_2 (AddComponent|AddPTLaserBP false))
      (Utilities|Map|Add (Variables|Runtime|GetConnected%20Lasers%20Map) Actor _returnvalue_2)
      (Transformation|SetWorldLocationAndRotation _returnvalue_2 _new_location _new_rotation false false)
      (Default|EnableLaser _returnvalue_2)
      (return))))

(fn GetLaserLocation&RotationfromHitResult
  (params (Hit%20Result :type Hit%20Result%20Structure))
  (bind (_bblockinghit _binitialoverlap _time _distance _location _impactpoint _normal _impactnormal _physmat _hitactor _hitcomponent _hitbonename _bonename _hititem _elementindex _faceindex _tracestart _traceend) (Collision|BreakHitResult Hit%20Result))
  (return _location (Math|Conversions|RotationFromXVector (Math|Vector|GetReflectionVector (Math|Vector|GetUnitDirection(Vector) _tracestart _traceend) _normal))))

(fn AreAllLasersOff?
  (bind _values (Utilities|Map|Values (Variables|Runtime|GetConnected%20Lasers%20Map)))
  (for _array_element _values
    (if (Variables|/Game/Puzzle_Template/zIgnore/Assets/Lasers/PT_Laser_BP.PT_Laser_BP_C|GetIs%20Enabled? _array_element)
      (return false)))
  (return true))

(fn IsReceivingLaser?
  (return false))