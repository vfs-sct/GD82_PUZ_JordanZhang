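; BP_Sliding_Door is a puzzle door that opens when it receives power and closes when power stops.
; A timeline shrinks the two inner door halves horizontally and drives a "State" material parameter for the door lights, reversing to close.
; While closing, it pushes actors overlapping either half's detection volume out along the door's forward axis, toward a side chosen by dot product.
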(event Custom|Open%20Door
  ;[0 0 0] Door Animation
  (bind (_direction _alpha _lights) (Timeline|Door_Animation Play)
    (:Update
      (Transformation|SetWorldScale3D (Variables|Default|GetInner_Door_Left) (Math|Vector|Lerp(Vector) "1.000000,1.000000,1.000000" "0.333330,1.000000,1.000000" _alpha))
      (Rendering|Material|SetScalarParameterValueonMaterials (Variables|Default|GetDoor_Mesh) "State" _lights)
      (switch Utilities|FlowControl|Switch|SwitchonETimelineDirection _direction
        (:Backward
          (CallFunction|PushDetectedActorsAway))))))

(event Custom|Close%20Door
  ;[0 0 0] Door Animation
  (bind (_direction _alpha _lights) (Timeline|Door_Animation Reverse)
    (:Update
      (Transformation|SetWorldScale3D (Variables|Default|GetInner_Door_Left) (Math|Vector|Lerp(Vector) "1.000000,1.000000,1.000000" "0.333330,1.000000,1.000000" _alpha))
      (Rendering|Material|SetScalarParameterValueonMaterials (Variables|Default|GetDoor_Mesh) "State" _lights)
      (switch Utilities|FlowControl|Switch|SwitchonETimelineDirection _direction
        (:Backward
          (CallFunction|PushDetectedActorsAway))))))

(event EventReceivingPower
  ;[0 0 0] Handle power
  (CallFunction|OpenDoor))

(event EventStoppedReceivingPower
  ;[0 0 0] Handle power
  (CallFunction|CloseDoor))

(fn ConstructionScript
  (|CallParentFunction))

(fn PushDetectedActorsAway
  (bind _returnvalue (Transformation|GetActorForwardVector))
  (bind _output_get (LocalVariables|SetLocal%20Overlapping%20Actors (Collision|GetOverlappingActors (Variables|Default|GetInner_Door_Left_Detection) 0 :!class /Script/Engine.PrimitiveComponent)))
  (Utilities|Array|AppendArray _output_get (Collision|GetOverlappingActors (Variables|Default|GetInner_Door_Right_Detection) 0 :!class /Script/Engine.PrimitiveComponent))
  (for _array_element (LocalVariables|GetLocal%20Overlapping%20Actors)
    (if (!= _array_element self)
      (Transformation|AddWorldOffset (Variables|/Script/Engine.Actor|GetRootComponent _array_element) (* (* (Math|Vector|SelectVector _returnvalue (* _returnvalue -1.0) (> (Class|Actor|GetHorizontalDotProductto _array_element) 0.0)) 125.0) (Utilities|Time|GetWorldDeltaSeconds)) false false))))