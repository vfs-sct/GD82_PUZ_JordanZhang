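; Dust particle prop Blueprint for the puzzle template that fills a resizable box volume with Niagara particles.
; The construction script passes the box's full scaled size to the Niagara component's Box Size variable.
; It derives Spawn Rate from the length of the scaled extent times an amount multiplier, so density adjusts as the volume is resized.
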(fn ConstructionScript
  (bind _box (Variables|Default|GetBox))
  (bind _returnvalue (Components|Box|GetScaledBoxExtent _box))
  (Niagara|SetNiagaraVariable(Vector3) (Variables|Default|GetNiagara) "Box Size" (* _returnvalue 2.0))
  (Niagara|SetNiagaraVariable(Float) (Variables|Default|GetNiagara) "Spawn Rate" (* (Math|Vector|VectorLength (/ _returnvalue 5e+02)) (Variables|Default|GetParticles%20Amount%20Multiplier))))