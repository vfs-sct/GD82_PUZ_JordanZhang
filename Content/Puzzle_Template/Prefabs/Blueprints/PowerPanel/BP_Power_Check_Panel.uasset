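; Power check panel for puzzles that powers its target actors while it receives enough power inputs.
; Received and stopped power events adjust a counter against the required amount.
; Two DoOnce gates re-arm each other, so connection and loss each fire once per threshold crossing, calling their notifications and toggling power on the targets.
; A reversible timeline animates the mesh's State material parameter, while Icon_State switches instantly.
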(event Custom|Play%20Mesh%20Materials%20Animation
  ;[0 0 0] Animate the state of the materials included in the mesh
  (Rendering|Material|SetScalarParameterValueonMaterials (Variables|Default|GetMesh) "Icon_State" 1.0)
  (bind _alpha (Timeline|Timeline_0 Play)
    (:Update
      (Rendering|Material|SetScalarParameterValueonMaterials (Variables|Default|GetMesh) "State" _alpha))))

(event Custom|Reverse%20Mesh%20Materials%20Animation
  ;[0 0 0] Animate the state of the materials included in the mesh
  (Rendering|Material|SetScalarParameterValueonMaterials (Variables|Default|GetMesh) "Icon_State" 0.0)
  (bind _alpha (Timeline|Timeline_0 Reverse)
    (:Update
      (Rendering|Material|SetScalarParameterValueonMaterials (Variables|Default|GetMesh) "State" _alpha))))

(event EventOnPowerReceived
  ;[0 0 0] Manage Power, when we reach the amount required, send power to actors to power
  (bind _result (Math|Integer|IncrementInt (Variables|Runtime|GetCurrent%20Power%20Amount))
    (:%20%20
      (if (>= _result (Variables|Settings|GetPower%20Amount%20Required))
        (Utilities|FlowControl|DoOnce false
          (:Completed
            (Default|CallOnFullyConnected)
            (CallFunction|PlayMeshMaterialsAnimation)
            (CallFunction|TogglePowertoActors true (Variables|Default|GetActors%20To%20Power))
            (Utilities|FlowControl|DoOnce true) ; enters at Reset
          ))))))

(event EventOnPowerStop
  ;[0 0 0] Manage Power, when we reach the amount required, send power to actors to power
  (bind _result (Math|Integer|DecrementInt (Variables|Runtime|GetCurrent%20Power%20Amount))
    (:%20%20
      (if (< _result (Variables|Settings|GetPower%20Amount%20Required))
        (Utilities|FlowControl|DoOnce true
          (:Completed
            (Default|CallOnConnectionLost)
            (CallFunction|ReverseMeshMaterialsAnimation)
            (CallFunction|TogglePowertoActors false (Variables|Default|GetActors%20To%20Power))
            (Utilities|FlowControl|DoOnce false) ; enters at Reset
          ))))))

(fn ConstructionScript
  (|CallParentFunction))