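; BP_Wall_Button_Toggle is an interactable wall button that toggles power to other actors in the puzzle template.
; Each interaction passes the inverse of IsGivingPower to TogglePowerToActors for the ActorsToPower array.
; The Toggle_Button timeline then plays or reverses based on IsGivingPower.
; Its update drives the State material parameter on Button and Light and scales Button along X.
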(event EventOnBeginInteract
  ;[0 0 0] On Begin Interact, give power to all actors in the array, then play an animation.
  (CallFunction|TogglePowertoActors (not (Variables|Default|GetIs%20Giving%20Power?)) (Variables|Default|GetActors%20To%20Power))
  (if (Variables|Default|GetIs%20Giving%20Power?)
    (bind (_direction _alpha _scale) (Timeline|Toggle_Button Play)
      (:Update
        (Rendering|Material|SetScalarParameterValueonMaterials (Variables|Default|GetButton) "State" _alpha)
        (Transformation|SetRelativeScale3D (Variables|Default|GetButton) (Math|Vector|Lerp(Vector) "0.200000,1.000000,1.000000" "0.600000,1.000000,1.000000" _scale))))
    (else
      (Timeline|Toggle_Button Reverse))))

(fn ConstructionScript
  (|CallParentFunction))