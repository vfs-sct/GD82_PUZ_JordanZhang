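; A timed wall button that powers the actors in its ActorsToPower array on interaction, then cuts their power when time runs out.
; The press timeline animates button scale and material state, then starts a power timeline whose play rate derives from PowerDuration and drives the timer light's Percent.
; When the timer finishes, power is removed and the press animation reverses, re-enabling interaction and playing a sound.
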(event Custom|Init%20Power%20Timer
  ;[0 0 0] On Begin Interact, give power to all actors in the array, then play an animation.
  (bind _percent (Timeline|Power_Timer PlayFromStart)
    (:Update
      (Rendering|Material|SetScalarParameterValueonMaterials (Variables|Default|GetTimer_Light) "Percent" _percent))
    (:Finished
      (Utilities|String|Reverse (Variables|Default|GetToggle_Button))
      (CallFunction|TogglePowertoActors false (Variables|Default|GetActors%20To%20Power)))))

(event EventOnBeginInteract
  (bind _timer_light (Variables|Default|GetTimer_Light))
  ;[0 0 0] On Begin Interact, give power to all actors in the array, then play an animation.
  (Variables|Default|SetCan%20Interact?%20 false)
  (CallFunction|TogglePowertoActors true (Variables|Default|GetActors%20To%20Power))
  (Components|Timeline|SetPlayRate (Variables|Default|GetPower_Timer) (/ 1.0 (- (Variables|Settings|GetPower%20Duration) 0.2)))
  (Rendering|Material|SetScalarParameterValueonMaterials _timer_light "Percent" 1.0)
  (Rendering|Material|SetScalarParameterValueonMaterials _timer_light "State" 0.0)
  (bind (_direction _alpha _scale) (Timeline|Toggle_Button PlayFromStart)
    (:Update
      (Rendering|Material|SetScalarParameterValueonMaterials (Variables|Default|GetButton) "State" _alpha)
      (Transformation|SetRelativeScale3D (Variables|Default|GetButton) (Math|Vector|Lerp(Vector) "0.200000,1.000000,1.000000" "0.600000,1.000000,1.000000" _scale))
      (Rendering|Material|SetScalarParameterValueonMaterials (Variables|Default|GetTimer_Light) "State" _alpha))
    (:Finished
      (switch Utilities|FlowControl|Switch|SwitchonETimelineDirection _direction
        (:Forward
          (CallFunction|InitPowerTimer))
        (:Backward
          (Variables|Default|SetCan%20Interact?%20 true)
          (Audio|Components|Audio|SetSound (Variables|Default|GetPressed%20/%20Released%20Audio) 0)
          (Audio|Components|Audio|Play (Variables|Default|GetPressed%20/%20Released%20Audio) 0.0))))))

(fn ConstructionScript
  (|CallParentFunction))