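; Puzzle moving platform that travels vertically or horizontally between two bases while powered, moving one way or cycling with an optional delay.
; The construction script sets base meshes and spacing from platform type and travel distance.
; Power events drive a duration-scaled, eased timeline for movement, start/stop audio and a material "State" power animation.
; Losing power clears pending turnaround timers, then either returns the platform to its start or stops it.
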(event Custom|Play%20Elevator%20Transition
  (bind _self self)
  (bind _delay_between_direction_change (Variables|Settings|GetDelay%20Between%20Direction%20Change))
  (bind _powered_movement_behaviour (Variables|Settings|GetPowered%20Movement%20Behaviour))
  (bind _delay_between_direction_change_2 (Variables|Settings|GetDelay%20Between%20Direction%20Change))
  ;[1 0.2604 0.3529] Elevator Animation
  (Audio|Components|Audio|SetSound (Variables|Default|GetPlatform%20Start%20/%20Stop%20Audio) (Variables|Sounds|GetPlatform%20Start%20Moving%20Sound))
  (Audio|Components|Audio|Play (Variables|Default|GetPlatform%20Moving%20Audio) 0.0)
  (bind (_direction _alpha) (Timeline|Move_Elevator Play)
    (:Update
      (Variables|Runtime|SetLast%20Transition%20Direction _direction)
      (bind _returnvalue (CallFunction|GetElevatorLocation(WithAlpha) (Math|Interpolation|Ease (Variables|Settings|GetTransition%20Interpolation%20Type) _alpha 0.0 1.0 2.0 8)))
      (Transformation|SetRelativeLocation (Variables|Default|GetPlatform) _returnvalue false false))
    (:Finished
      (Audio|Components|Audio|Stop (Variables|Default|GetPlatform%20Moving%20Audio))
      (Audio|Components|Audio|SetSound (Variables|Default|GetPlatform%20Start%20/%20Stop%20Audio) (Variables|Sounds|GetPlatform%20Stop%20Moving%20Sound))
      (Audio|Components|Audio|Play (Variables|Default|GetPlatform%20Start%20/%20Stop%20Audio) 0.0)
      (if (Variables|Runtime|GetIs%20Powered?)
        (switch Utilities|FlowControl|Switch|SwitchonETimelineDirection (Variables|Runtime|GetLast%20Transition%20Direction)
          (:Forward
            (switch Utilities|FlowControl|Switch|SwitchonPT_Moving_Platform_Powered_Behaviour_Enum _powered_movement_behaviour
              (:NewEnumerator2
                _)
              (:NewEnumerator3
                _))
            (if (> _delay_between_direction_change 0.0)
              (Utilities|Time|SetTimerbyFunctionName _self "Reverse Elevator Transition" _delay_between_direction_change_2)
              (Variables|Runtime|SetLast%20Transition%20Direction (Utilities|Select :Index (Variables|Runtime|GetLast%20Transition%20Direction) :Forward "Backward" :Backward "Forward") :!label _label)
              (else
                (CallFunction|ReverseElevatorTransition))))
          (:Backward
            (switch Utilities|FlowControl|Switch|SwitchonPT_Moving_Platform_Powered_Behaviour_Enum _powered_movement_behaviour
              (:NewEnumerator2
                _)
              (:NewEnumerator3
                _))
            (if (> _delay_between_direction_change 0.0)
              (Utilities|Time|SetTimerbyFunctionName _self "Play Elevator Transition" _delay_between_direction_change_2)
              (goto _label)
              (else
                (CallFunction|PlayElevatorTransition)))))
        (else
          (Variables|Runtime|SetLast%20Transition%20Direction (Utilities|Select :Index (Variables|Runtime|GetLast%20Transition%20Direction) :Forward "Backward" :Backward "Forward"))
          (CallFunction|ReversePowerAnim))))))

(event Custom|Reverse%20Elevator%20Transition
  (bind _self self)
  (bind _delay_between_direction_change (Variables|Settings|GetDelay%20Between%20Direction%20Change))
  (bind _powered_movement_behaviour (Variables|Settings|GetPowered%20Movement%20Behaviour))
  (bind _delay_between_direction_change_2 (Variables|Settings|GetDelay%20Between%20Direction%20Change))
  ;[1 0.2604 0.3529] Elevator Animation
  (Audio|Components|Audio|SetSound (Variables|Default|GetPlatform%20Start%20/%20Stop%20Audio) (Variables|Sounds|GetPlatform%20Start%20Moving%20Sound))
  (Audio|Components|Audio|Play (Variables|Default|GetPlatform%20Moving%20Audio) 0.0)
  (bind (_direction _alpha) (Timeline|Move_Elevator Reverse)
    (:Update
      (Variables|Runtime|SetLast%20Transition%20Direction _direction)
      (bind _returnvalue (CallFunction|GetElevatorLocation(WithAlpha) (Math|Interpolation|Ease (Variables|Settings|GetTransition%20Interpolation%20Type) _alpha 0.0 1.0 2.0 8)))
      (Transformation|SetRelativeLocation (Variables|Default|GetPlatform) _returnvalue false false))
    (:Finished
      (Audio|Components|Audio|Stop (Variables|Default|GetPlatform%20Moving%20Audio))
      (Audio|Components|Audio|SetSound (Variables|Default|GetPlatform%20Start%20/%20Stop%20Audio) (Variables|Sounds|GetPlatform%20Stop%20Moving%20Sound))
      (Audio|Components|Audio|Play (Variables|Default|GetPlatform%20Start%20/%20Stop%20Audio) 0.0)
      (if (Variables|Runtime|GetIs%20Powered?)
        (switch Utilities|FlowControl|Switch|SwitchonETimelineDirection (Variables|Runtime|GetLast%20Transition%20Direction)
          (:Forward
            (switch Utilities|FlowControl|Switch|SwitchonPT_Moving_Platform_Powered_Behaviour_Enum _powered_movement_behaviour
              (:NewEnumerator2
                _)
              (:NewEnumerator3
                _))
            (if (> _delay_between_direction_change 0.0)
              (Utilities|Time|SetTimerbyFunctionName _self "Reverse Elevator Transition" _delay_between_direction_change_2)
              (Variables|Runtime|SetLast%20Transition%20Direction (Utilities|Select :Index (Variables|Runtime|GetLast%20Transition%20Direction) :Forward "Backward" :Backward "Forward") :!label _label)
              (else
                (CallFunction|ReverseElevatorTransition))))
          (:Backward
            (switch Utilities|FlowControl|Switch|SwitchonPT_Moving_Platform_Powered_Behaviour_Enum _powered_movement_behaviour
              (:NewEnumerator2
                _)
              (:NewEnumerator3
                _))
            (if (> _delay_between_direction_change 0.0)
              (Utilities|Time|SetTimerbyFunctionName _self "Play Elevator Transition" _delay_between_direction_change_2)
              (goto _label)
              (else
                (CallFunction|PlayElevatorTransition)))))
        (else
          (Variables|Runtime|SetLast%20Transition%20Direction (Utilities|Select :Index (Variables|Runtime|GetLast%20Transition%20Direction) :Forward "Backward" :Backward "Forward"))
          (CallFunction|ReversePowerAnim))))))

(event Custom|Stop%20Elevator%20Transition
  (bind _self self)
  (bind _delay_between_direction_change (Variables|Settings|GetDelay%20Between%20Direction%20Change))
  (bind _powered_movement_behaviour (Variables|Settings|GetPowered%20Movement%20Behaviour))
  (bind _delay_between_direction_change_2 (Variables|Settings|GetDelay%20Between%20Direction%20Change))
  ;[1 0.2604 0.3529] Elevator Animation
  (Audio|Components|Audio|SetSound (Variables|Default|GetPlatform%20Start%20/%20Stop%20Audio) (Variables|Sounds|GetPlatform%20Stop%20Moving%20Sound))
  (Audio|Components|Audio|Play (Variables|Default|GetPlatform%20Moving%20Audio) 0.0)
  (bind (_direction _alpha) (Timeline|Move_Elevator Stop)
    (:Update
      (Variables|Runtime|SetLast%20Transition%20Direction _direction)
      (bind _returnvalue (CallFunction|GetElevatorLocation(WithAlpha) (Math|Interpolation|Ease (Variables|Settings|GetTransition%20Interpolation%20Type) _alpha 0.0 1.0 2.0 8)))
      (Transformation|SetRelativeLocation (Variables|Default|GetPlatform) _returnvalue false false))
    (:Finished
      (Audio|Components|Audio|Stop (Variables|Default|GetPlatform%20Moving%20Audio))
      (Audio|Components|Audio|SetSound (Variables|Default|GetPlatform%20Start%20/%20Stop%20Audio) (Variables|Sounds|GetPlatform%20Stop%20Moving%20Sound))
      (Audio|Components|Audio|Play (Variables|Default|GetPlatform%20Start%20/%20Stop%20Audio) 0.0)
      (if (Variables|Runtime|GetIs%20Powered?)
        (switch Utilities|FlowControl|Switch|SwitchonETimelineDirection (Variables|Runtime|GetLast%20Transition%20Direction)
          (:Forward
            (switch Utilities|FlowControl|Switch|SwitchonPT_Moving_Platform_Powered_Behaviour_Enum _powered_movement_behaviour
              (:NewEnumerator2
                _)
              (:NewEnumerator3
                _))
            (if (> _delay_between_direction_change 0.0)
              (Utilities|Time|SetTimerbyFunctionName _self "Reverse Elevator Transition" _delay_between_direction_change_2)
              (Variables|Runtime|SetLast%20Transition%20Direction (Utilities|Select :Index (Variables|Runtime|GetLast%20Transition%20Direction) :Forward "Backward" :Backward "Forward") :!label _label)
              (else
                (CallFunction|ReverseElevatorTransition))))
          (:Backward
            (switch Utilities|FlowControl|Switch|SwitchonPT_Moving_Platform_Powered_Behaviour_Enum _powered_movement_behaviour
              (:NewEnumerator2
                _)
              (:NewEnumerator3
                _))
            (if (> _delay_between_direction_change 0.0)
              (Utilities|Time|SetTimerbyFunctionName _self "Play Elevator Transition" _delay_between_direction_change_2)
              (goto _label)
              (else
                (CallFunction|PlayElevatorTransition)))))
        (else
          (Variables|Runtime|SetLast%20Transition%20Direction (Utilities|Select :Index (Variables|Runtime|GetLast%20Transition%20Direction) :Forward "Backward" :Backward "Forward"))
          (CallFunction|ReversePowerAnim))))))

(event Custom|Reverse%20Power%20Anim
  ;[0 0.7912 1] Power animation
  (bind _alpha (Timeline|Animate_Power Reverse)
    (:Update
      (Rendering|Material|SetScalarParameterValueonMaterials (Variables|Default|GetBase_1) "State" _alpha))))

(event Custom|Play%20Power%20Anim
  ;[0 0.7912 1] Power animation
  (bind _alpha (Timeline|Animate_Power Play)
    (:Update
      (Rendering|Material|SetScalarParameterValueonMaterials (Variables|Default|GetBase_1) "State" _alpha))))

(event EventBeginPlay
  ;[1 0.4143 0] Update Elevator animation duration
  (Components|Timeline|SetPlayRate (Variables|Default|GetMove_Elevator) (/ 1.0 (Variables|Settings|GetTransition%20Duration))))

(event EventReceivingPower
  ;[0 1 0.1829] Receive power and start the elevator
  (Variables|Runtime|SetIs%20Powered? true)
  (switch Utilities|FlowControl|Switch|SwitchonPT_Moving_Platform_Powered_Behaviour_Enum (Variables|Settings|GetPowered%20Movement%20Behaviour)
    (:NewEnumerator0
      (CallFunction|PlayElevatorTransition :!label _label))
    (:NewEnumerator1
      (goto _label))
    (:NewEnumerator2
      (switch Utilities|FlowControl|Switch|SwitchonETimelineDirection (Variables|Runtime|GetLast%20Transition%20Direction) :!label _label_2
        (:Forward
          (CallFunction|PlayElevatorTransition))
        (:Backward
          (CallFunction|ReverseElevatorTransition))))
    (:NewEnumerator3
      (goto _label_2)))
  (CallFunction|PlayPowerAnim))

(event EventStoppedReceivingPower
  ;[0 1 0.1829] Receive power and start the elevator
  (Variables|Runtime|SetIs%20Powered? false)
  (CallFunction|ClearDirectionChangeDelays)
  (switch Utilities|FlowControl|Switch|SwitchonPT_Moving_Platform_Unpowered_Behaviour_Enum (Variables|Settings|GetUnpowered%20Movement%20Behaviour)
    (:NewEnumerator0
      (CallFunction|ReverseElevatorTransition))
    (:NewEnumerator1
      (CallFunction|StopElevatorTransition)
      (CallFunction|ReversePowerAnim))))

(fn ConstructionScript
  (|CallParentFunction)
  (CallFunction|UpdateBase)
  (Variables|/Script/Engine.AudioComponent|SetAttenuationSettings (Variables|Default|GetPlatform%20Moving%20Audio) (Variables|Default|GetSounds%20Attenuation))
  (Variables|/Script/Engine.AudioComponent|SetAttenuationSettings (Variables|Default|GetPlatform%20Start%20/%20Stop%20Audio) (Variables|Default|GetSounds%20Attenuation)))

(fn UpdateBase
  (switch Utilities|FlowControl|Switch|SwitchonPT_Moving_Platform_Type_Enum (Variables|Settings|GetPlatform%20Type)
    (:NewEnumerator0
      (Components|StaticMesh|SetStaticMesh (Variables|Default|GetBase_1) "/Game/Puzzle_Template/zIgnore/Assets/Moving_Platform/PT_Moving_Platform_Vertical_Base_SM.PT_Moving_Platform_Vertical_Base_SM")
      (Components|StaticMesh|SetStaticMesh (Variables|Default|GetBase_2) "/Game/Puzzle_Template/zIgnore/Assets/Moving_Platform/PT_Moving_Platform_Vertical_Base_SM.PT_Moving_Platform_Vertical_Base_SM")
      (Transformation|SetRelativeLocation (Variables|Default|GetBase_2) (Math|Vector|MakeVector 0.0 0.0 (- (Variables|Settings|GetTravel%20Distance) 12.5)) false false)
      (Transformation|SetRelativeRotation (Variables|Default|GetBase_1) (Math|Rotator|MakeRotator 0.0 0.0 0.0) false false)
      (Transformation|SetRelativeRotation (Variables|Default|GetBase_2) (Math|Rotator|MakeRotator 0.0 0.0 0.0) false false)
      (bind _returnvalue (CallFunction|GetElevatorLocation(WithAlpha) 0.0))
      (Transformation|SetRelativeLocation (Variables|Default|GetPlatform) _returnvalue false false))
    (:NewEnumerator1
      (Components|StaticMesh|SetStaticMesh (Variables|Default|GetBase_1) "/Game/Puzzle_Template/zIgnore/Assets/Moving_Platform/PT_Moving_Platform_Horizontal_Base_SM.PT_Moving_Platform_Horizontal_Base_SM")
      (Components|StaticMesh|SetStaticMesh (Variables|Default|GetBase_2) "/Game/Puzzle_Template/zIgnore/Assets/Moving_Platform/PT_Moving_Platform_Horizontal_Base_SM.PT_Moving_Platform_Horizontal_Base_SM")
      (Transformation|SetRelativeLocation (Variables|Default|GetBase_2) (Math|Vector|MakeVector (Variables|Settings|GetTravel%20Distance) 0.0 12.5) false false)
      (Transformation|SetRelativeRotation (Variables|Default|GetBase_1) (Math|Rotator|MakeRotator 0.0 0.0 9e+01) false false)
      (Transformation|SetRelativeRotation (Variables|Default|GetBase_2) (Math|Rotator|MakeRotator 0.0 0.0 -9e+01) false false)
      (bind _returnvalue_2 (CallFunction|GetElevatorLocation(WithAlpha) 0.0))
      (Transformation|SetRelativeLocation (Variables|Default|GetPlatform) _returnvalue_2 false false))))

(fn GetElevatorLocation(WithAlpha)
  (params (Alpha :type Float%20%28double-precision%29))
  (switch Utilities|FlowControl|Switch|SwitchonPT_Moving_Platform_Powered_Behaviour_Enum (Variables|Settings|GetPowered%20Movement%20Behaviour)
    (:NewEnumerator0
      _)
    (:NewEnumerator1
      (return (Math|Vector|Lerp(Vector) (Variables|/Script/Engine.SceneComponent|GetRelativeLocation (Variables|Default|GetBase_2)) (Variables|/Script/Engine.SceneComponent|GetRelativeLocation (Variables|Default|GetBase_1)) Alpha)))
    (:NewEnumerator2
      _)
    (:NewEnumerator3
      (return (Math|Vector|Lerp(Vector) (Variables|/Script/Engine.SceneComponent|GetRelativeLocation (Variables|Default|GetBase_2)) (Variables|/Script/Engine.SceneComponent|GetRelativeLocation (Variables|Default|GetBase_1)) Alpha))))
  (return (Math|Vector|Lerp(Vector) (Variables|/Script/Engine.SceneComponent|GetRelativeLocation (Variables|Default|GetBase_1)) (Variables|/Script/Engine.SceneComponent|GetRelativeLocation (Variables|Default|GetBase_2)) Alpha)))

(fn ClearDirectionChangeDelays
  (Utilities|FlowControl|Sequence
    (:then_0
      (if (Class|KismetSystemLibrary|TimerExists self "Reverse Elevator Transition")
        (Utilities|Time|ClearTimerbyFunctionName self "Reverse Elevator Transition")
        (CallFunction|ReversePowerAnim)))
    (:then_1
      (if (Class|KismetSystemLibrary|TimerExists self "Play Elevator Transition")
        (Utilities|Time|ClearTimerbyFunctionName self "Play Elevator Transition")
        (CallFunction|ReversePowerAnim)))))