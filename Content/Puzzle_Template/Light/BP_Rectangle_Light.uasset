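; BP_Rectangle_Light is a configurable rectangular area light with a mesh panel and an optional four-piece border.
; The Construction Script derives the light's source width and height from the mesh's world scale, so scaling the panel resizes the emitter.
; It also applies exposed intensity, barn door, attenuation and mobility settings to the light.
; ShowBorders toggles the border pieces and stretches each pair to the matching panel axis.
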(fn ConstructionScript
  (bind _light (Variables|Default|GetLight))
  (bind _light_mesh (Variables|Default|GetLight_Mesh))
  (bind _light_mesh_2 (Variables|Default|GetLight_Mesh))
  (bind _border_1 (Variables|Default|GetBorder_1))
  (bind _returnvalue (Transformation|GetWorldScale _light_mesh_2))
  (bind _returnvalue_2 (Transformation|GetWorldScale _light_mesh))
  (bind (_x _y) (Math|Vector|BreakVector _returnvalue))
  (bind (_x_2 _y_2) (Math|Vector|BreakVector _returnvalue_2))
  (Class|RectLightComponent|SetSourceWidth _light (* _y 5e+01))
  (Class|RectLightComponent|SetSourceHeight _light (* _x 5e+01))
  (Rendering|Components|Light|SetIntensity _light (Variables|Default|GetIntensity))
  (Class|RectLightComponent|SetBarnDoorAngle (Variables|Default|GetLight) (Variables|Default|GetBarn%20Door%20Angle))
  (Class|RectLightComponent|SetBarnDoorLength (Variables|Default|GetLight) (Variables|Default|GetBarn%20Door%20Length))
  (Rendering|Lighting|SetAttenuationRadius (Variables|Default|GetLight) (Variables|Default|GetAttenuation))
  (Transformation|SetMobility (Variables|Default|GetLight) (Variables|Default|GetLight%20Mobility))
  (if (Variables|Default|GetShow%20Borders?)
    (Rendering|SetVisibility _border_1 true false)
    (Transformation|SetWorldScale3D (Variables|Default|GetBorder_1) (Math|Vector|MakeVector _x_2 0.2 1.0))
    (Transformation|SetWorldScale3D (Variables|Default|GetBorder_3) (Math|Vector|MakeVector _y_2 0.2 1.0))
    (else
      (Rendering|SetVisibility _border_1 false false))))