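; Game mode for puzzle template gameplay levels that fades the screen, spawns the player at a checkpoint and loads the game instance's current theme.
; Checkpoints are indexed by ID; the chosen one is activated, unpowers its actors and positions the possessed pawn, with index 0 as fallback.
; Restarting reopens the level with the current ID as a URL option, which BeginPlay parses to choose the spawn.
; GetCheckpointFromID is an empty stub.
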(event EventBeginPlay
  ;[0 0 0] On Begin Play, play a simple fade animation
  (CallFunction|StartFadeTransition 1.0 0.5 false true)
  (CallFunction|SpawnPlayeratCheckpoint (Utilities|GetInitialCheckpointID))
  (bind _aspt_main_gi (Utilities|Casting|CastToPT_Main_GI (Game|GetGameInstance)))
  (CallFunction|LoadPuzzleTemplateTheme (Variables|/Game/Puzzle_Template/PT_Main_GI.PT_Main_GI_C|GetCurrent%20Theme _aspt_main_gi)))

(fn ConstructionScript)

(fn SpawnPlayeratCheckpoint
  (params (Checkpoint%20ID :type Integer))
  (bind _returnvalue (Game|GetPlayerCharacter 0))
  (bind _localsortedcheckpoints (LocalVariables|GetLocalSortedCheckpoints))
  (bind _output (Utilities|Array|Get(acopy) _localsortedcheckpoints))
  (bind _capsulecomponent (Variables|/Script/Engine.Character|GetCapsuleComponent _returnvalue))
  (bind (_outradius _outhalfheight) (Components|Capsule|GetScaledCapsuleSize _capsulecomponent))
  ;[0 0 0] Try spawning the player character actor at the checkpoint id.
  (Variables|Runtime|SetCurrent%20Checkpoint%20ID Checkpoint%20ID)
  (bind _outactors (Actor|GetAllActorsOfClass "/Game/Puzzle_Template/Prefabs/Blueprints/Checkpoint/BP_Checkpoint.BP_Checkpoint_C"))
  (for _array_element _outactors
    (Utilities|Array|SetArrayElem (LocalVariables|GetLocalSortedCheckpoints) (Variables|/Game/Puzzle_Template/Prefabs/Blueprints/Checkpoint/BP_Checkpoint.BP_Checkpoint_C|GetCheckpoint%20ID _array_element) _array_element true))
  (for _array_element_2 (LocalVariables|GetLocalSortedCheckpoints)
    (if (< (Variables|/Game/Puzzle_Template/Prefabs/Blueprints/Checkpoint/BP_Checkpoint.BP_Checkpoint_C|GetCheckpoint%20ID _array_element_2) 0)
      (Variables|/Game/Puzzle_Template/Prefabs/Blueprints/Checkpoint/BP_Checkpoint.BP_Checkpoint_C|SetIs%20Activated? _array_element_2 true)
      (elif (== (Variables|/Game/Puzzle_Template/Prefabs/Blueprints/Checkpoint/BP_Checkpoint.BP_Checkpoint_C|GetCheckpoint%20ID _array_element_2) (Variables|Runtime|GetCurrent%20Checkpoint%20ID))
        (LocalVariables|SetLocalFinalCheckpoint _array_element_2)
        (LocalVariables|SetLocalFoundValidCheckpoint true)
        (bind _returnvalue_2 (Game|SpawnActorfromClass (Variables|Default|GetDefaultPawnClass) (Math|Transform|MakeTransform "0, 0, 0" "0, 0, 0" "1.000000,1.000000,1.000000") "AlwaysSpawn" "SelectDefaultAtRuntime" 0 0))
        (bind _output_get (Variables|Runtime|SetPlayer%20Pawn _returnvalue_2))
        (Pawn|Possess (Game|GetPlayerController 0) _output_get)
        (Variables|/Game/Puzzle_Template/Prefabs/Blueprints/Checkpoint/BP_Checkpoint.BP_Checkpoint_C|SetIs%20Activated? (LocalVariables|GetLocalFinalCheckpoint) true)
        (Default|ShowCheckpointPopupText (LocalVariables|GetLocalFinalCheckpoint))
        (Default|UnpowerActors (LocalVariables|GetLocalFinalCheckpoint))
        (bind _returnvalue_3 (Default|GetPlayerSpawnLocation (LocalVariables|GetLocalFinalCheckpoint) _outhalfheight _outradius))
        (Transformation|SetActorLocation (Variables|Runtime|GetPlayer%20Pawn) _returnvalue_3 false true)
        (Pawn|SetControlRotation (Game|GetPlayerController 0) (Math|Rotator|CombineRotators (Transformation|GetActorRotation (LocalVariables|GetLocalFinalCheckpoint)) (Math|Rotator|MakeRotator 0.0 0.0 (Variables|/Game/Puzzle_Template/Prefabs/Blueprints/Checkpoint/BP_Checkpoint.BP_Checkpoint_C|GetPlayer%20Spawn%20Yaw%20Offset (LocalVariables|GetLocalFinalCheckpoint)))))
        (return))))
  (if (not (LocalVariables|GetLocalFoundValidCheckpoint))
    (Development|PrintText (Utilities|Text|FormatText "ERROR: Unable to find checkpoint {id}!" (Variables|Runtime|GetCurrent%20Checkpoint%20ID)) true true "(R=1.000000,G=0.000000,B=0.000000,A=1.000000)" 5.0)
    (Utilities|IsValid _output
      (:Is%20Valid
        (LocalVariables|SetLocalFinalCheckpoint _output)
        (LocalVariables|SetLocalFoundValidCheckpoint true)
        (bind _returnvalue_4 (Game|SpawnActorfromClass (Variables|Default|GetDefaultPawnClass) (Math|Transform|MakeTransform "0, 0, 0" "0, 0, 0" "1.000000,1.000000,1.000000") "AlwaysSpawn" "SelectDefaultAtRuntime" 0 0))
        (bind _output_get_2 (Variables|Runtime|SetPlayer%20Pawn _returnvalue_4))
        (Pawn|Possess (Game|GetPlayerController 0) _output_get_2)
        (Variables|/Game/Puzzle_Template/Prefabs/Blueprints/Checkpoint/BP_Checkpoint.BP_Checkpoint_C|SetIs%20Activated? (LocalVariables|GetLocalFinalCheckpoint) true)
        (Default|ShowCheckpointPopupText (LocalVariables|GetLocalFinalCheckpoint))
        (Default|UnpowerActors (LocalVariables|GetLocalFinalCheckpoint))
        (bind _returnvalue_5 (Default|GetPlayerSpawnLocation (LocalVariables|GetLocalFinalCheckpoint) _outhalfheight _outradius))
        (Transformation|SetActorLocation (Variables|Runtime|GetPlayer%20Pawn) _returnvalue_5 false true)
        (Pawn|SetControlRotation (Game|GetPlayerController 0) (Math|Rotator|CombineRotators (Transformation|GetActorRotation (LocalVariables|GetLocalFinalCheckpoint)) (Math|Rotator|MakeRotator 0.0 0.0 (Variables|/Game/Puzzle_Template/Prefabs/Blueprints/Checkpoint/BP_Checkpoint.BP_Checkpoint_C|GetPlayer%20Spawn%20Yaw%20Offset (LocalVariables|GetLocalFinalCheckpoint)))))
        (return))
      (:Is%20Not%20Valid
        (Development|PrintText "ERROR: The level does not have any checkpoint, add at least one checkpoint to make the player spawn." true true "(R=1.000000,G=0.000000,B=0.000000,A=1.000000)" 5.0)))))

(fn RestartLevelatCurrentCheckpoint
  (bind _returnvalue (Game|GetCurrentLevelName true))
  (Game|OpenLevel(byName) (Utilities|String|StringToName _returnvalue) true (Utilities|String|ToString(Text) (Utilities|Text|FormatText "?Checkpoint={ID}" (Variables|Runtime|GetCurrent%20Checkpoint%20ID)))))

(fn GetCheckpointfromID
  (params (ID :type Integer)))

(fn GetInitialCheckpointID
  (bind _optionsstring (Variables|Default|GetOptionsString))
  (bind _returnvalue (Class|GameplayStatics|ParseOption _optionsstring "Checkpoint"))
  (if (not (Utilities|Array|IsEmpty _returnvalue))
    (return (Math|Conversions|ToInteger(Byte) _returnvalue))
    (else
      (return 0))))